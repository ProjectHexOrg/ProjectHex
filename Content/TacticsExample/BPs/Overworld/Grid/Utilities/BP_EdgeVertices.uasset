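; BP_EdgeVertices is an overworld grid utility actor that represents one edge as four evenly spaced vertices.
; Its construction script sets V1 and V4 to Corner1 and Corner2, and derives V2 and V3 by lerping between those corners at one-third and two-thirds.
; The event graph holds only disabled default events, so the Blueprint has no runtime logic.
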(event EventBeginPlay)

(event Collision|EventActorBeginOverlap
  (params (OtherActor :type Actor%20Object%20Reference)))

(event EventTick
  (params (DeltaSeconds :type Float%20%28single-precision%29)))

(fn ConstructionScript
  (Variables|Default|SetV1 (Variables|Default|GetCorner1))
  (Variables|Default|SetV2 (Math|Vector|Lerp(Vector) (Variables|Default|GetCorner1) (Variables|Default|GetCorner2) (/ 1.0 3.0)))
  (Variables|Default|SetV3 (Math|Vector|Lerp(Vector) (Variables|Default|GetCorner1) (Variables|Default|GetCorner2) (/ 2.0 3.0)))
  (Variables|Default|SetV4 (Variables|Default|GetCorner2)))