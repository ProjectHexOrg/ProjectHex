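; Overworld hex grid manager that spawns chunk and cell actors for a terraced terrain map.
; RefreshGrid reseeds the random stream, respawns the noise manager, clears old actors, builds chunks and neighbor-linked cells, then triggers chunk triangulation.
; Cells get elevation noise from Perlin values cached by position.
; Separate functions pick continent seeds, regroup cells by nearest seed like Voronoi regions, randomize terrain per chunk, and step elevations toward neighbors.
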(event EventBeginPlay)

(event Collision|EventActorBeginOverlap
  (params (OtherActor :type Actor%20Object%20Reference)))

(event EventTick
  (params (DeltaSeconds :type Float%20%28single-precision%29)))

(fn ConstructionScript
  (bind _gridtilesize (CallFunction|GetGridTileSize))
  (bind _returnvalue (/ (.x _gridtilesize) 2.0))
  (Variables|HexConstaants|SetHexOuterRadius _returnvalue)
  (Variables|HexConstaants|SetHexInnerRadius _returnvalue)
  (Variables|HexConstaants|SetHexElevationIncrement (.z _gridtilesize))
  (Variables|HexConstaants|SetHexCorners (Utilities|Map|MakeMap (Utilities|Enum|LiteralenumE_HexDirection "NewEnumerator0") (Math|Vector|MakeVector (Variables|HexConstaants|GetHexOuterRadius) 0.0 0.0) (Utilities|Enum|LiteralenumE_HexDirection "NewEnumerator1") (Math|Vector|MakeVector (* (Variables|HexConstaants|GetHexOuterRadius) 0.5) (Variables|HexConstaants|GetHexInnerRadius) 0.0) (Utilities|Enum|LiteralenumE_HexDirection "NewEnumerator2") (Math|Vector|MakeVector (* (Variables|HexConstaants|GetHexOuterRadius) -0.5) (Variables|HexConstaants|GetHexInnerRadius) 0.0) (Utilities|Enum|LiteralenumE_HexDirection "NewEnumerator3") (Math|Vector|MakeVector (* (Variables|HexConstaants|GetHexOuterRadius) -1.0) 0.0 0.0) (Utilities|Enum|LiteralenumE_HexDirection "NewEnumerator4") (Math|Vector|MakeVector (* (Variables|HexConstaants|GetHexOuterRadius) -0.5) (* (Variables|HexConstaants|GetHexInnerRadius) -1.0) 0.0) (Utilities|Enum|LiteralenumE_HexDirection "NewEnumerator5") (Math|Vector|MakeVector (* (Variables|HexConstaants|GetHexOuterRadius) 0.5) (* (Variables|HexConstaants|GetHexInnerRadius) -1.0) 0.0)))
  (bind _output_get (Variables|HexConstaants|SetTerraceSteps (+ (* (Variables|HexConstaants|GetTerracesPerSlope) 2) 1)))
  (Variables|HexConstaants|SetHorizontalTerraceStepSize (/ 1.0 (Math|Conversions|ToFloat(Integer) _output_get)))
  (Variables|HexConstaants|SetVerticalTerraceStepSize (/ 1.0 (+ (Math|Conversions|ToFloat(Integer) (Variables|HexConstaants|GetTerracesPerSlope)) 1.0)))
  (Variables|Mesh|SetCellCount (* (Variables|Mesh|GetChunkCount) (Variables|Mesh|GetChunkSize))))

(fn CreateChunks
  (bind _chunkcount (Variables|Mesh|GetChunkCount))
  (for _index (range 0 (- (.x _chunkcount) 1))
    (LocalVariables|SetX _index)
    (for _index_2 (range 0 (- (.y _chunkcount) 1))
      (LocalVariables|SetY _index_2)
      (bind _returnvalue (Game|SpawnActorfromClass "/Game/Blueprints/Overworld/Grid/Generation/BP_OverworldGridChunk.BP_OverworldGridChunk_C" (Math|Transform|MakeTransform "0, 0, 0" "0, 0, 0" "1.000000,1.000000,1.000000") "Undefined" "MultiplyWithRoot" 0 (Variables|HexConstaants|GetHexOuterRadius) (Variables|HexConstaants|GetHexInnerRadius) (Variables|HexConstaants|GetHexElevationIncrement) (Variables|HexConstaants|GetHexCorners) (Variables|Grid|GetGrid) (Variables|HexConstaants|GetSolidColorFactor) (Variables|HexConstaants|GetTerracesPerSlope) (Variables|Generation|GetRandomStream) (Variables|Generation|GetNoiseStrength) (Variables|Generation|GetElevationNoiseStrength) (Variables|Generation|GetNoiseManager) self 0))
      (Utilities|Map|Add (Variables|Mesh|GetChunks) (Utilities|Struct|MakeIntPoint (LocalVariables|GetX) (LocalVariables|GetY)) _returnvalue))))

(fn CreateCell
  (params (Index :type S%20Hex%20Index%20Structure))
  (bind _location (Utility|IndextoLocation Index))
  (bind _out (MeshUtility|PerturbElevation _location))
  (bind _returnvalue (Game|SpawnActorfromClass "/Game/Blueprints/Overworld/Grid/Generation/BP_HexCell.BP_HexCell_C" (Math|Transform|MakeTransform _location "0, 0, 0" "1.000000,1.000000,1.000000") "Undefined" "MultiplyWithRoot" 0 Index _out 0 "NewEnumerator2" 0))
  (LocalVariables|SetNewCell _returnvalue)
  (Utilities|Map|Add (Variables|Mesh|GetCells) Index (LocalVariables|GetNewCell))
  (bind _enumvalue (|ForEachE_HexDirection)
    (:LoopBody
      (if (.ReturnValue (Utilities|Map|Find (Variables|Mesh|GetCells) (CallFunction|GetCellIndexinDirection _enumvalue Index)))
        (Default|SetNeighbor (LocalVariables|GetNewCell) _enumvalue (.Value (Utilities|Map|Find (Variables|Mesh|GetCells) (CallFunction|GetCellIndexinDirection _enumvalue Index))))))
    (:then
      (return (LocalVariables|GetNewCell)))))

(fn CreateHexCells
  (bind _cellcount (Variables|Mesh|GetCellCount))
  (for _index (range 0 (- (.x _cellcount) 1))
    (LocalVariables|SetX _index)
    (for _index_2 (range 0 (- (.y _cellcount) 1))
      (LocalVariables|SetY _index_2)
      (bind _cell (Mesh|CreateCell (Utilities|Struct|MakeS_HexIndex (LocalVariables|GetX) (LocalVariables|GetY))))
      (Default|AddCelltoChunk (.Value (Utilities|Map|Find (Variables|Mesh|GetChunks) (/ (Utilities|Struct|MakeIntPoint (LocalVariables|GetX) (LocalVariables|GetY)) (Variables|Mesh|GetChunkSize)))) _cell))))

(fn IndextoLocation
  (params (Index :type S%20Hex%20Index%20Structure))
  (LocalVariables|SetXOffset 0.0)
  (if (CallFunction|IsIntEven (Utilities|Struct|BreakS_HexIndex Index))
    _
    (else
      (LocalVariables|SetXOffset (Variables|HexConstaants|GetHexInnerRadius))))
  (return (Math|Vector|MakeVector (* (* (Utilities|Struct|BreakS_HexIndex Index) (Variables|HexConstaants|GetHexOuterRadius)) 1.5) (+ (* (Utilities|Struct|BreakS_HexIndex Index) (* (Variables|HexConstaants|GetHexInnerRadius) 2.0)) (LocalVariables|GetXOffset)) 0.0)))

(fn ClearMesh
  (bind _values (Utilities|Map|Values (Variables|Mesh|GetChunks)))
  (for _array_element _values
    (Actor|DestroyActor _array_element))
  (bind _values_2 (Utilities|Map|Values (Variables|Mesh|GetCells)))
  (for _array_element_2 _values_2
    (Actor|DestroyActor _array_element_2))
  (Variables|Mesh|SetCells (Utilities|Map|MakeMap))
  (Variables|Mesh|SetChunks (Utilities|Map|MakeMap)))

(fn RefreshGrid
  (Variables|Generation|SetRandomStream (Math|Random|MakeRandomStream (Variables|Generation|GetSeed)))
  (Utilities|IsValid (Variables|Generation|GetNoiseManager)
    (:Is%20Valid
      (Actor|DestroyActor (Variables|Generation|GetNoiseManager)))
    (:Is%20Not%20Valid
      _))
  (bind _returnvalue (Game|SpawnActorfromClass "/Game/Blueprints/Overworld/Grid/Generation/BP_Noise.BP_Noise_C" (Math|Transform|MakeTransform "0, 0, 0" "0, 0, 0" "1.000000,1.000000,1.000000") "Undefined" "MultiplyWithRoot" 0 0))
  (Variables|Generation|SetNoiseManager _returnvalue)
  (Utilities|FlowControl|Sequence
    (:then_0
      (Mesh|ClearMesh))
    (:then_1
      (Mesh|CreateChunks)
      (Mesh|CreateHexCells))
    (:then_3
      (Mesh|TriangulateGrid))))

(fn TriangulateGrid
  (bind _values (Utilities|Map|Values (Variables|Mesh|GetChunks)))
  (for _array_element _values
    (Default|CallOnChunkRequiresRefresh _array_element)))

(fn GetCenterHex
  (bind _cellcount (Variables|Mesh|GetCellCount))
  (return (.Value (Utilities|Map|Find (Variables|Mesh|GetCells) (Utilities|Struct|MakeS_HexIndex (/ (.x _cellcount) 2) (/ (.y _cellcount) 2))))))

(fn PerturbElevation
  (params (Position :type Vector))
  (bind _returnvalue (* Position 1e+02))
  (bind _output_get (LocalVariables|SetKey (Math|Vector|MakeVector (Math|Conversions|ToFloat(Integer) (Math|Float|Round (.x _returnvalue))) (Math|Conversions|ToFloat(Integer) (Math|Float|Round (.y _returnvalue))) (Math|Conversions|ToFloat(Integer) (Math|Float|Round (.z _returnvalue))))))
  (if (.ReturnValue (Utilities|Map|Find (Variables|/Game/Blueprints/Overworld/Grid/Generation/BP_Noise.BP_Noise_C|GetNoiseMap (Variables|Generation|GetNoiseManager)) _output_get))
    (LocalVariables|SetNoise (.Value (Utilities|Map|Find (Variables|/Game/Blueprints/Overworld/Grid/Generation/BP_Noise.BP_Noise_C|GetNoiseMap (Variables|Generation|GetNoiseManager)) _output_get)))
    (else
      (bind _output_get_2 (LocalVariables|SetNoise (Math|Vector|MakeVector (Class|KismetMathLibrary|PerlinNoise1D (Math|Random|RandomFloatfromStream (Variables|Generation|GetRandomStream))) (Class|KismetMathLibrary|PerlinNoise1D (Math|Random|RandomFloatfromStream (Variables|Generation|GetRandomStream))) (Class|KismetMathLibrary|PerlinNoise1D (Math|Random|RandomFloatfromStream (Variables|Generation|GetRandomStream))))))
      (Utilities|Map|Add (Variables|/Game/Blueprints/Overworld/Grid/Generation/BP_Noise.BP_Noise_C|GetNoiseMap (Variables|Generation|GetNoiseManager)) (LocalVariables|GetKey) _output_get_2)))
  (return (+ (.z Position) (* (.z (LocalVariables|GetNoise)) (Variables|Generation|GetElevationNoiseStrength)))))

(fn GenerateChunkSeeds
  (Variables|Generation|SetContinentSeeds (Utilities|Array|MakeArray))
  (bind _values (Utilities|Map|Values (Variables|Mesh|GetChunks)))
  (for _array_element _values
    (LocalVariables|SetChunk _array_element)
    (bind _values_2 (Utilities|Map|Values (Variables|/Game/Blueprints/Overworld/Grid/Generation/BP_OverworldGridChunk.BP_OverworldGridChunk_C|GetCells (LocalVariables|GetChunk))))
    (Default|SetTerrainTypeandElevation (.OutItem (Utilities|Array|RandomFromStream _values_2 (Variables|Generation|GetRandomStream))) "NewEnumerator3" 1)
    (Utilities|Array|Add (Variables|Generation|GetContinentSeeds) (Variables|/Game/Blueprints/Overworld/Grid/Generation/BP_HexCell.BP_HexCell_C|GetIndex (.OutItem (Utilities|Array|RandomFromStream _values_2 (Variables|Generation|GetRandomStream)))))
    (Default|CallOnChunkRequiresRefresh (LocalVariables|GetChunk))))

(fn ReChunkCellsfromSeeds
  (Utilities|FlowControl|Sequence
    (:then_1
      (bind _values (Utilities|Map|Values (Variables|Mesh|GetCells)))
      (for _array_element _values
        (LocalVariables|SetTargetCell _array_element)
        (LocalVariables|SetMinDistance (CallFunction|GetDistanceBetweenIndexes (Variables|/Game/Blueprints/Overworld/Grid/Generation/BP_HexCell.BP_HexCell_C|GetIndex (LocalVariables|GetTargetCell)) (Utilities|Array|Get(acopy) (Variables|Generation|GetContinentSeeds))))
        (Utilities|FlowControl|Sequence
          (:then_0
            (for _array_element_2 (Variables|Generation|GetContinentSeeds)
              (LocalVariables|SetSeedIndex _array_element_2)
              (LocalVariables|SetD (CallFunction|GetDistanceBetweenIndexes (Variables|/Game/Blueprints/Overworld/Grid/Generation/BP_HexCell.BP_HexCell_C|GetIndex (LocalVariables|GetTargetCell)) (LocalVariables|GetSeedIndex)))
              (if (<= (CallFunction|GetDistanceBetweenIndexes (Variables|/Game/Blueprints/Overworld/Grid/Generation/BP_HexCell.BP_HexCell_C|GetIndex (LocalVariables|GetTargetCell)) (LocalVariables|GetSeedIndex)) (LocalVariables|GetMinDistance))
                (LocalVariables|SetClosestSeedIndex (LocalVariables|GetSeedIndex))
                (LocalVariables|SetMinDistance (LocalVariables|GetD)))))
          (:then_1
            (Default|AddCelltoChunk (Variables|/Game/Blueprints/Overworld/Grid/Generation/BP_HexCell.BP_HexCell_C|GetParentChunk (.Value (Utilities|Map|Find (Variables|Mesh|GetCells) (LocalVariables|GetClosestSeedIndex)))) (LocalVariables|GetTargetCell))))))
    (:then_2
      (bind _values_2 (Utilities|Map|Values (Variables|Mesh|GetChunks)))
      (for _array_element_3 _values_2
        (LocalVariables|SetChunk _array_element_3)
        (bind _output_get (LocalVariables|SetChunkElevation (Math|Random|RandomIntegerinRangefromStream (Variables|Generation|GetRandomStream) 0 4)))
        (LocalVariables|SetChunkTerrainType (Utilities|Select :Index _output_get :Option%200 "NewEnumerator2" :Option%201 "NewEnumerator3" :Option%202 "NewEnumerator9" :Option%203 "NewEnumerator4" :Option%204 "NewEnumerator7"))
        (bind _values_3 (Utilities|Map|Values (Variables|/Game/Blueprints/Overworld/Grid/Generation/BP_OverworldGridChunk.BP_OverworldGridChunk_C|GetCells _array_element_3)))
        (for _array_element_4 _values_3
          (Default|SetTerrainTypeandElevation _array_element_4 (LocalVariables|GetChunkTerrainType) 1))))))

(fn BlendChunkswithNeighbors
  (bind _values (Utilities|Map|Values (Variables|Mesh|GetChunks)))
  (for _array_element _values
    (bind _output_get (LocalVariables|SetChunk _array_element))
    (bind _values_2 (Utilities|Map|Values (Variables|/Game/Blueprints/Overworld/Grid/Generation/BP_OverworldGridChunk.BP_OverworldGridChunk_C|GetCells _output_get)))
    (for _array_element_2 _values_2
      (LocalVariables|SetCell _array_element_2)
      (bind _values_3 (Utilities|Map|Values (Variables|/Game/Blueprints/Overworld/Grid/Generation/BP_HexCell.BP_HexCell_C|GetNeighbors (LocalVariables|GetCell))))
      (for _array_element_3 _values_3
        (LocalVariables|SetNeighborCell _array_element_3)
        (if (< (Variables|/Game/Blueprints/Overworld/Grid/Generation/BP_HexCell.BP_HexCell_C|GetElevation (LocalVariables|GetCell)) (Variables|/Game/Blueprints/Overworld/Grid/Generation/BP_HexCell.BP_HexCell_C|GetElevation (LocalVariables|GetNeighborCell)))
          (Default|SetTerrainTypeandElevation (LocalVariables|GetCell) (Variables|/Game/Blueprints/Overworld/Grid/Generation/BP_HexCell.BP_HexCell_C|GetTerrainType (LocalVariables|GetCell)) (+ (Variables|/Game/Blueprints/Overworld/Grid/Generation/BP_HexCell.BP_HexCell_C|GetElevation (LocalVariables|GetCell)) 1))
          (elif (> (Variables|/Game/Blueprints/Overworld/Grid/Generation/BP_HexCell.BP_HexCell_C|GetElevation (LocalVariables|GetCell)) (Variables|/Game/Blueprints/Overworld/Grid/Generation/BP_HexCell.BP_HexCell_C|GetElevation (LocalVariables|GetNeighborCell)))
            (Default|SetTerrainTypeandElevation (LocalVariables|GetCell) (Variables|/Game/Blueprints/Overworld/Grid/Generation/BP_HexCell.BP_HexCell_C|GetTerrainType (LocalVariables|GetCell)) (+ (Variables|/Game/Blueprints/Overworld/Grid/Generation/BP_HexCell.BP_HexCell_C|GetElevation (LocalVariables|GetCell)) -1))))))))