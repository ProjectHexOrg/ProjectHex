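; Hex cell actor for the overworld grid, holding terrain type, elevation, color, neighbors and a point-of-interest mesh.
; Construction derives color from terrain and height from elevation plus noise, and labels the cell with its index, grid index and round-trip converted index.
; Setting a neighbor recursively links the opposite direction back.
; Helpers classify edge types by comparing elevations, and setters update terrain, height or POI mesh.
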(event EventBeginPlay)

(event Collision|EventActorBeginOverlap
  (params (OtherActor :type Actor%20Object%20Reference)))

(event EventTick
  (params (DeltaSeconds :type Float%20%28single-precision%29)))

(fn ConstructionScript
  (bind _returnvalue (Transformation|GetActorLocation))
  (bind _index (Variables|Default|GetIndex))
  (bind _index_2 (Variables|Default|GetIndex))
  (bind _index_3 (Variables|Default|GetIndex))
  (bind _gridindex (CallFunction|GetGridIndexfromCellIndex _index))
  (bind _gridindex_2 (CallFunction|GetGridIndexfromCellIndex _index_3))
  (bind _cellindex (CallFunction|GetCellIndexfromGridIndex _gridindex 0.0))
  (Variables|Default|SetColor (CallFunction|TerrainTypetoColor (Variables|Default|GetTerrainType)))
  (Rendering|Components|TextRender|SetText (Variables|Default|GetTextRender_Index) (Utilities|Text|ToText(String) (Utilities|String|Append (Utilities|String|ToString(Integer) (.x _index_2)) ", " (Utilities|String|ToString(Integer) (.y _index_2)))))
  (Rendering|Components|TextRender|SetText (Variables|Default|GetTextRender_GridIndex) (Utilities|Text|ToText(String) (Utilities|String|Append (Utilities|String|ToString(Integer) (.x _gridindex_2)) ", " (Utilities|String|ToString(Integer) (.y _gridindex_2)))))
  (Rendering|Components|TextRender|SetText (Variables|Default|GetTextRender_ConvertedIndex) (Utilities|Text|ToText(String) (Utilities|String|Append (Utilities|String|ToString(Integer) (.x _cellindex)) ", " (Utilities|String|ToString(Integer) (.y _cellindex)))))
  (Transformation|SetActorRelativeLocation (Math|Vector|MakeVector (.x _returnvalue) (.y _returnvalue) (+ (* (Math|Conversions|ToFloat(Integer) (Variables|Default|GetElevation)) (.z (CallFunction|GetGridTileSize))) (Variables|Default|GetElevationNoise))))
  (Rendering|Components|TextRender|SetTextRenderColor (Variables|Default|GetTextRender_Index) (Math|Conversions|ToColor(LinearColor) (Variables|Default|GetColor))))

(fn GetNeighbor
  (params (Direction :type E_HexDirection%20Enum :default "NewEnumerator0"))
  (bind _neighbors (Variables|Default|GetNeighbors))
  (bind (_value _returnvalue) (Utilities|Map|Find _neighbors Direction))
  (return _value _returnvalue))

(fn SetNeighbor
  (params (Direction :type E_HexDirection%20Enum :default "NewEnumerator0") (Neighbor :type BP%20Hex%20Cell%20Object%20Reference))
  (Utilities|Map|Add (Variables|Default|GetNeighbors) Direction Neighbor)
  (if (!= (.Neighbor (CallFunction|GetNeighbor Neighbor (CallFunction|OppositeDirection Direction))) self)
    (CallFunction|SetNeighbor Neighbor (CallFunction|OppositeDirection Direction) self)))

(fn GetEdgeTypefromDirection
  (params (Direction :type E_HexDirection%20Enum :default "NewEnumerator0"))
  (bind _neighbor (CallFunction|GetNeighbor Direction))
  (Utilities|IsValid _neighbor
    (:Is%20Valid
      (bind _edgetype (CallFunction|GetHexEdgeType (Variables|Default|GetElevation) (Variables|BP_HexCell_C|GetElevation _neighbor)))
      (return _edgetype))
    (:Is%20Not%20Valid
      (Utilities|String|LogString "Error: Tried to get edge type for null neighbor."))))

(fn GetEdgeTypefromCell
  (params (OtherCell :type BP%20Hex%20Cell%20Object%20Reference))
  (bind _edgetype (CallFunction|GetHexEdgeType (Variables|BP_HexCell_C|GetElevation OtherCell) (Variables|Default|GetElevation)))
  (return _edgetype))

(fn SetTerrainTypeandElevation
  (params (TerrainType :type E_TerrainType%20Enum :default "NewEnumerator0") (Elevation :type Integer))
  (bind _returnvalue (Transformation|GetActorLocation))
  (Variables|Default|SetTerrainType TerrainType)
  (Variables|Default|SetElevation Elevation)
  (Variables|Default|SetColor (CallFunction|TerrainTypetoColor (Variables|Default|GetTerrainType)))
  (Transformation|SetActorRelativeLocation (Math|Vector|MakeVector (.x _returnvalue) (.y _returnvalue) (+ (* (Math|Conversions|ToFloat(Integer) (Variables|Default|GetElevation)) (.z (CallFunction|GetGridTileSize))) (Variables|Default|GetElevationNoise)))))

(fn SetPOI
  (params (POI :type S%20POI%20Structure))
  (bind _output_get (Variables|Default|SetPOI POI))
  (Components|StaticMesh|SetStaticMesh (Variables|Default|GetPOI_StaticMesh) (.Mesh (Utilities|Struct|BreakS_POI _output_get))))