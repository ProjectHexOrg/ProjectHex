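; Overworld flow manager that tracks units on a tile grid, grouped by team, and runs their movement between points of interest.
; Units are registered on grid tiles, and following a path updates occupancy and deducts tile-type movement cost per step.
; Reaching a POI cancels movement and opens a paused narrative box, which can load the POI's battle level with the active team's party stored on the game instance.
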(event EventBeginPlay)

(event Collision|EventActorBeginOverlap
  (params (OtherActor :type Actor%20Object%20Reference)))

(event EventTick
  (params (DeltaSeconds :type Float%20%28single-precision%29)))

(fn ConstructionScript)

(fn AddUnit
  (params (Unit :type BP%20Unit%20Object%20Reference) (Index :type Int%20Point%20Structure) (TeamIndex :type Integer))
  (Utilities|Array|Add (Variables|Default|GetUnitsOnMap) Unit)
  (Default|SetGrid Unit (Variables|Default|GetGrid))
  (Units|SetUnitIndexonGrid Unit Index true true)
  (EventDispatchers|BindEventtoOnUnitReachedNewTile Unit (EventDispatchers|CreateEvent :!event OnUnitReachedNewTile))
  (Units|SetUnitTeamIndex Unit TeamIndex))

(fn SetUnitIndexonGrid
  (params (Unit :type BP%20Unit%20Object%20Reference) (Index :type Int%20Point%20Structure) (Force :type Boolean) (SnapLocation :type Boolean))
  (bind _grid (Variables|Default|GetGrid))
  (bind _gridtiles (Variables|/Game/Blueprints/Tactical/Grid/BP_GridManager.BP_GridManager_C|GetGridTiles _grid))
  (bind (_value _returnvalue) (Utilities|Map|Find _gridtiles Index))
  (Utilities|FlowControl|Sequence
    (:then_0
      ;[1 1 1] If new index, we move the unit from the previous index to the new one.
      (if (or (!= (Variables|/Game/Blueprints/Tactical/Units/BP_Unit.BP_Unit_C|GetIndex Unit) Index) Force)
        (Utilities|FlowControl|Sequence
          (:then_0
            (bind _output_get (LocalVariables|SetPreviousTile (.Value (Utilities|Map|Find (Variables|/Game/Blueprints/Tactical/Grid/BP_GridManager.BP_GridManager_C|GetGridTiles (Variables|Default|GetGrid)) (Variables|/Game/Blueprints/Tactical/Units/BP_Unit.BP_Unit_C|GetIndex Unit)))))
            (if (== (Utilities|Struct|BreakS_TileData _output_get) Unit)
              (bind _structout (Utilities|Struct|SetmembersinS_TileData (LocalVariables|GetPreviousTile)))
              (Utilities|Map|Add (Variables|/Game/Blueprints/Tactical/Grid/BP_GridManager.BP_GridManager_C|GetGridTiles (Variables|Default|GetGrid)) (Utilities|Struct|BreakS_TileData _structout) _structout)))
          (:then_1
            (Default|SetGridIndex Unit Index)
            (if (!= Index (Utilities|Struct|MakeIntPoint -999 -999))
              (bind _structout_2 (Utilities|Struct|SetmembersinS_TileData (.Value (Utilities|Map|Find (Variables|/Game/Blueprints/Tactical/Grid/BP_GridManager.BP_GridManager_C|GetGridTiles (Variables|Default|GetGrid)) Index)) Unit))
              (Utilities|Map|Add (Variables|/Game/Blueprints/Tactical/Grid/BP_GridManager.BP_GridManager_C|GetGridTiles (Variables|Default|GetGrid)) (Utilities|Struct|BreakS_TileData _structout_2) _structout_2)))
          (:then_2
            (Default|CallOnUnitGridIndexChanged Unit)))))
    (:then_1
      ;[1 1 1] Move actor to new tile in the world space.
      (if SnapLocation
        (Transformation|SetActorLocation Unit (select _returnvalue (.location (Utilities|Struct|BreakS_TileData _value)) "-99999.000000,-99999.000000,-99999.000000") false false)))))

(fn SetUnitTeamIndex
  (params (Unit :type BP%20Unit%20Object%20Reference) (TeamIndex :type Integer))
  (Utilities|FlowControl|Sequence
    (:then_0
      (if (!= (Variables|/Game/Blueprints/Tactical/Units/BP_Unit.BP_Unit_C|GetTeamIndex Unit) -1)
        (bind _output_get (LocalVariables|SetUnitSet (.unitset (.Value (Utilities|Map|Find (Variables|Default|GetUnitTeams) (Variables|/Game/Blueprints/Tactical/Units/BP_Unit.BP_Unit_C|GetTeamIndex Unit))))))
        (Utilities|Set|Remove _output_get Unit)
        (if (> (Utilities|Set|Length (LocalVariables|GetUnitSet)) 0)
          (Utilities|Map|Add (Variables|Default|GetUnitTeams) (Variables|/Game/Blueprints/Tactical/Units/BP_Unit.BP_Unit_C|GetTeamIndex Unit) (Utilities|Struct|MakeS_UnitSet (LocalVariables|GetUnitSet)))
          (else
            (Utilities|Map|Remove (Variables|Default|GetUnitTeams) (Variables|/Game/Blueprints/Tactical/Units/BP_Unit.BP_Unit_C|GetTeamIndex Unit))))))
    (:then_1
      (if (!= TeamIndex -1)
        (bind _output_get_2 (LocalVariables|SetUnitSet (.unitset (.Value (Utilities|Map|Find (Variables|Default|GetUnitTeams) TeamIndex)))))
        (Utilities|Set|Add _output_get_2 Unit)
        (Utilities|Map|Add (Variables|Default|GetUnitTeams) TeamIndex (Utilities|Struct|MakeS_UnitSet (LocalVariables|GetUnitSet)))))
    (:then_2
      (Default|SetTeamIndex Unit TeamIndex)
      (Default|CallOnUnitTeamsChanged))))

(fn OnUnitReachedNewTile
  (params (Unit :type BP%20Unit%20Object%20Reference) (Index :type Int%20Point%20Structure))
  (bind _grid (Variables|Default|GetGrid))
  (bind _mappois (Variables|Default|GetMapPOIs))
  (bind _cellindex (CallFunction|GetCellIndexfromGridIndex Index 1.0))
  (bind _gridtiles (Variables|/Game/Blueprints/Tactical/Grid/BP_GridManager.BP_GridManager_C|GetGridTiles _grid))
  (bind (_value _returnvalue) (Utilities|Map|Find _mappois _cellindex))
  (bind _value_2 (Utilities|Map|Find _gridtiles Index))
  (bind _type (Utilities|Struct|BreakS_TileData _value_2))
  (bind _cost (CallFunction|GetTileTypeCost _type))
  (bind _returnvalue_2 (- 0 _cost))
  (Default|SpawnAnimatedNumber Unit _returnvalue_2 "NewEnumerator0")
  (Default|ModifyCurrentMP Unit _returnvalue_2 true false)
  (Units|SetUnitIndexonGrid Unit Index false false)
  (if _returnvalue
    (Default|CancelPathFollowing Unit)
    (Flow|StartPOI _value)))

(fn StartSeason
  (Variables|Default|SetIsFlowActive true)
  ;[1 1 1] Notify units overworld movement has started.
  (for _array_element (Variables|Default|GetUnitsOnMap)
    (Default|OverworldActive _array_element))
  ;[1 1 1] Overworld movement started notification.
  (Default|CallOnOverworldActive)
  (Flow|SetActiveUnit (Utilities|Array|Get(acopy) (Variables|Default|GetUnitsOnMap))))

(fn EndCurrentTurn)

(fn SetActiveUnit
  (params (Unit :type BP%20Unit%20Object%20Reference))
  (bind _output_get (Variables|Default|SetActiveUnit Unit))
  (Default|CenterCameraonGridTile (Variables|Default|GetGrid) (Variables|/Game/Blueprints/Tactical/Units/BP_Unit.BP_Unit_C|GetIndex _output_get))
  (Default|CallOnUnitActivated _output_get))

(fn MoveUnit
  (params (Unit :type BP%20Unit%20Object%20Reference) (Path :type Array%20of%20Int%20Point%20Structures))
  (if (> (Utilities|Array|Length Path) 0)
    (EventDispatchers|BindEventtoOnUnitReachedNewTile Unit (EventDispatchers|CreateEvent :!event OnUnitReachedNewTile))
    (EventDispatchers|BindEventtoOnUnitFinishedWalking Unit (EventDispatchers|CreateEvent :!event OnUnitFinishedWalkingPath))
    (Default|EventFollowPath Unit Path)))

(fn OnUnitFinishedWalkingPath
  (params (Unit :type BP%20Unit%20Object%20Reference))
  (Utilities|IsValid Unit
    (:Is%20Valid
      (EventDispatchers|UnbindEventfromOnUnitReachedNewTile Unit (EventDispatchers|CreateEvent :!event OnUnitReachedNewTile))
      (EventDispatchers|UnbindEventfromOnUnitFinishedWalking Unit (EventDispatchers|CreateEvent :!event OnUnitFinishedWalkingPath))
      (Development|PrintString "Done Walking"))))

(fn StartPOI
  (params (POI :type S%20POI%20Structure))
  (bind _output_get (Variables|Default|SetActivePOI POI))
  (bind _returnvalue (UserInterface|CreateWidget "/Game/Blueprints/Overworld/UI/W_NarrativeBox.W_NarrativeBox_C" 0 _output_get))
  (bind _output_get_2 (Variables|Default|SetNarrativeBox _returnvalue))
  (UserInterface|Viewport|AddtoPlayerScreen _output_get_2)
  (EventDispatchers|BindEventtoOnNarrativeClosed _output_get_2 (EventDispatchers|CreateEvent :!event OnNarrativeBoxClosed))
  (EventDispatchers|BindEventtoOnLoadBattle _output_get_2 (EventDispatchers|CreateEvent :!event LoadBattle))
  (Game|SetGamePaused true))

(fn OnNarrativeBoxClosed
  (Game|SetGamePaused false)
  (Widget|RemovefromParent (Variables|Default|GetNarrativeBox))
  (Variables|Default|SetNarrativeBox 0)
  (Variables|Default|SetActivePOI ""))

(fn LoadBattle
  (bind _asgi_primary_game_instance (Utilities|Casting|CastToGI_PrimaryGameInstance (Game|GetGameInstance)))
  (Variables|/Game/Blueprints/Utilities/GI_PrimaryGameInstance.GI_PrimaryGameInstance_C|SetPartyInBattle _asgi_primary_game_instance (Utilities|Array|Get(acopy) (Variables|/Game/Blueprints/Utilities/GI_PrimaryGameInstance.GI_PrimaryGameInstance_C|GetDeployedParties _asgi_primary_game_instance) (Variables|/Game/Blueprints/Tactical/Units/BP_Unit.BP_Unit_C|GetTeamIndex (Variables|Default|GetActiveUnit))))
  (Game|OpenLevel(byName) (.LoadableLevelName (Utilities|Struct|BreakS_POI (Variables|Default|GetActivePOI)))))