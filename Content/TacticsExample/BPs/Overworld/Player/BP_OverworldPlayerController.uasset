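; Overworld player controller that handles camera control and click-to-move for possessed overworld characters.
; Pan, zoom and rotate inputs drive a separate camera target actor, interpolated every tick and recentered when a character is possessed.
; Holding secondary action traces under the cursor to update and draw the character's path, and release starts movement, which the controller ticks.
; Primary action re-possesses the default overworld pawn, clearing the current character.
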(event Input|EnhancedActionEvents|EnhancedInputActionIA_Overworld_PrimaryAction
  (params (ActionValue :type Boolean) (ElapsedSeconds :type Float%20%28double-precision%29) (TriggeredSeconds :type Float%20%28double-precision%29) (InputAction :type Input%20Action%20Object%20Reference :default "/Game/InputActions/Overworld/IA_Overworld_PrimaryAction.IA_Overworld_PrimaryAction"))
  ;[1 1 1] Actions
  (:Completed
    (Pawn|Possess (Variables|PawnManagement|GetDefaultPawn))))

(event Input|EnhancedActionEvents|EnhancedInputActionIA_Overworld_SecondaryAction
  (params (ActionValue :type Boolean) (ElapsedSeconds :type Float%20%28double-precision%29) (TriggeredSeconds :type Float%20%28double-precision%29) (InputAction :type Input%20Action%20Object%20Reference :default "/Game/InputActions/Overworld/IA_Overworld_SecondaryAction.IA_Overworld_SecondaryAction"))
  (bind (_hit _location) (PawnManagement|GetLocationUnderCursor))
  (bind _currentpawnasoverworldcharacter (Variables|PawnManagement|GetCurrentPawnAsOverworldCharacter))
  (bind _currentpawnasoverworldcharacter_2 (Variables|PawnManagement|GetCurrentPawnAsOverworldCharacter))
  (bind _currentpawnasoverworldcharacter_3 (Variables|PawnManagement|GetCurrentPawnAsOverworldCharacter))
  ;[1 1 1] Actions
  (:Triggered
    (Utilities|IsValid _currentpawnasoverworldcharacter
      (:Is%20Valid
        (if _hit
          (Default|UpdateCachedDestination _currentpawnasoverworldcharacter _location)
          (Default|DrawPath _currentpawnasoverworldcharacter)))))
  (:Started
    (Utilities|IsValid _currentpawnasoverworldcharacter_3
      (:Is%20Valid
        (Default|ClearPawnMovement _currentpawnasoverworldcharacter_3))))
  (:Completed
    (Utilities|IsValid _currentpawnasoverworldcharacter_2
      (:Is%20Valid
        (Default|StartMovement _currentpawnasoverworldcharacter_2)))))

(event Input|EnhancedActionEvents|EnhancedInputActionIA_Overworld_CameraZoom
  (params (ActionValue :type Float%20%28double-precision%29) (ElapsedSeconds :type Float%20%28double-precision%29) (TriggeredSeconds :type Float%20%28double-precision%29) (InputAction :type Input%20Action%20Object%20Reference :default "/Game/InputActions/Overworld/Camera/IA_Overworld_CameraZoom.IA_Overworld_CameraZoom"))
  ;[1 1 1] Camera Controls
  (Variables|Camera|SetTargetZoom (Math|Float|Clamp(Float) (+ (Variables|Camera|GetTargetZoom) (* ActionValue (Variables|Camera|GetCameraZoomSpeed))) (Variables|Camera|GetCameraZoomMin) (Variables|Camera|GetCameraZoomMax))))

(event Input|EnhancedActionEvents|EnhancedInputActionIA_Overworld_CameraPan
  (params (ActionValue :type Vector%202D%20Structure) (ElapsedSeconds :type Float%20%28double-precision%29) (TriggeredSeconds :type Float%20%28double-precision%29) (InputAction :type Input%20Action%20Object%20Reference :default "/Game/InputActions/Overworld/Camera/IA_Overworld_CameraPan.IA_Overworld_CameraPan"))
  (bind _camerapanspeed (Variables|Camera|GetCameraPanSpeed))
  (bind _returnvalue (* ActionValue _camerapanspeed))
  ;[1 1 1] Camera Controls
  (Variables|Camera|SetTargetLocation (+ (+ (Variables|Camera|GetTargetLocation) (* (Transformation|GetActorForwardVector (Variables|Default|GetCameraTarget)) (.x _returnvalue))) (* (.y _returnvalue) (Transformation|GetActorRightVector (Variables|Default|GetCameraTarget))))))

(event Input|EnhancedActionEvents|EnhancedInputActionIA_Overworld_CameraRotationLeft
  (params (ActionValue :type Boolean) (ElapsedSeconds :type Float%20%28double-precision%29) (TriggeredSeconds :type Float%20%28double-precision%29) (InputAction :type Input%20Action%20Object%20Reference :default "/Game/InputActions/Overworld/Camera/IA_Overworld_CameraRotationLeft.IA_Overworld_CameraRotationLeft"))
  ;[1 1 1] Camera Controls
  (:Started
    (Variables|Camera|SetIsCameraRotatingCW true))
  (:Canceled
    (Variables|Camera|SetIsCameraRotatingCW false :!label _label))
  (:Completed
    (goto _label)))

(event Input|EnhancedActionEvents|EnhancedInputActionIA_Overworld_CameraRotationRight
  (params (ActionValue :type Boolean) (ElapsedSeconds :type Float%20%28double-precision%29) (TriggeredSeconds :type Float%20%28double-precision%29) (InputAction :type Input%20Action%20Object%20Reference :default "/Game/InputActions/Overworld/Camera/IA_Overworld_CameraRotationRight.IA_Overworld_CameraRotationRight"))
  ;[1 1 1] Camera Controls
  (:Started
    (Variables|Camera|SetIsCameraRotatingCCW true))
  (:Canceled
    (Variables|Camera|SetIsCameraRotatingCCW false :!label _label))
  (:Completed
    (goto _label)))

(event EventTick
  (params (DeltaSeconds :type Float%20%28single-precision%29))
  (bind _currentpawnasoverworldcharacter (Variables|PawnManagement|GetCurrentPawnAsOverworldCharacter))
  ;[1 1 1] Tick
  (Camera|UpdateCameraonTick DeltaSeconds)
  (Utilities|IsValid _currentpawnasoverworldcharacter
    (:Is%20Valid
      (Default|PawnMovementonTick _currentpawnasoverworldcharacter))))

(event EventPossess
  (params (PossessedPawn :type Pawn%20Object%20Reference))
  ;[1 1 1] Game Flow
  (Utilities|IsValid (Variables|PawnManagement|GetCurrentPawnAsOverworldCharacter)
    (:Is%20Valid
      (Default|ClearPawnMovement (Variables|PawnManagement|GetCurrentPawnAsOverworldCharacter)))
    (:Is%20Not%20Valid
      _))
  (bind _asbp_overworld_character (Utilities|Casting|CastToBP_OverworldCharacter PossessedPawn)
    (:then
      (bind _output_get (Variables|PawnManagement|SetCurrentPawnAsOverworldCharacter _asbp_overworld_character))
      (PawnManagement|InitCharacteronPossess _output_get))
    (:CastFailed
      (Utilities|Casting|CastToBP_OverworldPawn PossessedPawn)
      (Variables|PawnManagement|SetCurrentPawnAsOverworldCharacter 0))))

(event EventBeginPlay
  ;[1 1 1] Game Flow
  (bind _returnvalue (Actor|GetActorOfClass "/Game/Blueprints/Overworld/Player/BP_OverworldPawn.BP_OverworldPawn_C"))
  (Variables|PawnManagement|SetDefaultPawn _returnvalue)
  (Variables|Camera|SetTargetZoom (Variables|/Script/Engine.SpringArmComponent|GetTargetArmLength (Variables|/Game/Blueprints/Overworld/Player/BP_OverworldPawn.BP_OverworldPawn_C|GetSpringArm (Variables|PawnManagement|GetDefaultPawn))))
  (Variables|Camera|SetTargetLocation (Transformation|GetActorLocation (Variables|PawnManagement|GetDefaultPawn)))
  (Input|AddMappingContext (PlayerController|LocalPlayerSubsystems|GetEnhancedInputLocalPlayerSubsystem self) "/Game/InputActions/Overworld/IMC_Overworld.IMC_Overworld" 0 "(bIgnoreAllPressedKeysUntilRelease=True,bForceImmediately=False,bNotifyUserSettings=False)")
  (Variables|Default|SetbShowMouseCursor true)
  (bind _returnvalue_2 (Actor|GetActorOfClass "/Game/Blueprints/Overworld/Player/BP_CameraTarget.BP_CameraTarget_C"))
  (Variables|Default|SetCameraTarget _returnvalue_2)
  (Game|Player|SetViewTargetwithBlend (Game|GetPlayerController 0) (Variables|Default|GetCameraTarget) 0.0 "VTBlend_Linear" 0.0 false))

(fn ConstructionScript)

(fn UpdateCameraonTick
  (params (DeltaTime :type Float%20%28single-precision%29))
  (Camera|GetCameraZoomInterp DeltaTime)
  (Camera|GetCameraLocationInterp DeltaTime)
  (Camera|GetCameraRotationInterp DeltaTime))

(fn GetCameraZoomInterp
  (params (DeltaTime :type Float%20%28double-precision%29))
  (Variables|/Script/Engine.SpringArmComponent|SetTargetArmLength (Variables|/Game/Blueprints/Overworld/Player/BP_CameraTarget.BP_CameraTarget_C|GetSpringArm (Variables|Default|GetCameraTarget)) (Math|Interpolation|FInterpTo (Variables|/Script/Engine.SpringArmComponent|GetTargetArmLength (Variables|/Game/Blueprints/Overworld/Player/BP_CameraTarget.BP_CameraTarget_C|GetSpringArm (Variables|Default|GetCameraTarget))) (Variables|Camera|GetTargetZoom) DeltaTime (Variables|Camera|GetCameraZoomInterp)))
  (return))

(fn GetCameraLocationInterp
  (params (DeltaTime :type Float%20%28single-precision%29))
  (Transformation|SetActorLocation (Variables|Default|GetCameraTarget) (Math|Interpolation|VInterpTo (Transformation|GetActorLocation (Variables|Default|GetCameraTarget)) (Variables|Camera|GetTargetLocation) DeltaTime (Variables|Camera|GetCameraLocationInterp)) false false)
  (return))

(fn GetCameraRotationInterp
  (params (DeltaTime :type Float%20%28single-precision%29))
  (LocalVariables|SetTarget (Transformation|GetActorRotation (Variables|Default|GetCameraTarget)))
  (Utilities|FlowControl|Sequence
    (:then_0
      (if (Variables|Camera|GetIsCameraRotatingCW)
        (LocalVariables|SetTarget (Math|Rotator|CombineRotators (LocalVariables|GetTarget) (Math|Rotator|MakeRotator 0.0 0.0 (* (Variables|Camera|GetCameraRotationDegree) 1.0))))))
    (:then_1
      (if (Variables|Camera|GetIsCameraRotatingCCW)
        (LocalVariables|SetTarget (Math|Rotator|CombineRotators (LocalVariables|GetTarget) (Math|Rotator|MakeRotator 0.0 0.0 (* (Variables|Camera|GetCameraRotationDegree) -1.0))))))
    (:then_2
      (if (or (Variables|Camera|GetIsCameraRotatingCW) (Variables|Camera|GetIsCameraRotatingCCW))
        (Transformation|SetActorRotation (Variables|Default|GetCameraTarget) (Math|Interpolation|RInterpTo (Transformation|GetActorRotation (Variables|Default|GetCameraTarget)) (LocalVariables|GetTarget) DeltaTime (Variables|Camera|GetCameraRotationInterp)))
        (return)))))

(fn GetLocationUnderCursor
  (bind _hitresult (Game|Player|GetHitResultUnderCursorbyChannel "TraceTypeQuery1" true))
  (bind (_bblockinghit _binitialoverlap _time _distance _location) (Collision|BreakHitResult _hitresult))
  (return _bblockinghit _location))

(fn InitCharacteronPossess
  (params (PawnAsOverworldCharacter :type BP%20Overworld%20Character%20Object%20Reference))
  (Variables|Camera|SetTargetLocation (Transformation|GetWorldLocation (Variables|/Script/Engine.Actor|GetRootComponent PawnAsOverworldCharacter))))