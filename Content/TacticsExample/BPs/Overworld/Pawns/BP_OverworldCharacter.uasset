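; Overworld tactics character that previews navmesh paths and moves along them on a movement point (MP) budget.
; UpdateCachedDestination finds a path once the destination shifts far enough and subdivides it into short segments, which DrawPath renders as spline meshes, branching on remaining MP.
; StartMovement consumes waypoints through SimpleMoveToLocation, with PawnMovementOnTick advancing near each goal.
; Tick drains MP by distance travelled and clears movement when it runs out.
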(event EventTick
  (params (DeltaSeconds :type Float%20%28single-precision%29))
  (bind _output_get (Variables|Default|SetMP (- (Variables|Default|GetMP) (* DeltaSeconds (Math|Vector|VectorLength (Transformation|GetVelocity))))))
  (if (and (<= _output_get 0.0) (> (Utilities|Array|Length (Variables|Default|GetCachedPath)) 0))
    (CallFunction|ClearPawnMovement)))

(fn ConstructionScript
  (Transformation|DetachFromComponent (Variables|Default|GetCamera) "KeepWorld" "KeepWorld" "KeepWorld" true))

(fn DrawPathSplineMesh
  (params (PathPoints :type Array%20of%20Vectors) (MPLimit :type Float%20%28double-precision%29))
  (LocalVariables|SetRemainingMP MPLimit)
  (CallFunction|ClearSplineMeshComponents)
  (Spline|ClearSplinePoints (Variables|Default|GetSpline) true)
  (for _array_element PathPoints
    (Spline|AddSplinePoint (Variables|Default|GetSpline) (+ _array_element "0.000000,0.000000,30.000000") "World" true))
  (for _index (range 0 (- (Spline|GetNumberOfSplinePoints (Variables|Default|GetSpline)) 2))
    (if (> (LocalVariables|GetRemainingMP) 0.0)
      (bind _returnvalue (AddComponent|AddSplineMeshComponent false))
      (LocalVariables|SetSplineMeshComponent _returnvalue)
      (else
        (bind _returnvalue_2 (AddComponent|AddSplineMeshComponent false))
        (LocalVariables|SetSplineMeshComponent _returnvalue_2)))
    (LocalVariables|SetRemainingMP (- (LocalVariables|GetRemainingMP) (Math|Float|Absolute(Float) (Math|Vector|Distance(Vector) (.Location (Spline|GetLocationandTangentatSplinePoint (Variables|Default|GetSpline) _index "Local")) (.Location (Spline|GetLocationandTangentatSplinePoint (Variables|Default|GetSpline) (+ _index 1) "Local"))))))
    (Utilities|Array|Add (Variables|Default|GetSplineMeshComponents) (LocalVariables|GetSplineMeshComponent))
    (Transformation|DetachFromComponent (LocalVariables|GetSplineMeshComponent) "KeepWorld" "KeepWorld" "KeepWorld" true)
    (SplineMesh|SetStartandEnd (LocalVariables|GetSplineMeshComponent) (.Location (Spline|GetLocationandTangentatSplinePoint (Variables|Default|GetSpline) _index "Local")) (.Tangent (Spline|GetLocationandTangentatSplinePoint (Variables|Default|GetSpline) _index "Local")) (.Location (Spline|GetLocationandTangentatSplinePoint (Variables|Default|GetSpline) (+ _index 1) "Local")) (.Tangent (Spline|GetLocationandTangentatSplinePoint (Variables|Default|GetSpline) (+ _index 1) "Local")) true :!class /Script/Engine.SplineMeshComponent)))

(fn ClearSplineMeshComponents
  (for _array_element (Variables|Default|GetSplineMeshComponents)
    (Components|DestroyComponent _array_element))
  (Utilities|Array|Clear (Variables|Default|GetSplineMeshComponents)))

(fn SplitPathbyFixedDistance
  (params (Path :type Array%20of%20Vectors) (SegmentLengthMax :type Float%20%28double-precision%29))
  (LocalVariables|SetRet (Utilities|Array|MakeArray (Utilities|Array|Get(acopy) Path)))
  (for _index (range 0 (- (Utilities|Array|Length Path) 2))
    (LocalVariables|SetI _index)
    (LocalVariables|SetCurrentPoint (Utilities|Array|Get(acopy) Path (LocalVariables|GetI)))
    (LocalVariables|SetTargetPoint (Utilities|Array|Get(acopy) Path (+ (LocalVariables|GetI) 1)))
    (LocalVariables|SetD (Math|Vector|Distance(Vector) (LocalVariables|GetCurrentPoint) (LocalVariables|GetTargetPoint)))
    (bind _output_get (LocalVariables|SetN (Math|Float|Ceil (/ (Math|Vector|Distance(Vector) (LocalVariables|GetCurrentPoint) (LocalVariables|GetTargetPoint)) SegmentLengthMax))))
    (for _index_2 (range 1 _output_get)
      (Utilities|Array|Add (LocalVariables|GetRet) (Math|Interpolation|VInterpTo (LocalVariables|GetCurrentPoint) (LocalVariables|GetTargetPoint) 1.0 (/ _index_2 (LocalVariables|GetN))))))
  (return (LocalVariables|GetRet)))

(fn DrawPath
  (CallFunction|DrawPathSplineMesh (Variables|Default|GetCachedPath) (Variables|Default|GetMP)))

(fn ClearPawnMovement
  (Development|PrintString (Utilities|String|Append (Utilities|String|ToString(Name) (Variables|Default|GetID)) " : Clear Path"))
  (Variables|Default|SetMoving false)
  (Variables|Default|SetCachedPath (Utilities|Array|MakeArray))
  (CallFunction|ClearSplineMeshComponents)
  (Class|NavMovementComponent|StopActiveMovement (Variables|Character|GetCharacterMovement)))

(fn PawnMovementonTick
  (Utilities|FlowControl|Sequence
    (:then_0
      (if (Variables|Default|GetMoving)
        (Development|PrintString (Utilities|String|Append (Utilities|String|ToString(Name) (Variables|Default|GetID)) " : Moving"))
        (if (Math|Float|NearlyEqual(Float) (Math|Vector|Distance(Vector) (Transformation|GetActorLocation) (Variables|Default|GetGoalLocation)) 0.0 1e+02)
          (CallFunction|StartMovement))))))

(fn UpdateCachedDestination
  (params (Location :type Vector))
  (Development|PrintString (Utilities|String|Append (Utilities|String|ToString(Name) (Variables|Default|GetID)) " : Update Destination"))
  (if (> (Math|Vector|Distance(Vector) Location (Variables|Default|GetCachedDestination)) (Variables|Default|GetMinPathRedrawDistance))
    (bind _output_get (Variables|Default|SetCachedDestination Location))
    (bind _output_get_2 (LocalVariables|SetStartPos (Transformation|GetActorLocation)))
    (bind _returnvalue (Class|NavigationSystemV1|FindPathtoLocationSynchronously _output_get_2 _output_get 0 0))
    (bind _output_get_3 (LocalVariables|SetPathLocalRef (Variables|/Script/NavigationSystem.NavigationPath|GetPathPoints _returnvalue)))
    (bind _segmentedpath (CallFunction|SplitPathbyFixedDistance _output_get_3 25.0))
    (Variables|Default|SetCachedPath _segmentedpath)
    (else
      (return))))

(fn StartMovement
  (Development|PrintString (Utilities|String|Append (Utilities|String|ToString(Name) (Variables|Default|GetID)) " : Move"))
  (if (> (Utilities|Array|Length (Variables|Default|GetCachedPath)) 0)
    (Variables|Default|SetGoalLocation (Utilities|Array|Get(acopy) (Variables|Default|GetCachedPath)))
    (Utilities|Array|RemoveIndex (Variables|Default|GetCachedPath))
    (Variables|Default|SetMoving true)
    (AI|Navigation|SimpleMovetoLocation (Pawn|GetController) (Variables|Default|GetGoalLocation))
    (else
      (Variables|Default|SetMoving false)
      (CallFunction|ClearSplineMeshComponents)
      (Development|PrintString "CachedPath Empty"))))

(fn OnEndTurn)