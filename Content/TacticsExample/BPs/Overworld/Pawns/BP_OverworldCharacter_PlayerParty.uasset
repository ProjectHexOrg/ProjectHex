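; BP_OverworldCharacter_PlayerParty is the overworld pawn representing the player's party in the tactics example.
; It derives its movement points by scaling the party's MP by a fixed factor, both at construction and when a turn ends.
; On turn end it also runs the parent logic and clears pawn movement, while the event graph holds only unused placeholder events.
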(event EventBeginPlay)

(event Collision|EventActorBeginOverlap
  (params (OtherActor :type Actor%20Object%20Reference)))

(event EventTick
  (params (DeltaSeconds :type Float%20%28single-precision%29)))

(fn ConstructionScript
  (|CallParentFunction)
  (Variables|Default|SetMP (* (Utilities|Struct|BreakS_Party (Variables|Default|GetParty)) 2e+02)))

(fn OnEndTurn
  (|CallParentFunction)
  (CallFunction|ClearPawnMovement)
  (Variables|Default|SetMP (* (Utilities|Struct|BreakS_Party (Variables|Default|GetParty)) 2e+02)))