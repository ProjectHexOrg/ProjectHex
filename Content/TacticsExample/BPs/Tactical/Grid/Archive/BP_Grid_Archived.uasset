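; Archived tactical grid actor that builds a square, hexagon or triangle tile grid as instanced static mesh tiles.
; SpawnGrid clears old instances, applies mesh and material from DT_GridShapeData, then derives a snapped center and bottom-left origin per shape.
; Index-based helpers place and scale tiles, with hexagons using parity-offset doubled Y indices and triangles flipping yaw by parity.
; The construction script's SpawnGrid call is disconnected, so nothing here triggers generation.
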(event EventBeginPlay)

(event Collision|EventActorBeginOverlap
  (params (OtherActor :type Actor%20Object%20Reference)))

(event EventTick
  (params (DeltaSeconds :type Float%20%28single-precision%29)))

(fn ConstructionScript)

(fn SpawnGrid
  (params (CenterLocation :type Vector) (TileSize :type Vector) (TileCount :type Vector%202D%20Structure) (TileShape :type E_GridShape%20Enum :default "NewEnumerator0"))
  (bind _returnvalue (CallFunction|GetCurrentShapeData))
  (bind (_meshsize _mesh _meshmaterial _flatmesh _flatmaterial) (Utilities|Struct|BreakS_GridShapeData _returnvalue))
  ;[1 1 1] Init
  (Variables|Default|SetGridCenterLocation CenterLocation)
  (Variables|Default|SetGridTileSize TileSize)
  (Variables|Default|SetGridTileShape TileShape)
  (Variables|Default|SetGridTileCount (Math|Vector2D|MakeVector2D (Math|Conversions|ToFloat(Integer) (Math|Float|Round (.x (Variables|Default|GetGridTileCount)))) (Math|Conversions|ToFloat(Integer) (Math|Float|Round (.y (Variables|Default|GetGridTileCount))))))
  (CallFunction|DestroyGrid)
  ;[1 1 1] Set mesh and texture
  (Components|StaticMesh|SetStaticMesh (Variables|Default|GetInstancedStaticMesh) _flatmesh)
  (Rendering|Material|SetMaterial (Variables|Default|GetInstancedStaticMesh) 0 _flatmaterial)
  ;[1 1 1] Calculate and set center and bottom left location.
  (bind (_center _bottomleft) (CallFunction|CalculateCenterandBottomLeft))
  (Variables|Default|SetGridCenterLocation _center)
  (Variables|Default|SetGridBottomLeftCornerLocation _bottomleft)
  ;[1 1 1] Grid tiling for loop
  (for _index (range 0 (- (Math|Float|Round (.x (Variables|Default|GetGridTileCount))) 1))
    (LocalVariables|SetX _index)
    (if (Utilities|Enum|NotEqual(Enum) (Variables|Default|GetGridTileShape) "NewEnumerator2")
      (for _index_2 (range 0 (- (Math|Float|Round (.y (Variables|Default|GetGridTileCount))) 1))
        (LocalVariables|SetY _index_2)
        (LocalVariables|SetIndex (Math|Vector2D|MakeVector2D (Math|Conversions|ToFloat(Integer) (LocalVariables|GetX)) (Math|Conversions|ToFloat(Integer) (LocalVariables|GetY))))
        ;[1 1 1] Find tile transform
        (LocalVariables|SetTileTransform (Math|Transform|MakeTransform (+ (CallFunction|GetTileLocationfromGridIndex (LocalVariables|GetIndex)) "0.000000,0.000000,2.000000") (CallFunction|GetTileRotationfromGridIndex (LocalVariables|GetIndex)) (/ (Variables|Default|GetGridTileSize) (.MeshSize (Utilities|Struct|BreakS_GridShapeData (CallFunction|GetCurrentShapeData))))))
        ;[1 1 1] Create new tile.
        (Components|InstancedStaticMesh|AddInstance (Variables|Default|GetInstancedStaticMesh) (LocalVariables|GetTileTransform) true))
      (else
        (for _index_3 (range (Math|Integer|SelectInt 0 1 (CallFunction|IsIntEven (LocalVariables|GetX))) (- (* (Math|Float|Round (.y (Variables|Default|GetGridTileCount))) 2) 1))
          (LocalVariables|SetY _index_3)
          (Utilities|FlowControl|Sequence
            (:then_0
              (LocalVariables|SetIndex (Math|Vector2D|MakeVector2D (Math|Conversions|ToFloat(Integer) (LocalVariables|GetX)) (Math|Conversions|ToFloat(Integer) (LocalVariables|GetY))))
              (LocalVariables|SetTileTransform (Math|Transform|MakeTransform (+ (CallFunction|GetTileLocationfromGridIndex (LocalVariables|GetIndex)) "0.000000,0.000000,2.000000") (CallFunction|GetTileRotationfromGridIndex (LocalVariables|GetIndex)) (/ (Variables|Default|GetGridTileSize) (.MeshSize (Utilities|Struct|BreakS_GridShapeData (CallFunction|GetCurrentShapeData))))))
              (Components|InstancedStaticMesh|AddInstance (Variables|Default|GetInstancedStaticMesh) (LocalVariables|GetTileTransform) true))
            (:then_1
              (Math|Integer|IncrementInt _index_3))))))))

(fn GetCurrentShapeData
  (bind _gridtileshape (Variables|Default|GetGridTileShape))
  (bind _returnvalue (Utilities|String|EnumtoString _gridtileshape))
  (bind _returnvalue_2 (Utilities|GetDataTableRow "/Game/Blueprints/Tactical/Grid/GridShapes/DT_GridShapeData.DT_GridShapeData" (Utilities|String|StringToName _returnvalue))
    (:then
      _)
    (:RowNotFound
      (Development|PrintString (Utilities|String|Append "Error - Row Not Found : " _returnvalue) true true "(R=1.000000,G=0.000000,B=0.084660,A=1.000000)" 1e+01)))
  (return _returnvalue_2))

(fn DestroyGrid
  (Components|InstancedStaticMesh|ClearInstances (Variables|Default|GetInstancedStaticMesh)))

(fn CalculateCenterandBottomLeft
  (bind _gridtilecount (Variables|Default|GetGridTileCount))
  (switch Utilities|FlowControl|Switch|SwitchonE_GridShape (Variables|Default|GetGridTileShape)
    (:NewEnumerator1
      ;[1 1 1] Square grids
      (bind _output_get (LocalVariables|SetC (CallFunction|SnapVectortoVector (Variables|Default|GetGridCenterLocation) (Variables|Default|GetGridTileSize))))
      (return _output_get (- (LocalVariables|GetC) (* (/ (- (Variables|Default|GetGridTileCount) (Math|Vector2D|MakeVector2D (Math|Float|SelectFloat 0.0 1.0 (CallFunction|IsFloatEven (.x _gridtilecount))) (Math|Float|SelectFloat 0.0 1.0 (CallFunction|IsFloatEven (.y _gridtilecount))))) 2.0) (Variables|Default|GetGridTileSize)))))
    (:NewEnumerator2
      ;[1 1 1] Hexagon Grids
      (bind _output_get_2 (LocalVariables|SetC (CallFunction|SnapVectortoVector (Variables|Default|GetGridCenterLocation) (* (Variables|Default|GetGridTileSize) "1.500000,1.000000,1.000000"))))
      (return _output_get_2 (- (LocalVariables|GetC) (CallFunction|SnapVectortoVector (* (/ (Variables|Default|GetGridTileCount) "(X=3.000000,Y=2.000000)") (Variables|Default|GetGridTileSize)) (* (Variables|Default|GetGridTileSize) "1.500000,1.000000,1.000000")))))
    (:NewEnumerator3
      ;[1 1 1] Triangle Grids
      (bind _output_get_3 (LocalVariables|SetC (CallFunction|SnapVectortoVector (Variables|Default|GetGridCenterLocation) (* (Variables|Default|GetGridTileSize) "2.000000,1.000000,1.000000"))))
      (return _output_get_3 (- (LocalVariables|GetC) (CallFunction|SnapVectortoVector (* (/ (- (Variables|Default|GetGridTileCount) (Math|Vector2D|MakeVector2D 1.0 1.0)) "(X=2.000000,Y=4.000000)") (Variables|Default|GetGridTileSize)) (* (Variables|Default|GetGridTileSize) "2.000000,1.000000,1.000000")))))))

(fn GetTileRotationfromGridIndex
  (params (GridIndex :type Vector%202D%20Structure))
  (if (Utilities|Enum|Equal(Enum) (Variables|Default|GetGridTileShape) "NewEnumerator3")
    (return (Math|Rotator|MakeRotator 0.0 0.0 (+ (Math|Float|SelectFloat 1.8e+02 0.0 (CallFunction|IsFloatEven (.x GridIndex))) (Math|Float|SelectFloat 1.8e+02 0.0 (CallFunction|IsFloatEven (.y GridIndex))))))
    (else
      (return "0, 0, 0"))))

(fn GetTileLocationfromGridIndex
  (params (GridIndex :type Vector%202D%20Structure))
  (return (+ (Variables|Default|GetGridBottomLeftCornerLocation) (* (Variables|Default|GetGridTileSize) (* GridIndex (Utilities|Select :Index (Variables|Default|GetGridTileShape) :NewEnumerator0 "" :NewEnumerator1 "(X=1.000000,Y=1.000000)" :NewEnumerator2 "(X=0.750000,Y=0.500000)" :NewEnumerator3 "(X=1.000000,Y=0.500000)"))))))