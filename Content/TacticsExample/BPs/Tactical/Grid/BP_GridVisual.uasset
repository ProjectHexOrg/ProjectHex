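; Visual actor for the tactics grid, drawing tiles through two BP_GridMeshInstance child actors: a flat overlay and a tactical view colored by tile type.
; Tile updates re-add instances, showing only walkable tiles on the overlay.
; Tactical tiles stretch vertically down to the lowest grid Z.
; Tactical mode hides actors tagged NotTactical and defers mesh updates while off, regenerating all tiles on enable when flagged.
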(event EventBeginPlay
  (Actor|Tick|SetActorTickEnabled false))

(event Collision|EventActorBeginOverlap
  (params (OtherActor :type Actor%20Object%20Reference)))

(event EventTick
  (params (DeltaSeconds :type Float%20%28single-precision%29)))

(fn ConstructionScript)

(fn InitGridVisual
  (params (Grid :type BP%20Grid%20Manager%20Object%20Reference))
  ;[1 1 1] Setup references.
  (Variables|Default|SetGrid Grid)
  (Variables|Default|SetGridMeshInstance (.AsBP%20Grid%20Mesh%20Instance (Utilities|Casting|CastToBP_GridMeshInstance (Variables|/Script/Engine.ChildActorComponent|GetChildActor (Variables|Default|GetChildActor_GridMeshInstance)))))
  (Variables|Default|SetGridMeshInstance_Tactical (.AsBP%20Grid%20Mesh%20Instance (Utilities|Casting|CastToBP_GridMeshInstance (Variables|/Script/Engine.ChildActorComponent|GetChildActor (Variables|Default|GetChildActor_GridMeshInstance_Tactical)))))
  ;[1 1 1] Setup grid components.
  (Default|InitGridMeshInstance (Variables|Default|GetGridMeshInstance) (.flatmesh (Default|GetCurrentShapeData (Variables|Default|GetGrid))) (.flatmaterial (Default|GetCurrentShapeData (Variables|Default|GetGrid))) "QueryOnly" false)
  (Default|InitGridMeshInstance (Variables|Default|GetGridMeshInstance_Tactical) (.mesh (Default|GetCurrentShapeData (Variables|Default|GetGrid))) (.meshmaterial (Default|GetCurrentShapeData (Variables|Default|GetGrid))) "QueryOnly" true)
  ;[1 1 1] Center grid in world.
  (Transformation|SetActorLocation "0, 0, 0" false false)
  (CallFunction|SetOffsetfromGround (Variables|Default|GetOffsetFromGround))
  (CallFunction|SetGridLowestZ 999999.0)
  (CallFunction|SetIsTactical (Variables|Default|GetIs%20Tactical)))

(fn SetOffsetfromGround
  (params (Offset :type Float%20%28double-precision%29))
  (Variables|Default|SetOffsetFromGround Offset)
  (Transformation|SetRelativeLocation (Variables|Default|GetChildActor_GridMeshInstance) (Math|Vector|MakeVector 0.0 0.0 (Variables|Default|GetOffsetFromGround)) false false))

(fn DestroyGridVisual
  (bind _gridmeshinstance (Variables|Default|GetGridMeshInstance))
  (bind _gridmeshinstance_tactical (Variables|Default|GetGridMeshInstance_Tactical))
  ;[1 1 1] Clears instances on GridMeshInstance components.
  (Utilities|FlowControl|Sequence
    (:then_0
      (Utilities|IsValid _gridmeshinstance
        (:Is%20Valid
          (Default|ClearInstances _gridmeshinstance))))
    (:then_1
      (Utilities|IsValid _gridmeshinstance_tactical
        (:Is%20Valid
          (Default|ClearInstances _gridmeshinstance_tactical))))
    (:then_2
      (CallFunction|SetGridLowestZ 999999.0) ; Reset lowest Z for tactical grid generation.
    )))

(fn UpdateTileVisual
  (params (Data :type S%20Tile%20Data%20Structure))
  ;[1 1 1] Update tile visuals based on Data
  (Utilities|FlowControl|Sequence
    (:then_0
      (Default|RemoveInstance (Variables|Default|GetGridMeshInstance) (.index Data))
      (if (CallFunction|IsTileTypeWalkable (.type Data))
        (Default|AddInstance (Variables|Default|GetGridMeshInstance) (.index Data) (.transform Data) (.type Data) (.states Data))))
    (:then_1
      (CallFunction|UpdateTileVisualTactical Data))))

(fn UpdateTileVisualTactical
  (params (Data :type S%20Tile%20Data%20Structure))
  (bind _grid (Variables|Default|GetGrid))
  (bind (_location _rotation _scale) (Math|Transform|BreakTransform (.transform Data)))
  (bind _location_2 (Math|Transform|BreakTransform (.transform Data)))
  (bind _data (Default|GetCurrentShapeData _grid))
  (bind _meshsize (Utilities|Struct|BreakS_GridShapeData _data))
  (bind _z (Math|Vector|BreakVector _location_2))
  (bind _z_2 (Math|Vector|BreakVector _meshsize))
  (Utilities|FlowControl|Sequence
    (:then_0
      (if (< _z (Variables|Default|GetGridLowestZ))
        (CallFunction|SetGridLowestZ _z)))
    (:then_1
      (if (Variables|Default|GetIs%20Tactical)
        (Default|RemoveInstance (Variables|Default|GetGridMeshInstance_Tactical) (.index Data))
        (if (Utilities|Enum|NotEqual(Enum) (.type Data) "NewEnumerator0")
          (Default|AddInstance (Variables|Default|GetGridMeshInstance_Tactical) (.index Data) (Math|Transform|MakeTransform _location _rotation (Math|Vector|MakeVector (.x _scale) (.y _scale) (/ (+ (- (.Z (Math|Vector|BreakVector (.Location (Math|Transform|BreakTransform (.transform Data))))) (Variables|Default|GetGridLowestZ)) _z_2) _z_2))) (.type Data) (.states Data)))
        (else
          (Variables|Default|SetRegenerateTacticalOnEnable true))))))

(fn SetGridLowestZ
  (params (Z :type Float%20%28double-precision%29))
  (Variables|Default|SetGridLowestZ Z)
  (Variables|Default|SetRegenerateTacticalOnEnable true))

(fn SetIsTactical
  (params (IsTactical :type Boolean))
  (Variables|Default|SetIs%20Tactical IsTactical)
  (Development|SetHiddeninGame (Variables|Default|GetChildActor_GridMeshInstance_Tactical) (not (Variables|Default|GetIs%20Tactical)) false)
  (bind _outactors (Actor|GetAllActorswithTag "NotTactical"))
  (for _array_element _outactors
    (Rendering|SetActorHiddenInGame _array_element (Variables|Default|GetIs%20Tactical)))
  (if (and (Variables|Default|GetIs%20Tactical) (Variables|Default|GetRegenerateTacticalOnEnable))
    (Variables|Default|SetRegenerateTacticalOnEnable false)
    (bind _values (Utilities|Map|Values (Variables|/Game/Blueprints/Tactical/Grid/BP_GridManager.BP_GridManager_C|GetGridTiles (Variables|Default|GetGrid))))
    (for _array_element_2 _values
      (CallFunction|UpdateTileVisualTactical _array_element_2))))