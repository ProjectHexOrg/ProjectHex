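; BP_GridManager builds and owns a tactical grid of square, hexagon or triangle tiles, stored in a map by index.
; SpawnGrid lays out tiles, optionally sphere-tracing the environment and BP_GridModifier actors for height and type.
; It converts between indices, world locations and cursor hits, and tracks tile states with a reverse state-to-index map.
; Child-actor BP_GridVisual renders tile changes; two BP_GridPathfinding child actors receive a grid reference.
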(event EventBeginPlay)

(fn ConstructionScript
  (Variables|GridGeneration|SetGridVisual (.AsBP%20Grid%20Visual (Utilities|Casting|CastToBP_GridVisual (Variables|/Script/Engine.ChildActorComponent|GetChildActor (Variables|Default|GetChildActor_GridVisual)))))
  (bind _output_get (Variables|GridGeneration|SetGridPathfinding (.AsBP%20Grid%20Pathfinding (Utilities|Casting|CastToBP_GridPathfinding (Variables|/Script/Engine.ChildActorComponent|GetChildActor (Variables|Default|GetChildActor_GridPathfinding))))))
  (Variables|/Game/Blueprints/Tactical/Grid/BP_GridPathfinding.BP_GridPathfinding_C|SetGrid _output_get self)
  (bind _output_get_2 (Variables|GridGeneration|SetGridPathfinding_ReachableTiles (.AsBP%20Grid%20Pathfinding (Utilities|Casting|CastToBP_GridPathfinding (Variables|/Script/Engine.ChildActorComponent|GetChildActor (Variables|Default|GetChildActor_GridPathfinding_ReachableTiles))))))
  (Variables|/Game/Blueprints/Tactical/Grid/BP_GridPathfinding.BP_GridPathfinding_C|SetGrid _output_get_2 self))

(fn SpawnGrid
  (params (CenterLocation :type Vector) (TileSize :type Vector) (TileCount :type Int%20Point%20Structure) (TileShape :type E_GridShape%20Enum :default "NewEnumerator0") (UseEnvironment :type Boolean))
  ;[1 1 1] Init
  (Variables|BasicParameters|SetGridCenterLocation CenterLocation)
  (Variables|BasicParameters|SetGridTileSize TileSize)
  (Variables|BasicParameters|SetGridTileShape TileShape)
  (Variables|BasicParameters|SetGridTileCount TileCount)
  (Variables|BasicParameters|SetUseEnvironment UseEnvironment)
  (Utilities|FlowControl|Sequence
    (:then_0
      (GridGeneration|DestroyGrid)
      ;[1 1 1] Set mesh and texture
      (Default|InitGridVisual (Variables|GridGeneration|GetGridVisual) self)
      ;[1 1 1] Calculate and set center and bottom left location.
      (bind (_center _bottomleft) (Utility_Calcs|CalculateCenterandBottomLeft))
      (Variables|BasicParameters|SetGridCenterLocation _center)
      (Variables|BasicParameters|SetGridBottomLeftCornerLocation _bottomleft)
      ;[1 1 1] Grid tiling for loop
      (for _index (range 0 (- (.x (Variables|BasicParameters|GetGridTileCount)) 1))
        (LocalVariables|SetX _index)
        (if (Utilities|Enum|NotEqual(Enum) (Variables|BasicParameters|GetGridTileShape) "NewEnumerator2")
          (for _index_2 (range 0 (- (.y (Variables|BasicParameters|GetGridTileCount)) 1))
            (LocalVariables|SetY _index_2)
            (LocalVariables|SetIndex (Utilities|Struct|MakeIntPoint (Math|Float|Truncate (Math|Conversions|ToFloat(Integer) (LocalVariables|GetX))) (Math|Float|Truncate (Math|Conversions|ToFloat(Integer) (LocalVariables|GetY)))))
            ;[1 1 1] Find tile transform
            (bind _output_get (LocalVariables|SetTileTransform (Math|Transform|MakeTransform (Utility|GetTileLocationfromGridIndex (LocalVariables|GetIndex)) (Utility|GetTileRotationfromGridIndex (LocalVariables|GetIndex)) (Utility|GetTileScale))))
            ;[1 1 1] Set tile location based on environment.
            (GridGeneration|AddGridTileCheckUseEnvironment (LocalVariables|GetIndex) _output_get))
          (else
            (for _index_3 (range (Math|Integer|SelectInt 0 1 (CallFunction|IsIntEven (LocalVariables|GetX))) (- (* (.y (Variables|BasicParameters|GetGridTileCount)) 2) 1))
              (LocalVariables|SetY _index_3)
              (Utilities|FlowControl|Sequence
                (:then_0
                  (LocalVariables|SetIndex (Utilities|Struct|MakeIntPoint (Math|Float|Truncate (Math|Conversions|ToFloat(Integer) (LocalVariables|GetX))) (Math|Float|Truncate (Math|Conversions|ToFloat(Integer) (LocalVariables|GetY)))))
                  (bind _output_get_2 (LocalVariables|SetTileTransform (Math|Transform|MakeTransform (Utility|GetTileLocationfromGridIndex (LocalVariables|GetIndex)) (Utility|GetTileRotationfromGridIndex (LocalVariables|GetIndex)) (Utility|GetTileScale))))
                  (GridGeneration|AddGridTileCheckUseEnvironment (LocalVariables|GetIndex) _output_get_2))
                (:then_1
                  (Math|Integer|IncrementInt _index_3))))))))
    (:then_1
      (Default|CallOnGridGenerated))))

(fn GetCurrentShapeData
  (return (CallFunction|GetShapeData (Variables|BasicParameters|GetGridTileShape))))

(fn DestroyGrid
  (Utilities|Map|Clear (Variables|GridGeneration|GetGridTiles))
  (Default|DestroyGridVisual (Variables|GridGeneration|GetGridVisual))
  (Default|CallOnGridDestroyed))

(fn CalculateCenterandBottomLeft
  (bind _gridtilecount (Variables|BasicParameters|GetGridTileCount))
  (switch Utilities|FlowControl|Switch|SwitchonE_GridShape (Variables|BasicParameters|GetGridTileShape)
    (:NewEnumerator1
      ;[1 1 1] Square grids
      (bind _output_get (LocalVariables|SetC (CallFunction|SnapVectortoVector (Variables|BasicParameters|GetGridCenterLocation) (Variables|BasicParameters|GetGridTileSize))))
      (return _output_get (- (LocalVariables|GetC) (* (/ (- (Variables|BasicParameters|GetGridTileCount) (Math|Vector2D|MakeVector2D (Math|Float|SelectFloat 0.0 1.0 (CallFunction|IsFloatEven (Math|Conversions|ToFloat(Integer) (.x _gridtilecount)))) (Math|Float|SelectFloat 0.0 1.0 (CallFunction|IsFloatEven (Math|Conversions|ToFloat(Integer) (.y _gridtilecount)))))) 2.0) (Variables|BasicParameters|GetGridTileSize)))))
    (:NewEnumerator2
      ;[1 1 1] Hexagon Grids
      (bind _output_get_2 (LocalVariables|SetC (CallFunction|SnapVectortoVector (Variables|BasicParameters|GetGridCenterLocation) (* (Variables|BasicParameters|GetGridTileSize) "1.500000,1.000000,1.000000"))))
      (return _output_get_2 (- (LocalVariables|GetC) (CallFunction|SnapVectortoVector (* (Math|Conversions|ToVector2D(IntPoint) (/ (Variables|BasicParameters|GetGridTileCount) (Utilities|Struct|MakeIntPoint 3 2))) (Variables|BasicParameters|GetGridTileSize)) (* (Variables|BasicParameters|GetGridTileSize) "1.500000,1.000000,1.000000")))))
    (:NewEnumerator3
      ;[1 1 1] Triangle Grids
      (bind _output_get_3 (LocalVariables|SetC (CallFunction|SnapVectortoVector (Variables|BasicParameters|GetGridCenterLocation) (* (Variables|BasicParameters|GetGridTileSize) "2.000000,1.000000,1.000000"))))
      (return _output_get_3 (- (LocalVariables|GetC) (CallFunction|SnapVectortoVector (* (Math|Conversions|ToVector2D(IntPoint) (/ (- (Variables|BasicParameters|GetGridTileCount) (Utilities|Struct|MakeIntPoint 1 1)) (Utilities|Struct|MakeIntPoint 2 4))) (Variables|BasicParameters|GetGridTileSize)) (* (Variables|BasicParameters|GetGridTileSize) "2.000000,1.000000,1.000000")))))))

(fn GetTileRotationfromGridIndex
  (params (GridIndex :type Int%20Point%20Structure))
  (if (Utilities|Enum|Equal(Enum) (Variables|BasicParameters|GetGridTileShape) "NewEnumerator3")
    (return (Math|Rotator|MakeRotator 0.0 0.0 (+ (Math|Float|SelectFloat 1.8e+02 0.0 (CallFunction|IsIntEven (.x GridIndex))) (Math|Float|SelectFloat 1.8e+02 0.0 (CallFunction|IsIntEven (.y GridIndex))))))
    (else
      (return "0, 0, 0"))))

(fn GetTileLocationfromGridIndex
  (params (GridIndex :type Int%20Point%20Structure))
  (return (+ (Variables|BasicParameters|GetGridBottomLeftCornerLocation) (* (Variables|BasicParameters|GetGridTileSize) (* GridIndex (Utilities|Select :Index (Variables|BasicParameters|GetGridTileShape) :NewEnumerator0 "" :NewEnumerator1 "(X=1.000000,Y=1.000000)" :NewEnumerator2 "(X=0.750000,Y=0.500000)" :NewEnumerator3 "(X=1.000000,Y=0.500000)"))))))

(fn TraceforGround
  (params (Location :type Vector))
  (LocalVariables|SetRadius (/ (.x (Variables|BasicParameters|GetGridTileSize)) (Math|Float|SelectFloat 5.0 3.0 (Utilities|Enum|Equal(Enum) (Variables|BasicParameters|GetGridTileShape) "NewEnumerator3"))))
  (LocalVariables|SetIsHeightFound false)
  (bind _outhits (Collision|MultiSphereTraceByChannel (+ Location "0.000000,0.000000,1000.000000") (- Location "0.000000,0.000000,1000.000000") (LocalVariables|GetRadius) "TraceTypeQuery3" false 0 "None"))
  (if (> (Utilities|Array|Length _outhits) 0)
    (LocalVariables|SetHitType "NewEnumerator1")
    (for _array_element _outhits
      (bind _asbp_grid_modifier (Utilities|Casting|CastToBP_GridModifier (.HitActor (Collision|BreakHitResult _array_element)))
        (:then
          (LocalVariables|SetHitType (Variables|/Game/Blueprints/Tactical/Grid/BP_GridModifier.BP_GridModifier_C|GetType _asbp_grid_modifier))
          (if (Variables|/Game/Blueprints/Tactical/Grid/BP_GridModifier.BP_GridModifier_C|GetUseForTileHeight _asbp_grid_modifier)
            (LocalVariables|SetIsHeightFound true)
            (LocalVariables|SetRetZ (Math|Float|SnapToGrid(Float) (- (.Z (Math|Vector|BreakVector (.Location (Collision|BreakHitResult _array_element)))) (LocalVariables|GetRadius)) (.z (Variables|BasicParameters|GetGridTileSize))) :!label _label)))
        (:CastFailed
          (if (not (LocalVariables|GetIsHeightFound))
            (goto _label)))))
    (return (Math|Vector|MakeVector (.x Location) (.y Location) (LocalVariables|GetRetZ)) (LocalVariables|GetHitType))
    (else
      (return Location "NewEnumerator0"))))

(fn AddGridTile
  (params (Data :type S%20Tile%20Data%20Structure))
  (Utilities|Map|Add (Variables|GridGeneration|GetGridTiles) (.index Data) Data)
  (Default|UpdateTileVisual (Variables|GridGeneration|GetGridVisual) Data)
  (Default|CallOnTileDataUpdated (.index Data)))

(fn GetCursorLocationonGrid
  (params (PlayerIndex :type Integer))
  (bind _returnvalue (Game|GetPlayerController PlayerIndex))
  (bind _gridcenterlocation (Variables|BasicParameters|GetGridCenterLocation))
  (bind _returnvalue_2 (Game|GetPlayerController PlayerIndex))
  (bind _returnvalue_3 (Class|KismetMathLibrary|MakePlanefromPointandNormal _gridcenterlocation "0.000000,0.000000,1.000000"))
  (bind (_hitresult _returnvalue_4) (Game|Player|GetHitResultUnderCursorbyChannel _returnvalue "TraceTypeQuery4" false))
  (bind _returnvalue_5 (Game|GetPlayerController PlayerIndex))
  (bind (_hitresult_2 _returnvalue_6) (Game|Player|GetHitResultUnderCursorbyChannel _returnvalue_5 "TraceTypeQuery3" false))
  (bind (_worldlocation _worlddirection) (Game|Player|ConvertMouseLocationToWorldSpace _returnvalue_2))
  (bind _returnvalue_7 (* _worlddirection 999999.0))
  (bind _returnvalue_8 (+ _worldlocation _returnvalue_7))
  (bind (_t _intersection _returnvalue_9) (Class|KismetMathLibrary|LinePlaneIntersection _worldlocation _returnvalue_8 _returnvalue_3))
  ;[1 1 1] Check for trace against grid.
  (if _returnvalue_4
    (return (.Location (Collision|BreakHitResult _hitresult)))
    (else
      (if (Variables|BasicParameters|GetUseEnvironment)
        ;[1 1 1] If using the environment check for trace against the ground and modifiers.
        (if _returnvalue_6
          (return (.Location (Collision|BreakHitResult _hitresult_2)))
          (else
            _)))
      ;[1 1 1] If not using the environment or the environmnent was not hit, check for hits against an infinite plane.
      (if _returnvalue_9
        (return _intersection)
        (else
          (return "-99999.000000,-99999.000000,-99999.000000"))))))

(fn SetGridOffsetfromGround
  (params (Offset :type Float%20%28double-precision%29))
  (Default|SetOffsetfromGround (Variables|GridGeneration|GetGridVisual) Offset))

(fn GetTileIndexfromWorldLocation
  (params (Location :type Vector))
  (LocalVariables|SetLocationOnGrid (- Location (Variables|BasicParameters|GetGridBottomLeftCornerLocation)))
  (switch Utilities|FlowControl|Switch|SwitchonE_GridShape (Variables|BasicParameters|GetGridTileShape)
    (:NewEnumerator0
      (return (Utilities|Struct|MakeIntPoint -999 -999)))
    (:NewEnumerator1
      (bind _output_get (LocalVariables|SetSnappedLocationOnGrid (Math|Conversions|ToVector2D(Vector) (CallFunction|SnapVectortoVector (LocalVariables|GetLocationOnGrid) (Variables|BasicParameters|GetGridTileSize)))))
      (return (Class|KismetMathLibrary|ToIntPoint(Vector2D) (/ _output_get (Math|Conversions|ToVector2D(Vector) (Variables|BasicParameters|GetGridTileSize))))))
    (:NewEnumerator2
      (bind _output_get_2 (LocalVariables|SetSnappedLocationOnGrid (Math|Conversions|ToVector2D(Vector) (CallFunction|SnapVectortoVector (* (LocalVariables|GetLocationOnGrid) "1.000000,2.000000,1.000000") (* (Variables|BasicParameters|GetGridTileSize) "0.750000,0.250000,1.000000")))))
      (bind _output_get_3 (LocalVariables|SetTempIndex (/ _output_get_2 (* (Math|Conversions|ToVector2D(Vector) (Variables|BasicParameters|GetGridTileSize)) "(X=0.750000,Y=1.000000)"))))
      (if (CallFunction|IsFloatEven (.x _output_get_3))
        (return (Utilities|Struct|MakeIntPoint (Math|Float|Truncate (.x (LocalVariables|GetTempIndex))) (* (Math|Float|Round (/ (.y (LocalVariables|GetTempIndex)) 2.0)) 2)))
        (else
          (return (Utilities|Struct|MakeIntPoint (Math|Float|Truncate (.x (LocalVariables|GetTempIndex))) (+ (* (Math|Float|Round (- (/ (.y (LocalVariables|GetTempIndex)) 2.0) 0.5)) 2) 1))))))
    (:NewEnumerator3
      (bind _output_get_4 (LocalVariables|SetSnappedLocationOnGrid (Math|Conversions|ToVector2D(Vector) (CallFunction|SnapVectortoVector (LocalVariables|GetLocationOnGrid) (/ (Variables|BasicParameters|GetGridTileSize) "1.000000,2.000000,1.000000")))))
      (return (Class|KismetMathLibrary|ToIntPoint(Vector2D) (* (/ _output_get_4 (Math|Conversions|ToVector2D(Vector) (Variables|BasicParameters|GetGridTileSize))) "(X=1.000000,Y=2.000000)"))))))

(fn GetTileIndexUnderCursor
  (params (PlayerIndex :type Integer))
  (bind _location (Utility_Traces|GetCursorLocationonGrid PlayerIndex))
  (bind _index (Utility|GetTileIndexfromWorldLocation _location))
  (return _index))

(fn AddStatetoTile
  (params (Index :type Int%20Point%20Structure) (State :type E_TileState%20Enum :default "NewEnumerator0"))
  (bind _gridtiles (Variables|GridGeneration|GetGridTiles))
  (bind (_value _returnvalue) (Utilities|Map|Find _gridtiles Index))
  (if _returnvalue
    (bind _output_get (LocalVariables|SetData _value))
    (bind _returnvalue_2 (Utilities|Array|AddUnique (.states _output_get) State))
    (if (>= _returnvalue_2 0)
      (Utilities|Map|Add (Variables|GridGeneration|GetGridTiles) (.index (LocalVariables|GetData)) (LocalVariables|GetData))
      ;[1 1 1] Remove index from tile/state map for faster access.
      (bind _indexes (States|GetAllTileswithState State))
      (Utilities|Array|Add _indexes Index)
      (Utilities|Map|Add (Variables|GridGeneration|GetTileStateToIndexes) State (Utilities|Struct|MakeS_IntPointArray _indexes))
      (Default|UpdateTileVisual (Variables|GridGeneration|GetGridVisual) (LocalVariables|GetData))
      (Default|CallOnTileStateUpdated Index))))

(fn RemoveStatefromTile
  (params (Index :type Int%20Point%20Structure) (State :type E_TileState%20Enum :default "NewEnumerator0"))
  (bind _gridtiles (Variables|GridGeneration|GetGridTiles))
  (bind (_value _returnvalue) (Utilities|Map|Find _gridtiles Index))
  (if _returnvalue
    (bind _output_get (LocalVariables|SetData _value))
    (bind _returnvalue_2 (Utilities|Array|RemoveItem (.states _output_get) State))
    (if _returnvalue_2
      (Utilities|Map|Add (Variables|GridGeneration|GetGridTiles) (.index (LocalVariables|GetData)) (LocalVariables|GetData))
      (bind _indexes (States|GetAllTileswithState State))
      (Utilities|Array|RemoveItem _indexes Index)
      (Utilities|Map|Add (Variables|GridGeneration|GetTileStateToIndexes) State (Utilities|Struct|MakeS_IntPointArray _indexes))
      (Default|UpdateTileVisual (Variables|GridGeneration|GetGridVisual) (LocalVariables|GetData))
      (Default|CallOnTileStateUpdated Index))))

(fn IsIndexValid
  (params (Index :type Int%20Point%20Structure))
  (return (Utilities|Map|Contains (Variables|GridGeneration|GetGridTiles) Index)))

(fn GetTileScale
  (return (/ (Variables|BasicParameters|GetGridTileSize) (.MeshSize (Utilities|Struct|BreakS_GridShapeData (Utility|GetCurrentShapeData))))))

(fn RemoveGridTile
  (params (Index :type Int%20Point%20Structure))
  (bind _returnvalue (Utilities|Map|Remove (Variables|GridGeneration|GetGridTiles) Index))
  (if _returnvalue
    (Default|UpdateTileVisual (Variables|GridGeneration|GetGridVisual) (Utilities|Struct|MakeS_TileData Index "0.000000,0.000000,0.000000|0.000000,0.000000,0.000000|1.000000,1.000000,1.000000" "NewEnumerator0" "NewEnumerator0" 0))
    (Default|CallOnTileDataUpdated Index)))

(fn AddGridTileCheckUseEnvironment
  (params (Index :type Int%20Point%20Structure) (TileTransform :type Transform))
  ;[1 1 1] Set tile location based on environment.
  (if (Variables|BasicParameters|GetUseEnvironment)
    (bind (_outlocation _tiletype) (Utility_Traces|TraceforGround (.location TileTransform)))
    (GridGeneration|AddGridTile (Utilities|Struct|MakeS_TileData Index (Math|Transform|MakeTransform _outlocation (.rotation TileTransform) (.scale TileTransform)) _tiletype "NewEnumerator0" 0))
    (else
      ;[1 1 1] Create new tile. When not using environment.
      (GridGeneration|AddGridTile (Utilities|Struct|MakeS_TileData Index TileTransform "NewEnumerator1" "NewEnumerator0" 0)))))

(fn GetAllTileswithState
  (params (State :type E_TileState%20Enum :default "NewEnumerator0"))
  (return (.intpointarray (.Value (Utilities|Map|Find (Variables|GridGeneration|GetTileStateToIndexes) State)))))

(fn ClearStatefromTiles
  (params (State :type E_TileState%20Enum :default "NewEnumerator0"))
  (bind _indexes (States|GetAllTileswithState State))
  (for _array_element _indexes
    (States|RemoveStatefromTile _array_element State)))

(fn IsTileWalkable
  (params (Index :type Int%20Point%20Structure))
  (return (CallFunction|IsTileTypeWalkable (.Type (Utilities|Struct|BreakS_TileData (.Value (Utilities|Map|Find (Variables|GridGeneration|GetGridTiles) Index)))))))

(fn CenterCameraonGridTile
  (params (Index :type Int%20Point%20Structure))
  (bind _tilelocation (Utility|GetTileLocationfromGridIndex Index))
  (switch Utilities|FlowControl|Switch|SwitchonE_GridContext (Variables|BasicParameters|GetContext)
    (:NewEnumerator0
      (bind _asbp_tactical_pawn (Utilities|Casting|CastToBP_TacticalPawn (Game|Player|GetPlayerPawn 0)))
      (LocalVariables|SetTacticalPawn _asbp_tactical_pawn)
      (Variables|/Game/Blueprints/Tactical/Player/BP_TacticalPawn.BP_TacticalPawn_C|SetTargetLocation (LocalVariables|GetTacticalPawn) (Math|Vector|MakeVector (.x _tilelocation) (.y _tilelocation) (.z (Variables|/Game/Blueprints/Tactical/Player/BP_TacticalPawn.BP_TacticalPawn_C|GetTargetLocation (LocalVariables|GetTacticalPawn))))))))