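; BP_Unit is the grid-based tactics unit, with mesh, animation and stats loaded by UnitType.
; A timeline walks it tile by tile along paths, hopping across height changes.
; It manages HP, AP, MP and ability cooldowns through turn, combat and overworld resets, broadcasting changes.
; Ability hits change stats immediately but defer numbers, HP bar and hit or death animations until the ability animation reaches its tile.
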(event Custom|Event_FollowPath
  (params (Path :type Array%20of%20Int%20Point%20Structures))
  (if (> (Utilities|Array|Length Path) 0)
    (Variables|Pathing|SetCurrentPathToFollow Path)
    (Default|CallOnUnitStartedWalking self)
    (CallFunction|ContinuetoFollowPath)))

(event Custom|ContinueToFollowPath
  (bind _self self)
  (bind _grid (Variables|Grid|GetGrid))
  (bind _timeline_unitmovement (Variables|Default|GetTimeline_UnitMovement))
  (bind _currentpathtofollow (Variables|Pathing|GetCurrentPathToFollow))
  (bind _currentpathtofollow_2 (Variables|Pathing|GetCurrentPathToFollow))
  (bind _output (Utilities|Array|Get(acopy) _currentpathtofollow))
  (bind _output_2 (Utilities|Array|Get(acopy) _currentpathtofollow_2))
  (bind _gridtiles (Variables|/Game/Blueprints/Tactical/Grid/BP_GridManager.BP_GridManager_C|GetGridTiles _grid))
  (bind _value (Utilities|Map|Find _gridtiles _output_2))
  (bind _transform (Utilities|Struct|BreakS_TileData _value))
  (if (and (> (Utilities|Array|Length (Variables|Pathing|GetCurrentPathToFollow)) 0) (not (Variables|Pathing|GetCancelPath)))
    (Animation|SetAnimationState "NewEnumerator1") ; Set animation to walking since we are moving.
    ;[1 1 1] Set location and rotation to interpolate between for this step.
    (Variables|Pathing|SetPreviousTransform (Transformation|GetActorTransform))
    (Variables|Pathing|SetNextTransform (Math|Transform|MakeTransform (.location _transform) (Math|Rotator|MakeRotator 0.0 0.0 (.yaw (Math|Rotator|FindLookatRotation (.location (Variables|Pathing|GetPreviousTransform)) (.location _transform)))) "1.000000,1.000000,1.000000"))
    (Components|Timeline|SetPlayRate _timeline_unitmovement (/ (Components|Timeline|GetTimelineLength _timeline_unitmovement) (Variables|Pathing|GetMoveDurationPerTile)))
    ;[1 1 1] Move from current tile to next tile using timeline.
    (bind (_direction _locationalpha _rotationalpha _jump) (Timeline|Timeline_UnitMovement PlayFromStart)
      (:Update
        (Transformation|SetActorLocationAndRotation (+ (Math|Vector|Lerp(Vector) (.location (Variables|Pathing|GetPreviousTransform)) (.location (Variables|Pathing|GetNextTransform)) _locationalpha) (Math|Vector|MakeVector 0.0 0.0 (Math|Float|SelectFloat 0.0 _jump (Math|Float|NearlyEqual(Float) (.z (.location (Variables|Pathing|GetPreviousTransform))) (.z (.location (Variables|Pathing|GetNextTransform))) 5.0)))) (Math|Rotator|Lerp(Rotator) (.rotation (Variables|Pathing|GetPreviousTransform)) (.rotation (Variables|Pathing|GetNextTransform)) _rotationalpha true)))
      (:Finished
        (Default|CallOnUnitReachedNewTile _self _output)
        (Default|CallOnUnitFinishedWalkingTile _self _output)
        (Utilities|Array|RemoveIndex (Variables|Pathing|GetCurrentPathToFollow))
        (CallFunction|ContinuetoFollowPath)))
    (else
      (Animation|SetAnimationState "NewEnumerator0") ; Path completed return to idle animation
      (Default|CallOnUnitFinishedWalking)
      (Variables|Pathing|SetCancelPath false))))

(event Custom|Debug_RespawnAfterDeath
  (Utilities|FlowControl|Delay 2.0)
  (Stats|SetCurrentHP (.HP_Max (Utilities|Struct|BreakS_UnitData_Stats (Utilities|Struct|BreakS_UnitData (Variables|UnitData|GetUnitData)))) true)
  (Animation|SetAnimationState "NewEnumerator5"))

(event Custom|Debug_HideUnitAfterDeath
  (Utilities|FlowControl|Delay 2.0)
  (if (not (Stats|IsAlive))
    (Transformation|SetActorLocation "-99999.000000,-99999.000000,-99999.000000" false false)))

(event EventBeginPlay
  (Animation|SetAnimationState "NewEnumerator0")
  (bind _asw_hpbar (Utilities|Casting|CastToW_HPBar (UserInterface|GetUserWidgetObject (Variables|Default|GetWidget_HPBar))))
  (bind _output_get (Variables|UI|SetHPBar _asw_hpbar))
  (Default|EventSetUnit _output_get self))

(fn ConstructionScript
  (bind _unitdata (CallFunction|GetDefaultUnitData (Variables|UnitData|GetUnitType)))
  (UnitData|SetUnitData _unitdata))

(fn UpdateVisualifHoveredorSelected
  (Rendering|Material|SetVectorParameterValueonMaterials (Variables|Default|GetSkeletalMesh) "ColorMultiply" (Math|Conversions|ToVector(LinearColor) (* (* (Math|Color|SelectColor "(R=1.000000,G=0.161458,B=0.174373,A=1.000000)" "(R=1.000000,G=1.000000,B=1.000000,A=1.000000)" (Variables|Grid|GetIsSelected)) (Math|Float|SelectFloat 1.0 2.5 (Variables|Grid|GetIsHovered))) (Math|Float|SelectFloat 1.0 2.5 (Variables|Grid|GetIsSelected))))))

(fn SetIsHovered
  (params (IsHovered :type Boolean))
  (Variables|Grid|SetIsHovered IsHovered)
  (Hovered&Selected|UpdateVisualifHoveredorSelected)
  (Default|CallOnUnitHoveredChanged self))

(fn SetIsSelected
  (params (IsSelected :type Boolean))
  (Variables|Grid|SetIsSelected IsSelected)
  (Hovered&Selected|UpdateVisualifHoveredorSelected)
  (Default|CallOnUnitSelectedChanged self))

(fn SetUnitData
  (params (S_UnitData :type S%20Unit%20Data%20Structure%20%28by%20ref%29))
  (bind _skeletalmesh (Variables|Default|GetSkeletalMesh))
  (bind _hpbar (Variables|UI|GetHPBar))
  (bind _output_get (Variables|UnitData|SetUnitData S_UnitData))
  (Components|SkeletalMesh|SetSkeletalMeshAsset _skeletalmesh (.Mesh (Utilities|Struct|BreakS_UnitData_Assets (.Assets (Utilities|Struct|BreakS_UnitData _output_get)))))
  (Class|SkeletalMeshComponent|SetAnimClass _skeletalmesh (.AnimationBlueprint (Utilities|Struct|BreakS_UnitData_Assets (.Assets (Utilities|Struct|BreakS_UnitData _output_get)))))
  (Default|CallOnUnitStatsChanged self)
  (Utilities|IsValid _hpbar
    (:Is%20Valid
      (Default|EventUpdateHPBar _hpbar))))

(fn SetAnimationState
  (params (State :type E_UnitAnimationState%20Enum :default "NewEnumerator0"))
  (Class|BPIUnitAnimation|SetUnitAnimationState(Message) (Components|SkeletalMesh|GetAnimInstance (Variables|Default|GetSkeletalMesh)) State))

(fn SetGrid
  (params (Grid :type BP%20Grid%20Manager%20Object%20Reference))
  (bind _mesh_teamindex (Variables|Default|GetMesh_TeamIndex))
  (Variables|Grid|SetGrid Grid)
  (Components|StaticMesh|SetStaticMesh _mesh_teamindex (.FlatMesh (Utilities|Struct|BreakS_GridShapeData (Default|GetCurrentShapeData Grid))))
  (Rendering|Material|SetMaterial _mesh_teamindex 0 (.FlatMaterial (Utilities|Struct|BreakS_GridShapeData (Default|GetCurrentShapeData Grid))))
  (Rendering|Material|SetScalarParameterValueonMaterials _mesh_teamindex "IsFilled" 1.0)
  (Transformation|SetAbsolute _mesh_teamindex false true true)
  (Transformation|SetWorldScale3D _mesh_teamindex (/ (Variables|/Game/Blueprints/Tactical/Grid/BP_GridManager.BP_GridManager_C|GetGridTileSize (Variables|Grid|GetGrid)) (.MeshSize (Utilities|Struct|BreakS_GridShapeData (Default|GetCurrentShapeData Grid)))))
  (Transformation|SetWorldRotation _mesh_teamindex (Default|GetTileRotationfromGridIndex Grid (Variables|Grid|GetIndex)) false false)
  (Transformation|SetRelativeLocation _mesh_teamindex (Math|Vector|MakeVector 0.0 0.0 (+ (Variables|/Game/Blueprints/Tactical/Grid/BP_GridVisual.BP_GridVisual_C|GetOffsetFromGround (Variables|/Game/Blueprints/Tactical/Grid/BP_GridManager.BP_GridManager_C|GetGridVisual Grid)) 5.0)) false false))

(fn UnitUseAbility
  (params (TargetIndex :type Int%20Point%20Structure) (AbilityData :type S%20Ability%20Data%20Structure))
  (bind _returnvalue (Transformation|GetActorLocation))
  (bind _grid (Variables|Grid|GetGrid))
  (bind _requirements (Utilities|Struct|BreakS_AbilityData AbilityData))
  (bind (_x _y) (Math|Vector|BreakVector _returnvalue))
  (bind _gridtiles (Variables|/Game/Blueprints/Tactical/Grid/BP_GridManager.BP_GridManager_C|GetGridTiles _grid))
  (bind (_cost_hp _cost_ap _cost_mp) (Utilities|Struct|BreakS_AbilityData_Requirements _requirements))
  (bind _value (Utilities|Map|Find _gridtiles TargetIndex))
  (bind _transform (Utilities|Struct|BreakS_TileData _value))
  (bind (_x_2 _y_2) (Math|Vector|BreakVector (.location _transform)))
  ;[1 1 1] Point unit at target and start proper animation.
  (Transformation|SetActorRotation (Math|Rotator|FindLookatRotation (Math|Vector|MakeVector _x _y 0.0) (Math|Vector|MakeVector _x_2 _y_2 0.0)))
  (Animation|SetAnimationState "NewEnumerator2")
  ;[1 1 1] Spend cost to cast ability.
  (Stats|ModifyCurrentHP (- 0 _cost_hp) true)
  (Stats|ModifyCurrentAP (- 0 _cost_ap) false true)
  (Stats|ModifyCurrentMP (- 0 _cost_mp) false true)
  (Utilities|FlowControl|Sequence
    (:then_0
      (if (> (Utilities|Struct|BreakS_AbilityData_Requirements (Utilities|Struct|BreakS_AbilityData AbilityData)) 0) ; Ability has a cooldown?
        (Abilities|SetAbilityCooldown (PureUtilities|GetAbilityDataType AbilityData) (PureUtilities|GetAbilityDataCooldown AbilityData))))))

(fn ModifyCurrentHP
  (params (HPModifier :type Integer) (Display? :type Boolean))
  (Stats|SetCurrentHP (+ HPModifier (.HP_Currrent (Utilities|Struct|BreakS_UnitData_Stats (.Stats (Utilities|Struct|BreakS_UnitData (Variables|UnitData|GetUnitData)))))) Display?))

(fn SetCurrentHP
  (params (HP :type Integer) (Display? :type Boolean))
  (bind _unitdata (Variables|UnitData|GetUnitData))
  (bind _stats (Utilities|Struct|BreakS_UnitData _unitdata))
  (bind (_hp_max _hp_currrent) (Utilities|Struct|BreakS_UnitData_Stats _stats))
  (LocalVariables|SetDifference (- HP _hp_currrent))
  (bind _structout (Utilities|Struct|SetmembersinS_UnitData_Stats (.Stats (Utilities|Struct|BreakS_UnitData (Variables|UnitData|GetUnitData))) (Math|Integer|Clamp(Integer) HP 0 _hp_max)))
  (Utilities|Struct|SetmembersinS_UnitData (Variables|UnitData|GetUnitData) _structout)
  (Default|CallOnUnitStatsChanged self)
  (if Display?
    (Animation|SpawnAnimatedNumber (LocalVariables|GetDifference) "NewEnumerator0")
    (Default|EventUpdateHPBar (Variables|UI|GetHPBar))))

(fn UnitHitbyAbility
  (params (AbilityAnimation :type BP%20Ability%20Animation%20Object%20Reference) (AbilityImpactReal :type S%20Ability%20Data%20Impact%20Real%20Structure))
  (bind _modifier_hp (Utilities|Struct|BreakS_AbilityData_ImpactReal AbilityImpactReal))
  (bind _modifier_mp (Utilities|Struct|BreakS_AbilityData_ImpactReal AbilityImpactReal))
  (bind _modifier_ap (Utilities|Struct|BreakS_AbilityData_ImpactReal AbilityImpactReal))
  (Utilities|Map|Add (Variables|Abilities|GetIncomingAbilityImpacts) AbilityAnimation AbilityImpactReal)
  (EventDispatchers|BindEventtoOnAbilityAnimationHitTile AbilityAnimation (EventDispatchers|CreateEvent :!event OnAbilityAnimationHitTile))
  (Utilities|FlowControl|Sequence
    (:then_0
      (if (!= _modifier_hp 0)
        (Stats|ModifyCurrentHP _modifier_hp false)))
    (:then_1
      (if (!= _modifier_ap 0)
        (Stats|ModifyCurrentAP _modifier_ap false false)))
    (:then_2
      (if (!= _modifier_mp 0)
        (Stats|ModifyCurrentMP _modifier_mp false false)))))

(fn OnAbilityAnimationHitTile
  (params (AbilityAnimation :type BP%20Ability%20Animation%20Object%20Reference) (HitIndex :type Int%20Point%20Structure))
  (bind _incomingabilityimpacts (Variables|Abilities|GetIncomingAbilityImpacts))
  (bind (_value _returnvalue) (Utilities|Map|Find _incomingabilityimpacts AbilityAnimation))
  ;[1 1 1] If unit index matches hit index
  (if (Class|KismetMathLibrary|EqualIntPointIntPoint (Variables|Grid|GetIndex) HitIndex)
    ;[1 1 1] Get impact then remove from list of incoming abilities
    (if _returnvalue :!label _label
      (LocalVariables|SetAbilityImpactReal _value)
      (Utilities|Map|Remove (Variables|Abilities|GetIncomingAbilityImpacts) AbilityAnimation)
      ;[1 1 1] Handle UI for impact.
      (Animation|SpawnAnimatedNumber (.Modifier_MP (Utilities|Struct|BreakS_AbilityData_ImpactReal (LocalVariables|GetAbilityImpactReal))) "NewEnumerator1")
      (Animation|SpawnAnimatedNumber (.Modifier_AP (Utilities|Struct|BreakS_AbilityData_ImpactReal (LocalVariables|GetAbilityImpactReal))) "NewEnumerator2")
      (if (!= (.Modifier_HP (Utilities|Struct|BreakS_AbilityData_ImpactReal (LocalVariables|GetAbilityImpactReal))) 0)
        (Default|EventUpdateHPBar (Variables|UI|GetHPBar))
        (Animation|SpawnAnimatedNumber (.Modifier_HP (Utilities|Struct|BreakS_AbilityData_ImpactReal (LocalVariables|GetAbilityImpactReal))) "NewEnumerator0")
        ;[1 1 1] Did the impact deal damage
        (if (< (.Modifier_HP (Utilities|Struct|BreakS_AbilityData_ImpactReal (LocalVariables|GetAbilityImpactReal))) 0)
          ;[1 1 1] Is the unit dead
          (if (not (Stats|IsAlive))
            (if (Utilities|Enum|NotEqual(Enum) (Animation|GetAnimationState) "NewEnumerator4")
              (Animation|SetAnimationState "NewEnumerator4"))
            (else
              (Animation|SetAnimationState "NewEnumerator3"))))))
    (elif (Class|KismetMathLibrary|EqualIntPointIntPoint (Variables|Grid|GetSecondaryIndexForAbilityImpact) HitIndex)
      (Variables|Grid|SetSecondaryIndexForAbilityImpact (Utilities|Struct|MakeIntPoint -999 -999))
      (goto _label))))

(fn GetAnimationState
  (bind _state (Class|BPIUnitAnimation|GetUnitAnimationState(Message) (Components|SkeletalMesh|GetAnimInstance (Variables|Default|GetSkeletalMesh))))
  (return _state))

(fn SetTeamIndex
  (params (Index :type Integer))
  (Variables|UnitData|SetTeamIndex Index)
  (Class|ProgressBar|SetFillColorandOpacity (Variables|/Game/Blueprints/Tactical/Units/UI/W_HPBar.W_HPBar_C|GetProgressBar_HP (Variables|UI|GetHPBar)) (CallFunction|GetTeamColor (Variables|UnitData|GetTeamIndex)))
  (Rendering|Material|SetVectorParameterValueonMaterials (Variables|Default|GetMesh_TeamIndex) "Color" (Math|Conversions|ToVector(LinearColor) (CallFunction|GetTeamColor (Variables|UnitData|GetTeamIndex)))))

(fn SetGridIndex
  (params (Index :type Int%20Point%20Structure))
  (Variables|Grid|SetIndex Index)
  (Transformation|SetWorldRotation (Variables|Default|GetMesh_TeamIndex) (Default|GetTileRotationfromGridIndex (Variables|Grid|GetGrid) (Variables|Grid|GetIndex)) false false))

(fn CombatStarted
  (Stats|ResetMP false)
  (Stats|ResetAP)
  (Abilities|ResetAbilityCooldown))

(fn TurnStarted)

(fn TurnEnded
  (if (Stats|IsAlive)
    (Stats|ResetMP false)
    (Stats|ResetAP)
    (Abilities|DecreaseAbilityCooldowns)))

(fn CombatEnded
  (Stats|ResetMP false)
  (Stats|ResetAP)
  (Abilities|ResetAbilityCooldown))

(fn SetCurrentMP
  (params (MP :type Integer) (ClampMax? :type Boolean) (Display? :type Boolean))
  (bind _unitdata (Variables|UnitData|GetUnitData))
  (bind _unitdata_2 (Variables|UnitData|GetUnitData))
  (bind _stats (Utilities|Struct|BreakS_UnitData _unitdata))
  (bind (_mp_max _mp_current) (Utilities|Struct|BreakS_UnitData_Stats _stats))
  (LocalVariables|SetMPMax _mp_max)
  (LocalVariables|SetMPDifference (- MP _mp_current))
  (if ClampMax?
    (bind _structout (Utilities|Struct|SetmembersinS_UnitData_Stats (.Stats (Utilities|Struct|BreakS_UnitData (Variables|UnitData|GetUnitData))) (Math|Integer|Clamp(Integer) MP 0 (LocalVariables|GetMPMax))))
    (Utilities|Struct|SetmembersinS_UnitData _unitdata_2 _structout)
    (else
      (bind _structout_2 (Utilities|Struct|SetmembersinS_UnitData_Stats (.Stats (Utilities|Struct|BreakS_UnitData (Variables|UnitData|GetUnitData))) MP))
      (Utilities|Struct|SetmembersinS_UnitData _unitdata_2 _structout_2)))
  (Default|CallOnUnitStatsChanged self)
  (if Display?
    (Animation|SpawnAnimatedNumber (LocalVariables|GetMPDifference) "NewEnumerator1")))

(fn ModifyCurrentMP
  (params (MovementModifier :type Integer) (ClampMax? :type Boolean) (Display? :type Boolean))
  (Stats|SetCurrentMP (+ MovementModifier (Utilities|Struct|BreakS_UnitData_Stats (.Stats (Utilities|Struct|BreakS_UnitData (Variables|UnitData|GetUnitData))))) ClampMax? Display?))

(fn ResetMP
  (params (UseSupplies :type Boolean))
  (if UseSupplies
    (Stats|SetCurrentMP (Variables|Inventory|GetSupplies) false true)
    (else
      (Stats|SetCurrentMP (.MP_Max (Utilities|Struct|BreakS_UnitData_Stats (.Stats (Utilities|Struct|BreakS_UnitData (Variables|UnitData|GetUnitData))))) false true))))

(fn SpawnAnimatedNumber
  (params (Number :type Integer) (Color :type E_AnimatedNumberColor%20Enum :default "NewEnumerator0"))
  (if (!= Number 0)
    (Game|SpawnActorfromClass "/Game/Blueprints/Tactical/Units/UI/BP_AnimatedNumber.BP_AnimatedNumber_C" (Math|Transform|MakeTransform (Transformation|GetActorLocation) "0, 0, 0" "1.000000,1.000000,1.000000") "Undefined" "MultiplyWithRoot" 0 Number Color 0)))

(fn SetCurrentAP
  (params (AP :type Integer) (ClampMax? :type Boolean) (Display? :type Boolean))
  (bind _unitdata (Variables|UnitData|GetUnitData))
  (bind _unitdata_2 (Variables|UnitData|GetUnitData))
  (bind _stats (Utilities|Struct|BreakS_UnitData _unitdata))
  (bind (_ap_max _ap_current) (Utilities|Struct|BreakS_UnitData_Stats _stats))
  (LocalVariables|SetAPMax _ap_max)
  (LocalVariables|SetAPDifference (- AP _ap_current))
  (if ClampMax?
    (bind _structout (Utilities|Struct|SetmembersinS_UnitData_Stats (.Stats (Utilities|Struct|BreakS_UnitData (Variables|UnitData|GetUnitData))) (Math|Integer|Clamp(Integer) AP 0 (LocalVariables|GetAPMax))))
    (Utilities|Struct|SetmembersinS_UnitData _unitdata_2 _structout)
    (else
      (bind _structout_2 (Utilities|Struct|SetmembersinS_UnitData_Stats (.Stats (Utilities|Struct|BreakS_UnitData (Variables|UnitData|GetUnitData))) AP))
      (Utilities|Struct|SetmembersinS_UnitData _unitdata_2 _structout_2)))
  (Default|CallOnUnitStatsChanged self)
  (if Display?
    (Animation|SpawnAnimatedNumber (LocalVariables|GetAPDifference) "NewEnumerator2")))

(fn ModifyCurrentAP
  (params (APModifier :type Integer) (ClampMax? :type Boolean) (Display? :type Boolean))
  (Stats|SetCurrentAP (+ APModifier (.AP_Current (Utilities|Struct|BreakS_UnitData_Stats (.Stats (Utilities|Struct|BreakS_UnitData (Variables|UnitData|GetUnitData)))))) ClampMax? Display?))

(fn ResetAP
  (Stats|SetCurrentAP (.AP_Max (Utilities|Struct|BreakS_UnitData_Stats (.Stats (Utilities|Struct|BreakS_UnitData (Variables|UnitData|GetUnitData))))) false true))

(fn CanUseAbility
  (params (AbilityData :type S%20Ability%20Data%20Structure))
  (bind _unitdata (Variables|UnitData|GetUnitData))
  (bind _stats (Utilities|Struct|BreakS_UnitData _unitdata))
  (bind _requirements (Utilities|Struct|BreakS_AbilityData AbilityData))
  (bind (_hp_currrent _ap_current _mp_current) (Utilities|Struct|BreakS_UnitData_Stats _stats))
  (bind (_cost_ap _cost_mp) (Utilities|Struct|BreakS_AbilityData_Requirements _requirements))
  (if (Utilities|Array|ContainsItem (PureUtilities|GetAvailableAbilities) (Utilities|Struct|BreakS_AbilityData AbilityData)) ; Is ability allowed for this unit
    (if (Math|Boolean|ANDBoolean (> _hp_currrent 0) (>= _mp_current _cost_ap) (>= _ap_current _cost_mp)) ; Does the unit have enough resources?
      (if (<= (Abilities|GetAbilityCooldown (Utilities|Struct|BreakS_AbilityData AbilityData)) 0) ; Is the ability off cooldown?
        (return true)
        (else
          (return false)))
      (else
        (return false)))
    (else
      (return false))))

(fn IsAlive
  (return (> (.HP_Currrent (Utilities|Struct|BreakS_UnitData_Stats (.Stats (Utilities|Struct|BreakS_UnitData (Variables|UnitData|GetUnitData))))) 0)))

(fn GetAvailableAbilities
  (return (Utilities|Struct|BreakS_UnitData_Stats (Utilities|Struct|BreakS_UnitData (Variables|UnitData|GetUnitData)))))

(fn GetAbilityCooldown
  (params (Ability :type E_Ability%20Enum :default "NewEnumerator0"))
  (return (.Value (Utilities|Map|Find (Utilities|Struct|BreakS_UnitData_AbilityState (Utilities|Struct|BreakS_UnitData (Variables|UnitData|GetUnitData))) Ability))))

(fn SetAbilityCooldown
  (params (Ability :type E_Ability%20Enum :default "NewEnumerator0") (Cooldown :type Integer))
  (if (!= (Abilities|GetAbilityCooldown Ability) Cooldown)
    (Utilities|Map|Add (Utilities|Struct|BreakS_UnitData_AbilityState (Utilities|Struct|BreakS_UnitData (Variables|UnitData|GetUnitData))) Ability Cooldown)
    (Default|CallOnUnitStatsChanged self)))

(fn DecreaseAbilityCooldowns
  (bind _unitdata (Variables|UnitData|GetUnitData))
  (bind _abilitystate (Utilities|Struct|BreakS_UnitData _unitdata))
  (bind _abilitycooldowns (Utilities|Struct|BreakS_UnitData_AbilityState _abilitystate))
  (bind _keys (Utilities|Map|Keys _abilitycooldowns))
  ;[1 1 1] For each ability in the map, subtract 1 from the cooldown. If its still greater than 0 update value, otherwise remove from map the cooldown is over.
  (for _array_element _keys
    (LocalVariables|SetAbility _array_element)
    (if (.ReturnValue (Utilities|Map|Find _abilitycooldowns (LocalVariables|GetAbility)))
      (if (> (- (.Value (Utilities|Map|Find _abilitycooldowns (LocalVariables|GetAbility))) 1) 0)
        (Utilities|Map|Add _abilitycooldowns (LocalVariables|GetAbility) (- (.Value (Utilities|Map|Find _abilitycooldowns (LocalVariables|GetAbility))) 1))
        (else
          (Utilities|Map|Remove _abilitycooldowns (LocalVariables|GetAbility))))))
  (Default|CallOnUnitStatsChanged self))

(fn ResetAbilityCooldown
  (Utilities|Struct|SetmembersinS_UnitData_AbilityState (Utilities|Struct|BreakS_UnitData (Variables|UnitData|GetUnitData)) (Utilities|Map|MakeMap))
  (Default|CallOnUnitStatsChanged self))

(fn GetAbilityDataType
  (params (AbilityData :type S%20Ability%20Data%20Structure))
  (return (.Ability (Utilities|Struct|BreakS_AbilityData AbilityData))))

(fn GetAbilityDataCooldown
  (params (AbilityData :type S%20Ability%20Data%20Structure%20%28by%20ref%29))
  (return (Utilities|Struct|BreakS_AbilityData_Requirements (Utilities|Struct|BreakS_AbilityData AbilityData))))

(fn OverworldActive
  (Stats|ResetMP true)
  (Stats|ResetAP)
  (Abilities|ResetAbilityCooldown))

(fn CancelPathFollowing
  (Variables|Pathing|SetCancelPath true))