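; Player-side controller actor for tactical grid gameplay, handling cursor hover, tile and unit selection, and click actions.
; Each tick it traces for the hovered unit or tile, then passes it to primary and secondary action actors spawned per selection, repeating while held.
; It binds to grid and combat manager events to sync selection, swap move or ability actions each turn, and show combat and end-screen widgets.
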(event Custom|OnTileUnderCursorChanged
  (Utilities|FlowControl|Sequence
    (:then_0
      (Actions|TryExecuteHoveredAction (Variables|Actions|GetSelectedAction_Primary) (Variables|Grid|GetHoveredTile))
      (if (Variables|Actions|GetIsPrimaryActionOngoing)
        (Actions|TryExecuteAction (Variables|Actions|GetSelectedAction_Primary) (Variables|Grid|GetHoveredTile))))
    (:then_1
      (Actions|TryExecuteHoveredAction (Variables|Actions|GetSelectedAction_Secondary) (Variables|Grid|GetHoveredTile))
      (if (Variables|Actions|GetIsSecondaryActionOngoing)
        (Actions|TryExecuteAction (Variables|Actions|GetSelectedAction_Secondary) (Variables|Grid|GetHoveredTile))))))

(event Input|EnhancedActionEvents|EnhancedInputActionIA_Tactical_QuickKeys
  (params (ActionValue :type Float%20%28double-precision%29) (ElapsedSeconds :type Float%20%28double-precision%29) (TriggeredSeconds :type Float%20%28double-precision%29) (InputAction :type Input%20Action%20Object%20Reference :default "/Game/InputActions/Tactical/IA_Tactical_QuickKeys.IA_Tactical_QuickKeys"))
  (bind _combatmanager (Variables|Grid|GetCombatManager))
  (if (Math|Boolean|ANDBoolean (Variables|/Game/Blueprints/Tactical/Combat/BP_CombatManager.BP_CombatManager_C|GetIsInCombat _combatmanager) (not (Variables|/Game/Blueprints/Tactical/Combat/BP_CombatManager.BP_CombatManager_C|GetIsFinishingCombat _combatmanager)) (== (Variables|/Game/Blueprints/Tactical/Combat/BP_CombatManager.BP_CombatManager_C|GetCurrentUnit _combatmanager) (Variables|Grid|GetSelectedUnit)))
    (Default|SetSelectedAbilityfromIndex (Variables|/Game/Blueprints/Tactical/Combat/UI/W_Combat.W_Combat_C|GetButtonList_Abilities (Variables|UI|GetW_Combat)) (- (Math|Float|Round ActionValue) 1))))

(event Input|EnhancedActionEvents|EnhancedInputActionIA_Tactical_EndTurn
  (params (ActionValue :type Boolean) (ElapsedSeconds :type Float%20%28double-precision%29) (TriggeredSeconds :type Float%20%28double-precision%29) (InputAction :type Input%20Action%20Object%20Reference :default "/Game/InputActions/Tactical/IA_Tactical_EndTurn.IA_Tactical_EndTurn"))
  (bind _combatmanager (Variables|Grid|GetCombatManager))
  (if ActionValue
    (if (and (Variables|/Game/Blueprints/Tactical/Combat/BP_CombatManager.BP_CombatManager_C|GetIsInCombat _combatmanager) (not (Variables|/Game/Blueprints/Tactical/Combat/BP_CombatManager.BP_CombatManager_C|GetIsFinishingCombat _combatmanager)))
      (Default|EndCurrentTurn (Variables|Grid|GetCombatManager)))))

(event Input|EnhancedActionEvents|EnhancedInputActionIA_Tactical_EndCombat
  (params (ActionValue :type Boolean) (ElapsedSeconds :type Float%20%28double-precision%29) (TriggeredSeconds :type Float%20%28double-precision%29) (InputAction :type Input%20Action%20Object%20Reference :default "/Game/InputActions/Tactical/IA_Tactical_EndCombat.IA_Tactical_EndCombat"))
  (bind _combatmanager (Variables|Grid|GetCombatManager))
  (if ActionValue
    (if (and (Variables|/Game/Blueprints/Tactical/Combat/BP_CombatManager.BP_CombatManager_C|GetIsInCombat _combatmanager) (not (Variables|/Game/Blueprints/Tactical/Combat/BP_CombatManager.BP_CombatManager_C|GetIsFinishingCombat _combatmanager)))
      (Default|FinishCombat (Variables|Grid|GetCombatManager) -1))))

(event Input|EnhancedActionEvents|EnhancedInputActionIA_Tactical_PrimaryAction
  (params (ActionValue :type Boolean) (ElapsedSeconds :type Float%20%28double-precision%29) (TriggeredSeconds :type Float%20%28double-precision%29) (InputAction :type Input%20Action%20Object%20Reference :default "/Game/InputActions/Tactical/IA_Tactical_PrimaryAction.IA_Tactical_PrimaryAction"))
  (:Triggered
    (if ActionValue
      (HoveredAndSelected|UpdateTileUderCursor)
      (Variables|Actions|SetIsPrimaryActionOngoing true)
      (Actions|TryExecuteAction (Variables|Actions|GetSelectedAction_Primary) (Variables|Grid|GetHoveredTile))))
  (:Completed
    (Variables|Actions|SetIsPrimaryActionOngoing false)))

(event Input|EnhancedActionEvents|EnhancedInputActionIA_Tactical_SecondaryAction
  (params (ActionValue :type Boolean) (ElapsedSeconds :type Float%20%28double-precision%29) (TriggeredSeconds :type Float%20%28double-precision%29) (InputAction :type Input%20Action%20Object%20Reference :default "/Game/InputActions/Tactical/IA_Tactical_SecondaryAction.IA_Tactical_SecondaryAction"))
  (:Triggered
    (if ActionValue
      (HoveredAndSelected|UpdateTileUderCursor)
      (Variables|Actions|SetIsSecondaryActionOngoing true)
      (Actions|TryExecuteAction (Variables|Actions|GetSelectedAction_Secondary) (Variables|Grid|GetHoveredTile))))
  (:Completed
    (Variables|Actions|SetIsSecondaryActionOngoing false)))

(event EventBeginPlay
  (Utilities|FlowControl|Sequence
    (:then_0
      (bind _returnvalue (Actor|GetActorOfClass "/Game/Blueprints/Tactical/Grid/BP_GridManager.BP_GridManager_C"))
      (Utilities|IsValid _returnvalue
        (:Is%20Valid
          (bind _output_get (Variables|Grid|SetGrid _returnvalue))
          (EventDispatchers|BindEventtoOnGridGenerated _output_get (EventDispatchers|CreateEvent :!event OnGridGenerated))
          (EventDispatchers|BindEventtoOnTileDataUpdated _output_get (EventDispatchers|CreateEvent :!event OnTileDataUpdated)))))
    (:then_1
      (bind _returnvalue_2 (Actor|GetActorOfClass "/Game/Blueprints/Tactical/Combat/BP_CombatManager.BP_CombatManager_C"))
      (Utilities|IsValid _returnvalue_2
        (:Is%20Valid
          (bind _output_get_2 (Variables|Grid|SetCombatManager _returnvalue_2))
          (EventDispatchers|BindEventtoOnUnitGridIndexChanged _output_get_2 (EventDispatchers|CreateEvent :!event OnUnitGridIndexChanged))
          (EventDispatchers|BindEventtoOnCombatStarted (Variables|Grid|GetCombatManager) (EventDispatchers|CreateEvent :!event OnCombatStarted))
          (EventDispatchers|BindEventtoOnCombatEnded (Variables|Grid|GetCombatManager) (EventDispatchers|CreateEvent :!event OnCombatEnded))
          (EventDispatchers|BindEventtoOnUnitTurnStarted (Variables|Grid|GetCombatManager) (EventDispatchers|CreateEvent :!event OnUnitTurnStarted))
          (EventDispatchers|BindEventtoOnUnitTurnEnded (Variables|Grid|GetCombatManager) (EventDispatchers|CreateEvent :!event OnUnitTurnEnded))
          (EventDispatchers|BindEventtoOnCombatFinishing (Variables|Grid|GetCombatManager) (EventDispatchers|CreateEvent :!event OnCombatFinishing)))))
    (:then_2
      (Input|EnableInput (Game|GetPlayerController 0)))))

(event EventTick
  (params (DeltaSeconds :type Float%20%28single-precision%29))
  (HoveredAndSelected|UpdateTileUderCursor))

(fn ConstructionScript)

(fn UpdateTileUderCursor
  (Utilities|FlowControl|Sequence
    (:then_0
      (bind _unit (HoveredAndSelected|GetUnitUnderCursor))
      (if (!= _unit (Variables|Grid|GetHoveredUnit))
        (Utilities|FlowControl|Sequence
          (:then_0
            (Utilities|IsValid (Variables|Grid|GetHoveredUnit)
              (:Is%20Valid
                (Default|SetIsHovered (Variables|Grid|GetHoveredUnit) false))))
          (:then_1
            (bind _output_get (Variables|Grid|SetHoveredUnit _unit))
            (Utilities|IsValid _output_get
              (:Is%20Valid
                (Default|SetIsHovered _output_get true)))))))
    (:then_1
      (Utilities|IsValid (Variables|Grid|GetHoveredUnit)
        (:Is%20Valid
          (LocalVariables|SetNewHoveredIndex (Variables|/Game/Blueprints/Tactical/Units/BP_Unit.BP_Unit_C|GetIndex (Variables|Grid|GetHoveredUnit))))
        (:Is%20Not%20Valid
          (bind _index (Default|GetTileIndexUnderCursor (Variables|Grid|GetGrid)))
          (LocalVariables|SetNewHoveredIndex _index)))
      (if (!= (LocalVariables|GetNewHoveredIndex) (Variables|Grid|GetHoveredTile))
        (Default|RemoveStatefromTile (Variables|Grid|GetGrid) (Variables|Grid|GetHoveredTile) "NewEnumerator1")
        (Variables|Grid|SetHoveredTile (LocalVariables|GetNewHoveredIndex))
        (Default|AddStatetoTile (Variables|Grid|GetGrid) (Variables|Grid|GetHoveredTile) "NewEnumerator1")
        (CallFunction|OnTileUnderCursorChanged)))))

(fn SelectTileUnderCursor
  (bind _grid (Variables|Grid|GetGrid))
  (bind _index (Default|GetTileIndexUnderCursor _grid))
  (Default|AddStatetoTile _grid _index "NewEnumerator2"))

(fn DeselectTileUnderCursor
  (bind _grid (Variables|Grid|GetGrid))
  (bind _index (Default|GetTileIndexUnderCursor _grid))
  (Default|RemoveStatefromTile _grid _index "NewEnumerator2"))

(fn TryExecuteAction
  (params (Action :type BP%20Action%20Object%20Reference) (Index :type Int%20Point%20Structure))
  (Utilities|IsValid Action
    (:Is%20Valid
      (Default|ExecuteAction Action Index))))

(fn SetSelectedActions
  (params (LeftAction :type BP%20Action%20Class%20Reference) (RightAction :type BP%20Action%20Class%20Reference))
  (Utilities|FlowControl|Sequence
    (:then_0
      (Utilities|IsValid (Variables|Actions|GetSelectedAction_Primary)
        (:Is%20Valid
          (Actor|DestroyActor (Variables|Actions|GetSelectedAction_Primary))
          (Variables|Actions|SetSelectedAction_Primary 0))
        (:Is%20Not%20Valid
          _))
      (if (Utilities|IsValidClass LeftAction)
        (bind _returnvalue (Game|SpawnActorfromClass LeftAction (Math|Transform|MakeTransform "0, 0, 0" "0, 0, 0" "1.000000,1.000000,1.000000") "AlwaysSpawn" "MultiplyWithRoot" 0 self 0 0))
        (Variables|Actions|SetSelectedAction_Primary _returnvalue)))
    (:then_1
      (Utilities|IsValid (Variables|Actions|GetSelectedAction_Secondary)
        (:Is%20Valid
          (Actor|DestroyActor (Variables|Actions|GetSelectedAction_Secondary))
          (Variables|Actions|SetSelectedAction_Secondary 0))
        (:Is%20Not%20Valid
          _))
      (if (Utilities|IsValidClass RightAction)
        (bind _returnvalue_2 (Game|SpawnActorfromClass RightAction (Math|Transform|MakeTransform "0, 0, 0" "0, 0, 0" "1.000000,1.000000,1.000000") "AlwaysSpawn" "MultiplyWithRoot" 0 self 0 0))
        (Variables|Actions|SetSelectedAction_Secondary _returnvalue_2)))
    (:then_2
      (Default|CallOnSelectedActionsChanged (Variables|Actions|GetSelectedAction_Primary) (Variables|Actions|GetSelectedAction_Secondary)))))

(fn GetUnitUnderCursor
  (params (PlayerIndex :type Integer))
  (bind _returnvalue (Game|GetPlayerController PlayerIndex))
  (bind (_hitresult _returnvalue_2) (Game|Player|GetHitResultUnderCursorbyChannel _returnvalue "TraceTypeQuery5" false))
  (if _returnvalue_2
    ;[1 1 1] Hit a unit so return.
    (return (.AsBP%20Unit (Utilities|Casting|CastToBP_Unit (.HitActor (Collision|BreakHitResult _hitresult)))))
    (else
      ;[1 1 1] A unit was not found so check if we hit a tile which contains a unit.
      (bind _index (Default|GetTileIndexUnderCursor (Variables|Grid|GetGrid) PlayerIndex))
      (return (Utilities|Struct|BreakS_TileData (.Value (Utilities|Map|Find (Variables|/Game/Blueprints/Tactical/Grid/BP_GridManager.BP_GridManager_C|GetGridTiles (Variables|Grid|GetGrid)) _index)))))))

(fn SetSelectedTileandUnit
  (params (Index :type Int%20Point%20Structure) (Force :type Boolean))
  (Utilities|FlowControl|Sequence
    (:then_0
      ;[1 1 1] Handle selected tile. Removes selected state from old tile then add selected state to the new tile.
      (if (or (!= (Variables|Grid|GetSelectedTile) Index) Force)
        (Default|RemoveStatefromTile (Variables|Grid|GetGrid) (Variables|Grid|GetSelectedTile) "NewEnumerator2")
        (Variables|Grid|SetSelectedTile Index)
        (Default|AddStatetoTile (Variables|Grid|GetGrid) (Variables|Grid|GetSelectedTile) "NewEnumerator2")
        (else
          (Default|RemoveStatefromTile (Variables|Grid|GetGrid) (Variables|Grid|GetSelectedTile) "NewEnumerator2")
          (Variables|Grid|SetSelectedTile (Utilities|Struct|MakeIntPoint -999 -999))))
      (Default|CallOnSelectedTileChanged (Variables|Grid|GetSelectedTile)))
    (:then_1
      ;[1 1 1] Handle selected unit. Remove selected property from current selected unit. Then set the new selected unit.
      (LocalVariables|SetNewSelectedUnit (Utilities|Struct|BreakS_TileData (.Value (Utilities|Map|Find (Variables|/Game/Blueprints/Tactical/Grid/BP_GridManager.BP_GridManager_C|GetGridTiles (Variables|Grid|GetGrid)) (Variables|Grid|GetSelectedTile)))))
      (if (or (!= (Variables|Grid|GetSelectedUnit) (LocalVariables|GetNewSelectedUnit)) Force)
        (Utilities|FlowControl|Sequence
          (:then_0
            (Utilities|IsValid (Variables|Grid|GetSelectedUnit)
              (:Is%20Valid
                (Default|SetIsSelected (Variables|Grid|GetSelectedUnit) false))))
          (:then_1
            (bind _output_get (Variables|Grid|SetSelectedUnit (LocalVariables|GetNewSelectedUnit)))
            (Utilities|IsValid _output_get
              (:Is%20Valid
                (Default|SetIsSelected _output_get true)))))))))

(fn OnGridGenerated
  (if (Default|IsIndexValid (Variables|Grid|GetGrid) (Variables|Grid|GetSelectedTile))
    (HoveredAndSelected|SetSelectedTileandUnit (Variables|Grid|GetSelectedTile) true)
    (else
      (HoveredAndSelected|SetSelectedTileandUnit (Utilities|Struct|MakeIntPoint -999 -999) true))))

(fn OnTileDataUpdated
  (params (Index :type Int%20Point%20Structure))
  (if (Class|KismetMathLibrary|EqualIntPointIntPoint Index (Variables|Grid|GetSelectedTile))
    (Grid|OnGridGenerated)))

(fn OnUnitGridIndexChanged
  (params (Unit :type BP%20Unit%20Object%20Reference))
  (if (== Unit (Variables|Grid|GetSelectedUnit))
    (HoveredAndSelected|SetSelectedTileandUnit (Variables|/Game/Blueprints/Tactical/Units/BP_Unit.BP_Unit_C|GetIndex Unit) false)))

(fn TryExecuteHoveredAction
  (params (Action :type BP%20Action%20Object%20Reference) (Index :type Int%20Point%20Structure))
  (Utilities|IsValid Action
    (:Is%20Valid
      (Default|ExecuteHoveredAction Action Index))))

(fn OnCombatStarted
  (Actions|SetSelectedActions)
  (HoveredAndSelected|SetSelectedTileandUnit (Utilities|Struct|MakeIntPoint -999 -999) false)
  (bind _returnvalue (UserInterface|CreateWidget "/Game/Blueprints/Tactical/Combat/UI/W_Combat.W_Combat_C" 0 self))
  (bind _output_get (Variables|UI|SetW_Combat _returnvalue))
  (UserInterface|Viewport|AddtoPlayerScreen _output_get)
  (EventDispatchers|BindEventtoOnSelectedAbilityButtonChanged (Variables|/Game/Blueprints/Tactical/Combat/UI/W_Combat.W_Combat_C|GetButtonList_Abilities (Variables|UI|GetW_Combat)) (EventDispatchers|CreateEvent :!event OnSelectedAbilityChanged)))

(fn OnCombatEnded
  (Widget|RemovefromParent (Variables|UI|GetW_CombatEndScreen))
  (Variables|UI|SetW_CombatEndScreen 0))

(fn OnUnitTurnStarted
  (params (Unit :type BP%20Unit%20Object%20Reference))
  (HoveredAndSelected|SetSelectedTileandUnit (Variables|/Game/Blueprints/Tactical/Units/BP_Unit.BP_Unit_C|GetIndex Unit) true)
  (Utilities|IsValid (Variables|Grid|GetSelectedUnit)
    (:Is%20Valid
      (Actions|SetSelectedActions "/Game/Blueprints/Tactical/Player/Actions/Combat/BP_Action_CombatMove.BP_Action_CombatMove_C")
      (Default|LinkUnittoAbilitiesList (Variables|/Game/Blueprints/Tactical/Combat/UI/W_Combat.W_Combat_C|GetButtonList_Abilities (Variables|UI|GetW_Combat)) (Variables|Grid|GetSelectedUnit)))))

(fn OnUnitTurnEnded
  (params (Unit :type BP%20Unit%20Object%20Reference))
  (HoveredAndSelected|SetSelectedTileandUnit (Utilities|Struct|MakeIntPoint -999 -999) false)
  (Actions|SetSelectedActions)
  (Default|LinkUnittoAbilitiesList (Variables|/Game/Blueprints/Tactical/Combat/UI/W_Combat.W_Combat_C|GetButtonList_Abilities (Variables|UI|GetW_Combat))))

(fn OnSelectedAbilityChanged
  (params (SelectedButton :type Button%20Ability%20Object%20Reference))
  (Utilities|IsValid SelectedButton
    (:Is%20Valid
      (Actions|SetSelectedActions "/Game/Blueprints/Tactical/Player/Actions/Combat/BP_Action_CombatUseAbility.BP_Action_CombatUseAbility_C")
      (bind _asbp_action_combat_use_ability (Utilities|Casting|CastToBP_Action_CombatUseAbility (Variables|Actions|GetSelectedAction_Primary)))
      (Default|SetAbility _asbp_action_combat_use_ability (Variables|/Game/Blueprints/Tactical/Combat/Abilities/Widgets/Button_Ability.Button_Ability_C|GetAbilityType SelectedButton)))
    (:Is%20Not%20Valid
      (if (!= (Utilities|GetClass (Variables|Actions|GetSelectedAction_Primary)) "/Game/Blueprints/Tactical/Player/Actions/Combat/BP_Action_CombatMove.BP_Action_CombatMove_C")
        (Actions|SetSelectedActions "/Game/Blueprints/Tactical/Player/Actions/Combat/BP_Action_CombatMove.BP_Action_CombatMove_C")))))

(fn OnCombatFinishing
  (params (WinningTeamIndex :type Integer))
  (Actions|SetSelectedActions)
  (HoveredAndSelected|SetSelectedTileandUnit (Utilities|Struct|MakeIntPoint -999 -999) false)
  (Widget|RemovefromParent (Variables|UI|GetW_Combat))
  (Variables|UI|SetW_Combat 0)
  (bind _returnvalue (UserInterface|CreateWidget "/Game/Blueprints/Tactical/Combat/UI/W_CombatEndScreen.W_CombatEndScreen_C" 0 self WinningTeamIndex))
  (bind _output_get (Variables|UI|SetW_CombatEndScreen _returnvalue))
  (UserInterface|Viewport|AddtoPlayerScreen _output_get))

(fn CenterCameraonTilebyIndex
  (params (Index :type Int%20Point%20Structure))
  (bind _grid (Variables|Grid|GetGrid))
  (bind _tilelocation (Default|GetTileLocationfromGridIndex _grid Index))
  (bind _asbp_tactical_pawn (Utilities|Casting|CastToBP_TacticalPawn (Game|Player|GetPlayerPawn 0)))
  (LocalVariables|SetPawn _asbp_tactical_pawn)
  (Variables|/Game/Blueprints/Tactical/Player/BP_TacticalPawn.BP_TacticalPawn_C|SetTargetLocation (LocalVariables|GetPawn) (Math|Vector|MakeVector (.x _tilelocation) (.y _tilelocation) (.z (Variables|/Game/Blueprints/Tactical/Player/BP_TacticalPawn.BP_TacticalPawn_C|GetTargetLocation (LocalVariables|GetPawn))))))

(fn SetGrid
  (params (NewParam :type BP%20Grid%20Manager%20Object%20Reference))
  (bind _output_get (Variables|Grid|SetGrid NewParam))
  (EventDispatchers|BindEventtoOnGridGenerated _output_get (EventDispatchers|CreateEvent :!event OnGridGenerated))
  (EventDispatchers|BindEventtoOnTileDataUpdated _output_get (EventDispatchers|CreateEvent :!event OnTileDataUpdated)))

(fn SetCombatManager
  (params (CombatManager :type BP%20Combat%20Manager%20Object%20Reference))
  (bind _output_get (Variables|Grid|SetCombatManager CombatManager))
  (EventDispatchers|BindEventtoOnUnitGridIndexChanged _output_get (EventDispatchers|CreateEvent :!event OnUnitGridIndexChanged))
  (EventDispatchers|BindEventtoOnCombatStarted (Variables|Grid|GetCombatManager) (EventDispatchers|CreateEvent :!event OnCombatStarted))
  (EventDispatchers|BindEventtoOnCombatEnded (Variables|Grid|GetCombatManager) (EventDispatchers|CreateEvent :!event OnCombatEnded))
  (EventDispatchers|BindEventtoOnUnitTurnStarted (Variables|Grid|GetCombatManager) (EventDispatchers|CreateEvent :!event OnUnitTurnStarted))
  (EventDispatchers|BindEventtoOnUnitTurnEnded (Variables|Grid|GetCombatManager) (EventDispatchers|CreateEvent :!event OnUnitTurnEnded))
  (EventDispatchers|BindEventtoOnCombatFinishing (Variables|Grid|GetCombatManager) (EventDispatchers|CreateEvent :!event OnCombatFinishing)))