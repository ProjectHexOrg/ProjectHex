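; Player action for combat setup that previews an ability's range and area of effect on the tactical grid.
; On execute, it clears and repaints range tile states from the CombatManager's GetAbilityRange at the selected tile, then refreshes the AOE.
; Hover updates redraw only the AOE, shown when the hovered tile is within range.
; The AOE uses the CastAOE pattern, or just the hovered tile for the enum's first pattern value.
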(event EventBeginPlay
  (|CallParentFunction) ; This node is disabled and will not be called.\nDrag off pins to build functionality.
)

(event Collision|EventActorBeginOverlap
  (params (OtherActor :type Actor%20Object%20Reference))
  (|CallParentFunction OtherActor) ; This node is disabled and will not be called.\nDrag off pins to build functionality.
)

(event EventTick
  (params (DeltaSeconds :type Float%20%28single-precision%29))
  (|CallParentFunction DeltaSeconds) ; This node is disabled and will not be called.\nDrag off pins to build functionality.
)

(fn ConstructionScript
  (|CallParentFunction))

(fn ExecuteAction
  (params (Index :type Int%20Point%20Structure))
  (|CallParentFunction Index)
  (CallFunction|ShowAbilityRangePattern))

(fn ShowAbilityRangePattern
  (bind _playeractions (Variables|Default|GetPlayerActions))
  (bind _playeractions_2 (Variables|Default|GetPlayerActions))
  (Utilities|FlowControl|Sequence
    (:then_0
      (Default|ClearStatefromTiles (Variables|/Game/Blueprints/Tactical/Player/BP_PlayerActions.BP_PlayerActions_C|GetGrid (Variables|Default|GetPlayerActions)) "NewEnumerator8")
      (if (Default|IsIndexValid (Variables|/Game/Blueprints/Tactical/Player/BP_PlayerActions.BP_PlayerActions_C|GetGrid _playeractions_2) (Variables|/Game/Blueprints/Tactical/Player/BP_PlayerActions.BP_PlayerActions_C|GetSelectedTile _playeractions_2))
        (bind _rangeindexes (Default|GetAbilityRange (Variables|/Game/Blueprints/Tactical/Player/BP_PlayerActions.BP_PlayerActions_C|GetCombatManager _playeractions) (Variables|/Game/Blueprints/Tactical/Player/BP_PlayerActions.BP_PlayerActions_C|GetSelectedTile _playeractions) (Variables|Default|GetCast)))
        (for _array_element _rangeindexes
          (Default|AddStatetoTile (Variables|/Game/Blueprints/Tactical/Player/BP_PlayerActions.BP_PlayerActions_C|GetGrid (Variables|Default|GetPlayerActions)) _array_element "NewEnumerator8"))))
    (:then_1
      (CallFunction|ShowAbilityRangePatternAOE))))

(fn ShowAbilityRangePatternAOE
  (bind _playeractions (Variables|Default|GetPlayerActions))
  (bind _playeractions_2 (Variables|Default|GetPlayerActions))
  (Default|ClearStatefromTiles (Variables|/Game/Blueprints/Tactical/Player/BP_PlayerActions.BP_PlayerActions_C|GetGrid (Variables|Default|GetPlayerActions)) "NewEnumerator9")
  (if (Utilities|Array|ContainsItem (Utilities|Struct|BreakS_IntPointArray (.Value (Utilities|Map|Find (Variables|/Game/Blueprints/Tactical/Grid/BP_GridManager.BP_GridManager_C|GetTileStateToIndexes (Variables|/Game/Blueprints/Tactical/Player/BP_PlayerActions.BP_PlayerActions_C|GetGrid (Variables|Default|GetPlayerActions))) "NewEnumerator8"))) (Variables|/Game/Blueprints/Tactical/Player/BP_PlayerActions.BP_PlayerActions_C|GetHoveredTile (Variables|Default|GetPlayerActions)))
    (if (Utilities|Enum|NotEqual(Enum) (Utilities|Struct|BreakS_AbilityData_Cast (Variables|Default|GetCastAOE)) "NewEnumerator0")
      (bind _rangeindexes (Default|GetAbilityRange (Variables|/Game/Blueprints/Tactical/Player/BP_PlayerActions.BP_PlayerActions_C|GetCombatManager _playeractions) (Variables|/Game/Blueprints/Tactical/Player/BP_PlayerActions.BP_PlayerActions_C|GetHoveredTile _playeractions) (Variables|Default|GetCastAOE)))
      (for _array_element _rangeindexes
        (Default|AddStatetoTile (Variables|/Game/Blueprints/Tactical/Player/BP_PlayerActions.BP_PlayerActions_C|GetGrid (Variables|Default|GetPlayerActions)) _array_element "NewEnumerator9"))
      (else
        (Default|AddStatetoTile (Variables|/Game/Blueprints/Tactical/Player/BP_PlayerActions.BP_PlayerActions_C|GetGrid _playeractions_2) (Variables|/Game/Blueprints/Tactical/Player/BP_PlayerActions.BP_PlayerActions_C|GetHoveredTile _playeractions_2) "NewEnumerator9")))))

(fn ExecuteHoveredAction
  (params (Index :type Int%20Point%20Structure))
  (|CallParentFunction Index)
  (CallFunction|ShowAbilityRangePatternAOE))