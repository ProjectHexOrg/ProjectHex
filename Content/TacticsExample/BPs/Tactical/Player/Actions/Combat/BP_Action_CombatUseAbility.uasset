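; Player action for using a combat ability on the tactical grid, with range and area-of-effect previews.
; SetAbility loads the ability's Cast and CastAOE data, then tags tiles in range from the selected tile via the CombatManager.
; Hovering a tile inside that range previews the AOE pattern, or just that tile without one.
; Executing calls UseAbility and deselects the combat widget's button; EndPlay clears both tile states.
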(event EventBeginPlay
  (|CallParentFunction))

(event EventEndPlay
  (params (EndPlayReason :type EEndPlayReason%20Enum :default "Destroyed"))
  (bind _playeractions (Variables|Default|GetPlayerActions))
  (bind _grid (Variables|/Game/Blueprints/Tactical/Player/BP_PlayerActions.BP_PlayerActions_C|GetGrid _playeractions))
  (|CallParentFunction EndPlayReason)
  (Default|ClearStatefromTiles _grid "NewEnumerator8")
  (Default|ClearStatefromTiles _grid "NewEnumerator9"))

(fn ConstructionScript
  (|CallParentFunction))

(fn SetAbility
  (params (Ability :type E_Ability%20Enum :default "NewEnumerator0"))
  (bind _playeractions (Variables|Default|GetPlayerActions))
  (bind _grid (Variables|/Game/Blueprints/Tactical/Player/BP_PlayerActions.BP_PlayerActions_C|GetGrid _playeractions))
  (bind _output_get (Variables|Default|SetAbility Ability))
  (if (Utilities|Enum|NotEqual(Enum) _output_get "NewEnumerator0")
    (bind _abilitydata (CallFunction|GetAbilityData (Variables|Default|GetAbility)))
    (Variables|Default|SetCast (.cast _abilitydata))
    (Variables|Default|SetCastAOE (.castaoe _abilitydata))
    (CallFunction|ShowAbilityRangePattern)
    (else
      (Default|ClearStatefromTiles _grid "NewEnumerator8")
      (Default|ClearStatefromTiles _grid "NewEnumerator9"))))

(fn ShowAbilityRangePattern
  (Utilities|FlowControl|Sequence
    (:then_0
      (Default|ClearStatefromTiles (Variables|/Game/Blueprints/Tactical/Player/BP_PlayerActions.BP_PlayerActions_C|GetGrid (Variables|Default|GetPlayerActions)) "NewEnumerator8")
      (bind _rangeindexes (Default|GetAbilityRange (Variables|/Game/Blueprints/Tactical/Player/BP_PlayerActions.BP_PlayerActions_C|GetCombatManager (Variables|Default|GetPlayerActions)) (Variables|/Game/Blueprints/Tactical/Player/BP_PlayerActions.BP_PlayerActions_C|GetSelectedTile (Variables|Default|GetPlayerActions)) (Variables|Default|GetCast)))
      (for _array_element _rangeindexes
        (Default|AddStatetoTile (Variables|/Game/Blueprints/Tactical/Player/BP_PlayerActions.BP_PlayerActions_C|GetGrid (Variables|Default|GetPlayerActions)) _array_element "NewEnumerator8")))
    (:then_1
      (CallFunction|ShowAbilityRangePatternAOE))))

(fn ExecuteAction
  (params (Index :type Int%20Point%20Structure))
  (bind _playeractions (Variables|Default|GetPlayerActions))
  (bind _w_combat (Variables|/Game/Blueprints/Tactical/Player/BP_PlayerActions.BP_PlayerActions_C|GetW_Combat _playeractions))
  (|CallParentFunction Index)
  (Default|UseAbility (Variables|/Game/Blueprints/Tactical/Player/BP_PlayerActions.BP_PlayerActions_C|GetCombatManager (Variables|Default|GetPlayerActions)) (Variables|Default|GetAbility) (Variables|/Game/Blueprints/Tactical/Player/BP_PlayerActions.BP_PlayerActions_C|GetSelectedTile (Variables|Default|GetPlayerActions)) Index)
  (Utilities|IsValid _w_combat ; Widget is destroyed while finishing combat. So it may not be valid.
    (:Is%20Valid
      (Default|SetSelectedAbilityfromIndex (Variables|/Game/Blueprints/Tactical/Combat/UI/W_Combat.W_Combat_C|GetButtonList_Abilities _w_combat) -1))))

(fn ShowAbilityRangePatternAOE
  (bind _playeractions (Variables|Default|GetPlayerActions))
  (bind _playeractions_2 (Variables|Default|GetPlayerActions))
  (Default|ClearStatefromTiles (Variables|/Game/Blueprints/Tactical/Player/BP_PlayerActions.BP_PlayerActions_C|GetGrid (Variables|Default|GetPlayerActions)) "NewEnumerator9")
  (if (Utilities|Array|ContainsItem (Utilities|Struct|BreakS_IntPointArray (.Value (Utilities|Map|Find (Variables|/Game/Blueprints/Tactical/Grid/BP_GridManager.BP_GridManager_C|GetTileStateToIndexes (Variables|/Game/Blueprints/Tactical/Player/BP_PlayerActions.BP_PlayerActions_C|GetGrid (Variables|Default|GetPlayerActions))) "NewEnumerator8"))) (Variables|/Game/Blueprints/Tactical/Player/BP_PlayerActions.BP_PlayerActions_C|GetHoveredTile (Variables|Default|GetPlayerActions)))
    (if (Utilities|Enum|NotEqual(Enum) (Utilities|Struct|BreakS_AbilityData_Cast (Variables|Default|GetCastAOE)) "NewEnumerator0")
      (bind _rangeindexes (Default|GetAbilityRange (Variables|/Game/Blueprints/Tactical/Player/BP_PlayerActions.BP_PlayerActions_C|GetCombatManager _playeractions) (Variables|/Game/Blueprints/Tactical/Player/BP_PlayerActions.BP_PlayerActions_C|GetHoveredTile _playeractions) (Variables|Default|GetCastAOE)))
      (for _array_element _rangeindexes
        (Default|AddStatetoTile (Variables|/Game/Blueprints/Tactical/Player/BP_PlayerActions.BP_PlayerActions_C|GetGrid (Variables|Default|GetPlayerActions)) _array_element "NewEnumerator9"))
      (else
        (Default|AddStatetoTile (Variables|/Game/Blueprints/Tactical/Player/BP_PlayerActions.BP_PlayerActions_C|GetGrid _playeractions_2) (Variables|/Game/Blueprints/Tactical/Player/BP_PlayerActions.BP_PlayerActions_C|GetHoveredTile _playeractions_2) "NewEnumerator9")))))

(fn ExecuteHoveredAction
  (params (Index :type Int%20Point%20Structure))
  (|CallParentFunction Index)
  (CallFunction|ShowAbilityRangePatternAOE))