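; Player combat action that moves the selected unit on the tactical grid, previewing reachable tiles and the path to the hovered tile.
; Hovering shows the reach of the hovered unit, or of the selected unit plus a path, limited by movement points, diagonal rules and valid tile types.
; Pathfinding completion events highlight tiles via tile states, and executing sends the path to the CombatManager.
; Walk events suspend previews during movement and refresh them afterwards.
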(event EventBeginPlay
  (bind _playeractions (Variables|Default|GetPlayerActions))
  (bind _selectedunit (Variables|/Game/Blueprints/Tactical/Player/BP_PlayerActions.BP_PlayerActions_C|GetSelectedUnit _playeractions))
  (|CallParentFunction)
  (EventDispatchers|BindEventtoOnPathfindingCompleted (Variables|/Game/Blueprints/Tactical/Grid/BP_GridManager.BP_GridManager_C|GetGridPathfinding_ReachableTiles (Variables|/Game/Blueprints/Tactical/Player/BP_PlayerActions.BP_PlayerActions_C|GetGrid (Variables|Default|GetPlayerActions))) (EventDispatchers|CreateEvent :!event OnPathfindingCompletedReachables))
  (EventDispatchers|BindEventtoOnPathfindingCompleted (Variables|/Game/Blueprints/Tactical/Grid/BP_GridManager.BP_GridManager_C|GetGridPathfinding (Variables|/Game/Blueprints/Tactical/Player/BP_PlayerActions.BP_PlayerActions_C|GetGrid (Variables|Default|GetPlayerActions))) (EventDispatchers|CreateEvent :!event OnPathfindingCompletedPath))
  (EventDispatchers|BindEventtoOnUnitStartedWalking _selectedunit (EventDispatchers|CreateEvent :!event OnUnitStartedWalking))
  (EventDispatchers|BindEventtoOnUnitFinishedWalking _selectedunit (EventDispatchers|CreateEvent :!event OnUnitFinishedWalking))
  (Reachables|GenerateReachableTiles (Variables|/Game/Blueprints/Tactical/Player/BP_PlayerActions.BP_PlayerActions_C|GetSelectedUnit (Variables|Default|GetPlayerActions))))

(event EventEndPlay
  (params (EndPlayReason :type EEndPlayReason%20Enum :default "Destroyed"))
  (bind _playeractions (Variables|Default|GetPlayerActions))
  (bind _grid (Variables|/Game/Blueprints/Tactical/Player/BP_PlayerActions.BP_PlayerActions_C|GetGrid _playeractions))
  (|CallParentFunction EndPlayReason)
  (Default|ClearStatefromTiles _grid "NewEnumerator7")
  (Default|ClearStatefromTiles _grid "NewEnumerator4"))

(fn ConstructionScript
  (|CallParentFunction))

(fn GenerateReachableTiles
  (params (Unit :type BP%20Unit%20Object%20Reference))
  (if (!= Unit (Variables|Default|GetCurrentUnitForDisplayedReachableTiles))
    (Variables|Default|SetCurrentUnitForDisplayedReachableTiles Unit)
    (Default|ClearStatefromTiles (Variables|/Game/Blueprints/Tactical/Player/BP_PlayerActions.BP_PlayerActions_C|GetGrid (Variables|Default|GetPlayerActions)) "NewEnumerator7")
    ;[1 1 1] A valid unit is selected so find reachable tiles based on unit movement.
    (Default|FindPath (Variables|/Game/Blueprints/Tactical/Grid/BP_GridManager.BP_GridManager_C|GetGridPathfinding_ReachableTiles (Variables|/Game/Blueprints/Tactical/Player/BP_PlayerActions.BP_PlayerActions_C|GetGrid (Variables|Default|GetPlayerActions))) (Variables|/Game/Blueprints/Tactical/Units/BP_Unit.BP_Unit_C|GetIndex (Variables|Default|GetCurrentUnitForDisplayedReachableTiles)) (Utilities|Struct|MakeIntPoint -999 -999) (.CanMoveDiagonally (Utilities|Struct|BreakS_UnitData_Stats (.Stats (Utilities|Struct|BreakS_UnitData (Variables|/Game/Blueprints/Tactical/Units/BP_Unit.BP_Unit_C|GetUnitData (Variables|Default|GetCurrentUnitForDisplayedReachableTiles)))))) (.ValidTileTypes (Utilities|Struct|BreakS_UnitData_Stats (.Stats (Utilities|Struct|BreakS_UnitData (Variables|/Game/Blueprints/Tactical/Units/BP_Unit.BP_Unit_C|GetUnitData (Variables|Default|GetCurrentUnitForDisplayedReachableTiles)))))) 0.0 0.0 true (.MP_Current (Utilities|Struct|BreakS_UnitData_Stats (.Stats (Utilities|Struct|BreakS_UnitData (Variables|/Game/Blueprints/Tactical/Units/BP_Unit.BP_Unit_C|GetUnitData (Variables|Default|GetCurrentUnitForDisplayedReachableTiles)))))))))

(fn OnPathfindingCompletedReachables
  (params (ReachableTiles :type Array%20of%20Int%20Point%20Structures))
  (if (not (Variables|Default|GetIsUnitWalking))
    (for _array_element ReachableTiles
      (Default|AddStatetoTile (Variables|/Game/Blueprints/Tactical/Player/BP_PlayerActions.BP_PlayerActions_C|GetGrid (Variables|Default|GetPlayerActions)) _array_element "NewEnumerator7"))))

(fn ExecuteHoveredAction
  (params (Index :type Int%20Point%20Structure))
  (bind _playeractions (Variables|Default|GetPlayerActions))
  (bind _hoveredunit (Variables|/Game/Blueprints/Tactical/Player/BP_PlayerActions.BP_PlayerActions_C|GetHoveredUnit _playeractions))
  (|CallParentFunction Index)
  (if (not (Variables|Default|GetIsUnitWalking))
    (Utilities|IsValid _hoveredunit
      (:Is%20Valid
        (Reachables|GenerateReachableTiles _hoveredunit))
      (:Is%20Not%20Valid
        (Reachables|GenerateReachableTiles (Variables|/Game/Blueprints/Tactical/Player/BP_PlayerActions.BP_PlayerActions_C|GetSelectedUnit _playeractions))
        (Path|GeneratePath)))))

(fn GeneratePath
  (bind _playeractions (Variables|Default|GetPlayerActions))
  (bind _selectedunit (Variables|/Game/Blueprints/Tactical/Player/BP_PlayerActions.BP_PlayerActions_C|GetSelectedUnit _playeractions))
  (bind _unitdata (Variables|/Game/Blueprints/Tactical/Units/BP_Unit.BP_Unit_C|GetUnitData _selectedunit))
  (bind _stats (Utilities|Struct|BreakS_UnitData _unitdata))
  (bind (_validtiletypes _canmovediagonally _availableabilities _hp_max _hp_currrent _ap_max _ap_current _mp_max _mp_current) (Utilities|Struct|BreakS_UnitData_Stats _stats))
  (Default|ClearStatefromTiles (Variables|/Game/Blueprints/Tactical/Player/BP_PlayerActions.BP_PlayerActions_C|GetGrid (Variables|Default|GetPlayerActions)) "NewEnumerator4")
  (Utilities|Array|Clear (Variables|Default|GetGeneratedPath))
  (Default|FindPath (Variables|/Game/Blueprints/Tactical/Grid/BP_GridManager.BP_GridManager_C|GetGridPathfinding (Variables|/Game/Blueprints/Tactical/Player/BP_PlayerActions.BP_PlayerActions_C|GetGrid (Variables|Default|GetPlayerActions))) (Variables|/Game/Blueprints/Tactical/Units/BP_Unit.BP_Unit_C|GetIndex _selectedunit) (Variables|/Game/Blueprints/Tactical/Player/BP_PlayerActions.BP_PlayerActions_C|GetHoveredTile (Variables|Default|GetPlayerActions)) _canmovediagonally _validtiletypes 0.0 15.0 false _mp_current))

(fn OnPathfindingCompletedPath
  (params (Path :type Array%20of%20Int%20Point%20Structures))
  (bind _output_get (Variables|Default|SetGeneratedPath Path))
  (for _array_element _output_get
    (Default|AddStatetoTile (Variables|/Game/Blueprints/Tactical/Player/BP_PlayerActions.BP_PlayerActions_C|GetGrid (Variables|Default|GetPlayerActions)) _array_element "NewEnumerator4")))

(fn ExecuteAction
  (params (Index :type Int%20Point%20Structure))
  (bind _playeractions (Variables|Default|GetPlayerActions))
  (|CallParentFunction Index)
  (if (> (Utilities|Array|Length (Variables|Default|GetGeneratedPath)) 0)
    (Default|MoveUnit (Variables|/Game/Blueprints/Tactical/Player/BP_PlayerActions.BP_PlayerActions_C|GetCombatManager _playeractions) (Variables|/Game/Blueprints/Tactical/Player/BP_PlayerActions.BP_PlayerActions_C|GetSelectedUnit _playeractions) (Variables|Default|GetGeneratedPath))
    (Utilities|Array|Clear (Variables|Default|GetGeneratedPath))))

(fn OnUnitStartedWalking
  (params (Unit :type BP%20Unit%20Object%20Reference))
  (Variables|Default|SetIsUnitWalking true)
  (Default|ClearStatefromTiles (Variables|/Game/Blueprints/Tactical/Player/BP_PlayerActions.BP_PlayerActions_C|GetGrid (Variables|Default|GetPlayerActions)) "NewEnumerator7")
  (Variables|Default|SetCurrentUnitForDisplayedReachableTiles 0))

(fn OnUnitFinishedWalking
  (params (Unit :type BP%20Unit%20Object%20Reference))
  (Variables|Default|SetIsUnitWalking false)
  (CallFunction|ExecuteHoveredAction (Variables|/Game/Blueprints/Tactical/Player/BP_PlayerActions.BP_PlayerActions_C|GetHoveredTile (Variables|Default|GetPlayerActions))))