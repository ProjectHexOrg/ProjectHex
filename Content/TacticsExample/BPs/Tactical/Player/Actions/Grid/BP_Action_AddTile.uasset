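; Player grid action that adds a tile at a given grid index in the tactics example.
; ExecuteAction runs the parent logic, then acts only when the grid reports the index as not valid.
; It builds the tile transform from the grid's location, rotation and scale helpers and passes it to AddGridTileCheckUseEnvironment on the grid.
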(event EventBeginPlay
  (|CallParentFunction) ; This node is disabled and will not be called.\nDrag off pins to build functionality.
)

(event Collision|EventActorBeginOverlap
  (params (OtherActor :type Actor%20Object%20Reference))
  (|CallParentFunction OtherActor) ; This node is disabled and will not be called.\nDrag off pins to build functionality.
)

(event EventTick
  (params (DeltaSeconds :type Float%20%28single-precision%29))
  (|CallParentFunction DeltaSeconds) ; This node is disabled and will not be called.\nDrag off pins to build functionality.
)

(fn ConstructionScript
  (|CallParentFunction))

(fn ExecuteAction
  (params (Index :type Int%20Point%20Structure))
  (bind _playeractions (Variables|Default|GetPlayerActions))
  (bind _grid (Variables|/Game/Blueprints/Tactical/Player/BP_PlayerActions.BP_PlayerActions_C|GetGrid _playeractions))
  (|CallParentFunction Index)
  (if (not (Default|IsIndexValid (Variables|/Game/Blueprints/Tactical/Player/BP_PlayerActions.BP_PlayerActions_C|GetGrid (Variables|Default|GetPlayerActions)) Index))
    (Default|AddGridTileCheckUseEnvironment (Variables|/Game/Blueprints/Tactical/Player/BP_PlayerActions.BP_PlayerActions_C|GetGrid (Variables|Default|GetPlayerActions)) Index (Math|Transform|MakeTransform (Default|GetTileLocationfromGridIndex _grid Index) (Default|GetTileRotationfromGridIndex _grid Index) (Default|GetTileScale _grid)))))