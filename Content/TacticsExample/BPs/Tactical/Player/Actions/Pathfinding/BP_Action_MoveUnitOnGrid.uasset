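; Player action that moves the selected unit along a pathfound route on the tactical grid.
; Executing it requests a path from the selected tile to the target, limited by the unit's diagonal, tile type and current MP stats.
; On completion it marks path tiles, passes the move to the CombatManager and calls ResetMP.
; Each tile's mark clears as the unit walks it; EndPlay re-executes with an off-grid index.
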(event EventBeginPlay
  (|CallParentFunction) ; This node is disabled and will not be called.\nDrag off pins to build functionality.
)

(event Collision|EventActorBeginOverlap
  (params (OtherActor :type Actor%20Object%20Reference))
  (|CallParentFunction OtherActor) ; This node is disabled and will not be called.\nDrag off pins to build functionality.
)

(event EventTick
  (params (DeltaSeconds :type Float%20%28single-precision%29))
  (|CallParentFunction DeltaSeconds) ; This node is disabled and will not be called.\nDrag off pins to build functionality.
)

(event EventEndPlay
  (params (EndPlayReason :type EEndPlayReason%20Enum :default "Destroyed"))
  (CallFunction|ExecuteAction (Utilities|Struct|MakeIntPoint -999 -999)))

(fn ConstructionScript
  (|CallParentFunction))

(fn ExecuteAction
  (params (Index :type Int%20Point%20Structure))
  (|CallParentFunction Index)
  (Default|ClearStatefromTiles (Variables|/Game/Blueprints/Tactical/Player/BP_PlayerActions.BP_PlayerActions_C|GetGrid (Variables|Default|GetPlayerActions)) "NewEnumerator4")
  (bind _output_get (Variables|Default|SetCurrentUnit (Variables|/Game/Blueprints/Tactical/Player/BP_PlayerActions.BP_PlayerActions_C|GetSelectedUnit (Variables|Default|GetPlayerActions))))
  (Utilities|IsValid _output_get
    (:Is%20Valid
      (EventDispatchers|BindEventtoOnUnitFinishedWalkingTile (Variables|Default|GetCurrentUnit) (EventDispatchers|CreateEvent :!event OnUnitFinishedWalkingTile))
      (EventDispatchers|BindEventtoOnPathfindingCompleted (Variables|/Game/Blueprints/Tactical/Grid/BP_GridManager.BP_GridManager_C|GetGridPathfinding (Variables|/Game/Blueprints/Tactical/Player/BP_PlayerActions.BP_PlayerActions_C|GetGrid (Variables|Default|GetPlayerActions))) (EventDispatchers|CreateEvent :!event OnPathfindingCompleted))
      (Default|FindPath (Variables|/Game/Blueprints/Tactical/Grid/BP_GridManager.BP_GridManager_C|GetGridPathfinding (Variables|/Game/Blueprints/Tactical/Player/BP_PlayerActions.BP_PlayerActions_C|GetGrid (Variables|Default|GetPlayerActions))) (Variables|/Game/Blueprints/Tactical/Player/BP_PlayerActions.BP_PlayerActions_C|GetSelectedTile (Variables|Default|GetPlayerActions)) Index (.CanMoveDiagonally (Utilities|Struct|BreakS_UnitData_Stats (.Stats (Utilities|Struct|BreakS_UnitData (Variables|/Game/Blueprints/Tactical/Units/BP_Unit.BP_Unit_C|GetUnitData (Variables|Default|GetCurrentUnit)))))) (.ValidTileTypes (Utilities|Struct|BreakS_UnitData_Stats (.Stats (Utilities|Struct|BreakS_UnitData (Variables|/Game/Blueprints/Tactical/Units/BP_Unit.BP_Unit_C|GetUnitData (Variables|Default|GetCurrentUnit)))))) 0.0 0.0 false (.MP_Current (Utilities|Struct|BreakS_UnitData_Stats (.Stats (Utilities|Struct|BreakS_UnitData (Variables|/Game/Blueprints/Tactical/Units/BP_Unit.BP_Unit_C|GetUnitData (Variables|Default|GetCurrentUnit))))))))))

(fn OnPathfindingCompleted
  (params (Path :type Array%20of%20Int%20Point%20Structures))
  (Utilities|IsValid (Variables|Default|GetCurrentUnit)
    (:Is%20Valid
      (if (== (Variables|Default|GetCurrentUnit) (Variables|/Game/Blueprints/Tactical/Player/BP_PlayerActions.BP_PlayerActions_C|GetSelectedUnit (Variables|Default|GetPlayerActions)))
        (for _array_element Path
          (Default|AddStatetoTile (Variables|/Game/Blueprints/Tactical/Player/BP_PlayerActions.BP_PlayerActions_C|GetGrid (Variables|Default|GetPlayerActions)) _array_element "NewEnumerator4"))
        (Variables|/Game/Blueprints/Tactical/Units/BP_Unit.BP_Unit_C|SetMoveDurationPerTile (Variables|Default|GetCurrentUnit) (Variables|Default|GetMoveDurationPerTile))
        (Default|MoveUnit (Variables|/Game/Blueprints/Tactical/Player/BP_PlayerActions.BP_PlayerActions_C|GetCombatManager (Variables|Default|GetPlayerActions)) (Variables|Default|GetCurrentUnit) Path)
        (Default|ResetMP (Variables|Default|GetCurrentUnit) false)))))

(fn OnUnitFinishedWalkingTile
  (params (Unit :type BP%20Unit%20Object%20Reference) (Index :type Int%20Point%20Structure))
  (if (== Unit (Variables|Default|GetCurrentUnit))
    (Default|RemoveStatefromTile (Variables|/Game/Blueprints/Tactical/Player/BP_PlayerActions.BP_PlayerActions_C|GetGrid (Variables|Default|GetPlayerActions)) Index "NewEnumerator4")))