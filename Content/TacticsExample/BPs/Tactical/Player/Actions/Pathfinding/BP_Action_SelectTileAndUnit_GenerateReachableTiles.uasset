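; Player action for the tactics grid that extends tile and unit selection by highlighting the tiles reachable from the selected tile.
; Runs the grid's reachable-tiles pathfinder using the selected unit's movement stats, or configurable debug settings when no unit is selected.
; A completion event marks the returned tiles with a grid state.
; Unit walk events clear that highlight on start and regenerate it on finish.
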(event EventBeginPlay
  (|CallParentFunction) ; This node is disabled and will not be called.\nDrag off pins to build functionality.
)

(event Collision|EventActorBeginOverlap
  (params (OtherActor :type Actor%20Object%20Reference))
  (|CallParentFunction OtherActor) ; This node is disabled and will not be called.\nDrag off pins to build functionality.
)

(event EventTick
  (params (DeltaSeconds :type Float%20%28single-precision%29))
  (|CallParentFunction DeltaSeconds) ; This node is disabled and will not be called.\nDrag off pins to build functionality.
)

(fn ConstructionScript
  (|CallParentFunction))

(fn ExecuteAction
  (params (Index :type Int%20Point%20Structure))
  (|CallParentFunction Index)
  (CallFunction|GenerateReachableTiles))

(fn GenerateReachableTiles
  (bind _playeractions (Variables|Default|GetPlayerActions))
  (bind _playeractions_2 (Variables|Default|GetPlayerActions))
  (bind _selectedunit (Variables|/Game/Blueprints/Tactical/Player/BP_PlayerActions.BP_PlayerActions_C|GetSelectedUnit _playeractions))
  (bind _selectedunit_2 (Variables|/Game/Blueprints/Tactical/Player/BP_PlayerActions.BP_PlayerActions_C|GetSelectedUnit _playeractions_2))
  (bind _unitdata (Variables|/Game/Blueprints/Tactical/Units/BP_Unit.BP_Unit_C|GetUnitData _selectedunit))
  (bind _stats (Utilities|Struct|BreakS_UnitData _unitdata))
  (bind (_validtiletypes _canmovediagonally _availableabilities _hp_max _hp_currrent _ap_max _ap_current _mp_max _mp_current) (Utilities|Struct|BreakS_UnitData_Stats _stats))
  (Default|ClearStatefromTiles (Variables|/Game/Blueprints/Tactical/Player/BP_PlayerActions.BP_PlayerActions_C|GetGrid (Variables|Default|GetPlayerActions)) "NewEnumerator7")
  (EventDispatchers|BindEventtoOnPathfindingCompleted (Variables|/Game/Blueprints/Tactical/Grid/BP_GridManager.BP_GridManager_C|GetGridPathfinding_ReachableTiles (Variables|/Game/Blueprints/Tactical/Player/BP_PlayerActions.BP_PlayerActions_C|GetGrid (Variables|Default|GetPlayerActions))) (EventDispatchers|CreateEvent :!event OnPathfindingCompleted))
  ;[1 1 1] Is a unit selected?
  (Utilities|IsValid (Variables|/Game/Blueprints/Tactical/Player/BP_PlayerActions.BP_PlayerActions_C|GetSelectedUnit (Variables|Default|GetPlayerActions))
    (:Is%20Valid
      (EventDispatchers|BindEventtoOnUnitStartedWalking _selectedunit_2 (EventDispatchers|CreateEvent :!event OnUnitStartedWalking))
      (EventDispatchers|BindEventtoOnUnitFinishedWalking _selectedunit_2 (EventDispatchers|CreateEvent :!event OnUnitFinishedWalking))
      ;[1 1 1] A valid unit is selected so find reachable tiles based on unit movement.
      (Default|FindPath (Variables|/Game/Blueprints/Tactical/Grid/BP_GridManager.BP_GridManager_C|GetGridPathfinding_ReachableTiles (Variables|/Game/Blueprints/Tactical/Player/BP_PlayerActions.BP_PlayerActions_C|GetGrid (Variables|Default|GetPlayerActions))) (Variables|/Game/Blueprints/Tactical/Player/BP_PlayerActions.BP_PlayerActions_C|GetSelectedTile (Variables|Default|GetPlayerActions)) (Utilities|Struct|MakeIntPoint -999 -999) _canmovediagonally _validtiletypes 0.0 0.0 true _mp_current))
    (:Is%20Not%20Valid
      ;[1 1 1] Find reachable tiles using debug information since no unit is selected.
      (Default|FindPath (Variables|/Game/Blueprints/Tactical/Grid/BP_GridManager.BP_GridManager_C|GetGridPathfinding_ReachableTiles (Variables|/Game/Blueprints/Tactical/Player/BP_PlayerActions.BP_PlayerActions_C|GetGrid (Variables|Default|GetPlayerActions))) (Variables|/Game/Blueprints/Tactical/Player/BP_PlayerActions.BP_PlayerActions_C|GetSelectedTile (Variables|Default|GetPlayerActions)) (Utilities|Struct|MakeIntPoint -999 -999) (Variables|Default|GetIncludeFlyingOnly) (select (Variables|Default|GetIncludeFlyingOnly) (Utilities|Array|MakeArray "NewEnumerator1" "NewEnumerator3" "NewEnumerator4" "NewEnumerator5") (Utilities|Array|MakeArray "NewEnumerator1" "NewEnumerator3" "NewEnumerator4")) (Variables|Default|GetIterationDelay) (Variables|Default|GetMaxMSPerFrame) true (Variables|Default|GetMaxPathLength)))))

(fn OnPathfindingCompleted
  (params (Path :type Array%20of%20Int%20Point%20Structures))
  (for _array_element Path
    (Default|AddStatetoTile (Variables|/Game/Blueprints/Tactical/Player/BP_PlayerActions.BP_PlayerActions_C|GetGrid (Variables|Default|GetPlayerActions)) _array_element "NewEnumerator7")))

(fn OnUnitStartedWalking
  (params (Unit :type BP%20Unit%20Object%20Reference))
  (Default|ClearStatefromTiles (Variables|/Game/Blueprints/Tactical/Player/BP_PlayerActions.BP_PlayerActions_C|GetGrid (Variables|Default|GetPlayerActions)) "NewEnumerator7"))

(fn OnUnitFinishedWalking
  (params (Unit :type BP%20Unit%20Object%20Reference))
  (CallFunction|GenerateReachableTiles))