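; Player action that finds a path on the tactical grid from the selected tile to a target tile and highlights it.
; Executing it clears the previous path state, then calls GridPathfinding with diagonal, flying-only tile, length, delay and per-frame time-budget settings.
; The completion callback marks each returned tile with the path state.
; Selection changes and EndPlay re-execute with an invalid index, clearing the highlight.
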(event Custom|OnSelectedTileChanged
  (params (Index :type Int%20Point%20Structure))
  (CallFunction|ExecuteAction (Utilities|Struct|MakeIntPoint -999 -999)))

(event EventBeginPlay
  (|CallParentFunction)
  (EventDispatchers|BindEventtoOnSelectedTileChanged (Variables|Default|GetPlayerActions) (delegate Custom|OnSelectedTileChanged)))

(event EventEndPlay
  (params (EndPlayReason :type EEndPlayReason%20Enum :default "Destroyed"))
  (CallFunction|ExecuteAction (Utilities|Struct|MakeIntPoint -999 -999)))

(fn ConstructionScript
  (|CallParentFunction))

(fn ExecuteAction
  (params (Index :type Int%20Point%20Structure))
  (|CallParentFunction Index)
  (Default|ClearStatefromTiles (Variables|/Game/Blueprints/Tactical/Player/BP_PlayerActions.BP_PlayerActions_C|GetGrid (Variables|Default|GetPlayerActions)) "NewEnumerator4")
  (EventDispatchers|BindEventtoOnPathfindingCompleted (Variables|/Game/Blueprints/Tactical/Grid/BP_GridManager.BP_GridManager_C|GetGridPathfinding (Variables|/Game/Blueprints/Tactical/Player/BP_PlayerActions.BP_PlayerActions_C|GetGrid (Variables|Default|GetPlayerActions))) (EventDispatchers|CreateEvent :!event OnPathfindingCompleted))
  (Default|FindPath (Variables|/Game/Blueprints/Tactical/Grid/BP_GridManager.BP_GridManager_C|GetGridPathfinding (Variables|/Game/Blueprints/Tactical/Player/BP_PlayerActions.BP_PlayerActions_C|GetGrid (Variables|Default|GetPlayerActions))) (Variables|/Game/Blueprints/Tactical/Player/BP_PlayerActions.BP_PlayerActions_C|GetSelectedTile (Variables|Default|GetPlayerActions)) Index (Variables|Default|GetInclude%20Diagonals) (select (Variables|Default|GetIncludeFlyingOnly) (Utilities|Array|MakeArray "NewEnumerator1" "NewEnumerator3" "NewEnumerator4" "NewEnumerator5") (Utilities|Array|MakeArray "NewEnumerator1" "NewEnumerator3" "NewEnumerator4")) (Variables|Default|GetIterationDelay) (Variables|Default|GetMax%20MS%20Per%20Frame) false (Variables|Default|GetMaxPathLength)))

(fn OnPathfindingCompleted
  (params (Path :type Array%20of%20Int%20Point%20Structures))
  (for _array_element Path
    (Default|AddStatetoTile (Variables|/Game/Blueprints/Tactical/Player/BP_PlayerActions.BP_PlayerActions_C|GetGrid (Variables|Default|GetPlayerActions)) _array_element "NewEnumerator4")))