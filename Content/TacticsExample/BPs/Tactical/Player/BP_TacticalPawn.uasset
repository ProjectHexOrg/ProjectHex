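; Player camera pawn for the tactical example, possessed on BeginPlay with the mouse cursor shown and the tactical input mapping context added.
; Enhanced Input zoom, pan and rotate actions only change target values: clamped arm length, location along the pawn's axes, and stepped yaw.
; Tick eases the spring arm, actor location and rotation toward those targets with interpolation for smooth movement.
; It also caches the PlayerActions child actor on BeginPlay.
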(event Input|EnhancedActionEvents|EnhancedInputActionIA_Tactical_CameraZoom
  (params (ActionValue :type Float%20%28double-precision%29) (ElapsedSeconds :type Float%20%28double-precision%29) (TriggeredSeconds :type Float%20%28double-precision%29) (InputAction :type Input%20Action%20Object%20Reference :default "/Game/InputActions/Tactical/Camera/IA_Tactical_CameraZoom.IA_Tactical_CameraZoom"))
  ;[1 1 1] Camera Controls
  (Variables|Camera|SetTargetZoom (Math|Float|Clamp(Float) (+ (Variables|Camera|GetTargetZoom) (* ActionValue (Variables|Camera|GetCameraZoomSpeed))) (Variables|Camera|GetCameraZoomMin) (Variables|Camera|GetCameraZoomMax))))

(event Input|EnhancedActionEvents|EnhancedInputActionIA_Tactical_CameraPan
  (params (ActionValue :type Vector%202D%20Structure) (ElapsedSeconds :type Float%20%28double-precision%29) (TriggeredSeconds :type Float%20%28double-precision%29) (InputAction :type Input%20Action%20Object%20Reference :default "/Game/InputActions/Tactical/Camera/IA_Tactical_CameraPan.IA_Tactical_CameraPan"))
  (bind _camerapanspeed (Variables|Camera|GetCameraPanSpeed))
  (bind _returnvalue (* ActionValue _camerapanspeed))
  ;[1 1 1] Camera Controls
  (Variables|Camera|SetTargetLocation (+ (+ (Variables|Camera|GetTargetLocation) (* (Transformation|GetActorForwardVector) (.x _returnvalue))) (* (.y _returnvalue) (Transformation|GetActorRightVector)))))

(event Input|EnhancedActionEvents|EnhancedInputActionIA_Tactical_CameraRotationLeft
  (params (ActionValue :type Boolean) (ElapsedSeconds :type Float%20%28double-precision%29) (TriggeredSeconds :type Float%20%28double-precision%29) (InputAction :type Input%20Action%20Object%20Reference :default "/Game/InputActions/Tactical/Camera/IA_Tactical_CameraRotationLeft.IA_Tactical_CameraRotationLeft"))
  ;[1 1 1] Camera Controls
  (if ActionValue
    (Variables|Camera|SetTargetRotation (Math|Rotator|CombineRotators (Variables|Camera|GetTargetRotation) (Math|Rotator|MakeRotator 0.0 0.0 (Variables|Camera|GetCameraRotationDegree))))))

(event Input|EnhancedActionEvents|EnhancedInputActionIA_Tactical_CameraRotationRight
  (params (ActionValue :type Boolean) (ElapsedSeconds :type Float%20%28double-precision%29) (TriggeredSeconds :type Float%20%28double-precision%29) (InputAction :type Input%20Action%20Object%20Reference :default "/Game/InputActions/Tactical/Camera/IA_Tactical_CameraRotationRight.IA_Tactical_CameraRotationRight"))
  ;[1 1 1] Camera Controls
  (if ActionValue
    (Variables|Camera|SetTargetRotation (Math|Rotator|CombineRotators (Variables|Camera|GetTargetRotation) (Math|Rotator|MakeRotator 0.0 0.0 (* (Variables|Camera|GetCameraRotationDegree) -1.0))))))

(event EventTick
  (params (DeltaSeconds :type Float%20%28single-precision%29))
  ;[1 1 1] Game Flow
  (Camera|UpdateCameraonTick DeltaSeconds))

(event EventBeginPlay
  (bind _returnvalue (Game|GetPlayerController 0))
  ;[1 1 1] Game Flow
  (Variables|Default|SetPlayerActions (.AsBP%20Player%20Actions (Utilities|Casting|CastToBP_PlayerActions (Variables|/Script/Engine.ChildActorComponent|GetChildActor (Variables|Default|GetChildActor_PlayerActions)))))
  (Variables|Camera|SetTargetZoom (Variables|/Script/Engine.SpringArmComponent|GetTargetArmLength (Variables|Default|GetSpringArm)))
  (Variables|Camera|SetTargetLocation (Transformation|GetActorLocation))
  (Variables|Camera|SetTargetRotation (Transformation|GetActorRotation))
  (Pawn|Possess _returnvalue self)
  (Variables|/Script/Engine.PlayerController|SetbShowMouseCursor _returnvalue true)
  (bind _asplayer_controller (Utilities|Casting|CastToPlayerController _returnvalue))
  (Input|AddMappingContext (PlayerController|LocalPlayerSubsystems|GetEnhancedInputLocalPlayerSubsystem _asplayer_controller) "/Game/InputActions/Tactical/IMC_Tactical.IMC_Tactical" 0 "(bIgnoreAllPressedKeysUntilRelease=True,bForceImmediately=False,bNotifyUserSettings=False)"))

(fn ConstructionScript)

(fn GetCameraZoomInterp
  (params (DeltaTime :type Float%20%28double-precision%29))
  (bind _springarm (Variables|Default|GetSpringArm))
  (Variables|/Script/Engine.SpringArmComponent|SetTargetArmLength _springarm (Math|Interpolation|FInterpTo (Variables|/Script/Engine.SpringArmComponent|GetTargetArmLength _springarm) (Variables|Camera|GetTargetZoom) DeltaTime (Variables|Camera|GetCameraZoomInterp)))
  (return))

(fn GetCameraLocationInterp
  (params (DeltaTime :type Float%20%28single-precision%29))
  (Transformation|SetActorLocation (Math|Interpolation|VInterpTo (Transformation|GetActorLocation) (Variables|Camera|GetTargetLocation) DeltaTime (Variables|Camera|GetCameraLocationInterp)) false false)
  (return))

(fn GetCameraRotationInterp
  (params (DeltaTime :type Float%20%28single-precision%29))
  (Transformation|SetActorRotation (Math|Interpolation|RInterpTo (Transformation|GetActorRotation) (Variables|Camera|GetTargetRotation) DeltaTime (Variables|Camera|GetCameraRotationInterp)))
  (return))

(fn UpdateCameraonTick
  (params (DeltaTime :type Float%20%28single-precision%29))
  (Camera|GetCameraZoomInterp DeltaTime)
  (Camera|GetCameraLocationInterp DeltaTime)
  (Camera|GetCameraRotationInterp DeltaTime))