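; Combat manager actor for grid-based tactical battles, spawning the player party and an enemy and running combat from start to finish.
; It tracks units by team and grid tile, revalidating them when the grid changes, and cycles turns through living units.
; Abilities filter range patterns by walkability and corner-offset line-of-sight traces, then apply randomized impacts across the AOE.
; Deaths trigger a last-team-standing check, with events broadcasting state changes.
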(event EventBeginPlay
  (bind _grid (Variables|Default|GetGrid))
  (Utilities|IsValid _grid
    (:Is%20Valid
      (Grid|SetGrid _grid)
      (Setup|SpawnPlayerParty)
      (Setup|SpawnEnemies))))

(event Collision|EventActorBeginOverlap
  (params (OtherActor :type Actor%20Object%20Reference)))

(event EventTick
  (params (DeltaSeconds :type Float%20%28single-precision%29)))

(fn ConstructionScript)

(fn AddUnit
  (params (Unit :type BP%20Unit%20Object%20Reference) (Index :type Int%20Point%20Structure) (TeamIndex :type Integer))
  (Utilities|Array|Add (Variables|Default|GetUnitsInCombat) Unit)
  (Default|SetGrid Unit (Variables|Default|GetGrid))
  (Units|SetUnitIndexonGrid Unit Index false true)
  (EventDispatchers|BindEventtoOnUnitReachedNewTile Unit (EventDispatchers|CreateEvent :!event OnUnitReachedNewTile))
  (Units|SetUnitTeamIndex Unit TeamIndex))

(fn RemoveUnit
  (params (Unit :type BP%20Unit%20Object%20Reference) (DestroyUnit? :type Boolean))
  (Utilities|Array|RemoveItem (Variables|Default|GetUnitsInCombat) Unit)
  (Units|SetUnitIndexonGrid Unit (Utilities|Struct|MakeIntPoint -999 -999) false true)
  (Units|SetUnitTeamIndex Unit -1)
  (if DestroyUnit?
    (Actor|DestroyActor Unit)))

(fn SetUnitIndexonGrid
  (params (Unit :type BP%20Unit%20Object%20Reference) (Index :type Int%20Point%20Structure) (Force :type Boolean) (SnapLocation :type Boolean))
  (bind _grid (Variables|Default|GetGrid))
  (bind _gridtiles (Variables|/Game/Blueprints/Tactical/Grid/BP_GridManager.BP_GridManager_C|GetGridTiles _grid))
  (bind (_value _returnvalue) (Utilities|Map|Find _gridtiles Index))
  (Utilities|FlowControl|Sequence
    (:then_0
      ;[1 1 1] If new index, we move the unit from the previous index to the new one.
      (if (or (!= (Variables|/Game/Blueprints/Tactical/Units/BP_Unit.BP_Unit_C|GetIndex Unit) Index) Force)
        (Utilities|FlowControl|Sequence
          (:then_0
            (bind _output_get (LocalVariables|SetPreviousTile (.Value (Utilities|Map|Find (Variables|/Game/Blueprints/Tactical/Grid/BP_GridManager.BP_GridManager_C|GetGridTiles (Variables|Default|GetGrid)) (Variables|/Game/Blueprints/Tactical/Units/BP_Unit.BP_Unit_C|GetIndex Unit)))))
            (if (== (Utilities|Struct|BreakS_TileData _output_get) Unit)
              (bind _structout (Utilities|Struct|SetmembersinS_TileData (LocalVariables|GetPreviousTile)))
              (Utilities|Map|Add (Variables|/Game/Blueprints/Tactical/Grid/BP_GridManager.BP_GridManager_C|GetGridTiles (Variables|Default|GetGrid)) (Utilities|Struct|BreakS_TileData _structout) _structout)))
          (:then_1
            (Default|SetGridIndex Unit Index)
            (if (!= Index (Utilities|Struct|MakeIntPoint -999 -999))
              (bind _structout_2 (Utilities|Struct|SetmembersinS_TileData (.Value (Utilities|Map|Find (Variables|/Game/Blueprints/Tactical/Grid/BP_GridManager.BP_GridManager_C|GetGridTiles (Variables|Default|GetGrid)) Index)) Unit))
              (Utilities|Map|Add (Variables|/Game/Blueprints/Tactical/Grid/BP_GridManager.BP_GridManager_C|GetGridTiles (Variables|Default|GetGrid)) (Utilities|Struct|BreakS_TileData _structout_2) _structout_2)))
          (:then_2
            (Default|CallOnUnitGridIndexChanged Unit)))))
    (:then_1
      ;[1 1 1] Move actor to new tile in the world space.
      (if SnapLocation
        (Transformation|SetActorLocation Unit (select _returnvalue (.location (Utilities|Struct|BreakS_TileData _value)) "-99999.000000,-99999.000000,-99999.000000") false false)))))

(fn OnGridGenerated
  (bind _output_get (LocalVariables|SetCopyOfUnits (Variables|Default|GetUnitsInCombat)))
  (for _array_element _output_get
    (if (Utilities|Array|ContainsItem (.ValidTileTypes (Utilities|Struct|BreakS_UnitData_Stats (.stats (Variables|/Game/Blueprints/Tactical/Units/BP_Unit.BP_Unit_C|GetUnitData _array_element)))) (.type (.Value (Utilities|Map|Find (Variables|/Game/Blueprints/Tactical/Grid/BP_GridManager.BP_GridManager_C|GetGridTiles (Variables|Default|GetGrid)) (Variables|/Game/Blueprints/Tactical/Units/BP_Unit.BP_Unit_C|GetIndex _array_element)))))
      (Units|SetUnitIndexonGrid _array_element (Variables|/Game/Blueprints/Tactical/Units/BP_Unit.BP_Unit_C|GetIndex _array_element) true true)
      (else
        (Units|RemoveUnit _array_element true)))))

(fn OnTileDataUpdated
  (params (Index :type Int%20Point%20Structure))
  (bind _output_get (LocalVariables|SetCopyOfUnits (Variables|Default|GetUnitsInCombat)))
  (bind _array_element (Utilities|Array|ForEachLoopwithBreak _output_get :!label _label)
    (:LoopBody
      (if (Class|KismetMathLibrary|EqualIntPointIntPoint Index (Variables|/Game/Blueprints/Tactical/Units/BP_Unit.BP_Unit_C|GetIndex _array_element))
        (if (Utilities|Array|ContainsItem (.ValidTileTypes (Utilities|Struct|BreakS_UnitData_Stats (.stats (Variables|/Game/Blueprints/Tactical/Units/BP_Unit.BP_Unit_C|GetUnitData _array_element)))) (.type (.Value (Utilities|Map|Find (Variables|/Game/Blueprints/Tactical/Grid/BP_GridManager.BP_GridManager_C|GetGridTiles (Variables|Default|GetGrid)) (Variables|/Game/Blueprints/Tactical/Units/BP_Unit.BP_Unit_C|GetIndex _array_element)))))
          (Units|SetUnitIndexonGrid _array_element (Variables|/Game/Blueprints/Tactical/Units/BP_Unit.BP_Unit_C|GetIndex _array_element) false true)
          (goto _label Break)
          (else
            (Units|RemoveUnit _array_element true)
            (goto _label Break)))))))

(fn OnUnitReachedNewTile
  (params (Unit :type BP%20Unit%20Object%20Reference) (Index :type Int%20Point%20Structure))
  (Default|SpawnAnimatedNumber Unit (- 0 (CallFunction|GetTileTypeCost (Utilities|Struct|BreakS_TileData (.Value (Utilities|Map|Find (Variables|/Game/Blueprints/Tactical/Grid/BP_GridManager.BP_GridManager_C|GetGridTiles (Variables|Default|GetGrid)) Index))))) "NewEnumerator1"))

(fn UseAbility
  (params (Ability :type E_Ability%20Enum :default "NewEnumerator0") (OriginIndex :type Int%20Point%20Structure) (TargetIndex :type Int%20Point%20Structure))
  (bind _grid (Variables|Default|GetGrid))
  (bind _grid_2 (Variables|Default|GetGrid))
  (bind _gridtiles (Variables|/Game/Blueprints/Tactical/Grid/BP_GridManager.BP_GridManager_C|GetGridTiles _grid))
  (bind _gridtiles_2 (Variables|/Game/Blueprints/Tactical/Grid/BP_GridManager.BP_GridManager_C|GetGridTiles _grid_2))
  (bind _value (Utilities|Map|Find _gridtiles_2 OriginIndex))
  (bind _value_2 (Utilities|Map|Find _gridtiles OriginIndex))
  (bind _unitontile (Utilities|Struct|BreakS_TileData _value))
  (bind _unitontile_2 (Utilities|Struct|BreakS_TileData _value_2))
  (bind _abilitydata (CallFunction|GetAbilityData Ability))
  (LocalVariables|SetData _abilitydata)
  (Utilities|IsValid _unitontile
    (:Is%20Valid
      (bind _canuse (Default|CanUseAbility _unitontile (LocalVariables|GetData)))
      (if _canuse
        ;[1 1 1] Is ability being cast on a tile in range
        (bind _rangeindexes (Abilities|GetAbilityRange OriginIndex (Utilities|Struct|BreakS_AbilityData (LocalVariables|GetData)) :!label _label))
        (if (Utilities|Array|ContainsItem _rangeindexes TargetIndex)
          ;[1 1 1] Build AOE Array
          (if (Utilities|Enum|Equal(Enum) (Utilities|Struct|BreakS_AbilityData_Cast (Utilities|Struct|BreakS_AbilityData (LocalVariables|GetData))) "NewEnumerator0")
            (LocalVariables|SetAttackedIndexes (Utilities|Array|MakeArray TargetIndex))
            (else
              (bind _rangeindexes_2 (Abilities|GetAbilityRange TargetIndex (Utilities|Struct|BreakS_AbilityData (LocalVariables|GetData))))
              (LocalVariables|SetAttackedIndexes _rangeindexes_2)))
          ;[1 1 1] Spawn ability animation
          (bind _returnvalue (Game|SpawnActorfromClass (Utilities|Struct|BreakS_AbilityData_Assets (.assets (LocalVariables|GetData))) (Math|Transform|MakeTransform "0, 0, 0" "0, 0, 0" "1.000000,1.000000,1.000000") "AlwaysSpawn" "MultiplyWithRoot" 0 (Variables|Default|GetGrid) OriginIndex (LocalVariables|GetAttackedIndexes) TargetIndex 0))
          (LocalVariables|SetAbilityAnimation _returnvalue)
          (Utilities|FlowControl|Sequence
            (:then_0
              ;[1 1 1] If a unit is on the origin tile have that unit use the ability. (play animations and such)
              (Utilities|IsValid _unitontile_2
                (:Is%20Valid
                  (Default|UnitUseAbility _unitontile_2 TargetIndex (LocalVariables|GetData)))))
            (:then_1
              ;[1 1 1] Calculate ability impact on targets
              (LocalVariables|SetAbilityImpactReal (Utilities|Struct|MakeS_AbilityData_ImpactReal (CallFunction|MinMaxRandom (.MinMaxModifier_HP (Utilities|Struct|BreakS_AbilityData_Impact (Utilities|Struct|BreakS_AbilityData (LocalVariables|GetData))))) (CallFunction|MinMaxRandom (.MinMaxModifier_MP (Utilities|Struct|BreakS_AbilityData_Impact (Utilities|Struct|BreakS_AbilityData (LocalVariables|GetData))))) (CallFunction|MinMaxRandom (.MinMaxModifier_AP (Utilities|Struct|BreakS_AbilityData_Impact (Utilities|Struct|BreakS_AbilityData (LocalVariables|GetData)))))))
              ;[1 1 1] For each unit on a targeted tile
              (for _array_element (LocalVariables|GetAttackedIndexes)
                (bind _output_get (LocalVariables|SetUnit (Utilities|Struct|BreakS_TileData (.Value (Utilities|Map|Find (Variables|/Game/Blueprints/Tactical/Grid/BP_GridManager.BP_GridManager_C|GetGridTiles (Variables|Default|GetGrid)) _array_element)))))
                (Utilities|IsValid _output_get
                  (:Is%20Valid
                    ;[1 1 1] If unit is alive hit them with the ability.
                    (if (Default|IsAlive (LocalVariables|GetUnit))
                      (Default|UnitHitbyAbility (LocalVariables|GetUnit) (LocalVariables|GetAbilityAnimation) (LocalVariables|GetAbilityImpactReal))
                      ;[1 1 1] If unit is no longer alive, process its death.
                      (if (not (Default|IsAlive (LocalVariables|GetUnit)))
                        (CombatFlow|ProcessUnitDeath (LocalVariables|GetUnit))
                        ;[1 1 1] If only 1 team is left stop processing spell. This is to make sure there is not a no winner scenario. MAKE THIS BETTER.
                        (if (Variables|Default|GetIsFinishingCombat)
                          (return)))))))
              ;[1 1 1] If the unit cilled itself, end its turn and process its death.
              (if (not (Default|IsAlive (Variables|Default|GetCurrentUnit)))
                (LocalVariables|SetUnalivedUnit (Variables|Default|GetCurrentUnit))
                (CombatFlow|EndCurrentTurn)
                (CombatFlow|ProcessUnitDeath (LocalVariables|GetUnalivedUnit))))))))
    (:Is%20Not%20Valid
      (goto _label))))

(fn GetAbilityRange
  (params (OriginIndex :type Int%20Point%20Structure) (Cast :type S%20Ability%20Data%20Cast%20Structure))
  (bind (_rangepattern _rangeminmax _los) (Utilities|Struct|BreakS_AbilityData_Cast Cast))
  (bind _rangeindexes (CallFunction|GetIndexesfromPatternandRange OriginIndex (Variables|/Game/Blueprints/Tactical/Grid/BP_GridManager.BP_GridManager_C|GetGridTileShape (Variables|Default|GetGrid)) _rangepattern _rangeminmax))
  (bind _indexeswithlineofsight (Abilities|RemoveIndexesNotWalkable _rangeindexes))
  (if (.requirelineofsight _los)
    (bind _indexeswithlineofsight_2 (Abilities|RemoveIndexesWithoutLineOfSight OriginIndex _indexeswithlineofsight Cast))
    (return _indexeswithlineofsight_2)
    (else
      (return _indexeswithlineofsight))))

(fn HasLineOfSight
  (params (OriginIndex :type Int%20Point%20Structure) (TargetIndex :type Int%20Point%20Structure) (Cast :type S%20Ability%20Data%20Cast%20Structure))
  (bind _grid (Variables|Default|GetGrid))
  (bind _grid_2 (Variables|Default|GetGrid))
  (bind _los (Utilities|Struct|BreakS_AbilityData_Cast Cast))
  (bind _los_2 (Utilities|Struct|BreakS_AbilityData_Cast Cast))
  (bind _gridtilesize (Variables|/Game/Blueprints/Tactical/Grid/BP_GridManager.BP_GridManager_C|GetGridTileSize _grid))
  (bind _gridtiles (Variables|/Game/Blueprints/Tactical/Grid/BP_GridManager.BP_GridManager_C|GetGridTiles _grid_2))
  (bind _returnvalue (Math|Vector|MakeVector 0.0 0.0 (.heightfromground _los)))
  (bind _returnvalue_2 (* _gridtilesize (.offsetfromcenter _los_2)))
  (LocalVariables|SetOriginTile (.Value (Utilities|Map|Find _gridtiles OriginIndex)))
  (LocalVariables|SetTargetTile (.Value (Utilities|Map|Find _gridtiles TargetIndex)))
  (LocalVariables|SetTraceStart (+ (.location (Utilities|Struct|BreakS_TileData (LocalVariables|GetOriginTile))) _returnvalue))
  (LocalVariables|SetTraceEnd (+ (.location (Utilities|Struct|BreakS_TileData (LocalVariables|GetTargetTile))) _returnvalue))
  (for _array_element (Utilities|Array|MakeArray (Math|Vector2D|MakeVector2D (.x _returnvalue_2) 0.0) (Math|Vector2D|MakeVector2D (- 0.0 (.x _returnvalue_2)) 0.0) (Math|Vector2D|MakeVector2D 0.0 (.y _returnvalue_2)) (Math|Vector2D|MakeVector2D 0.0 (- 0.0 (.y _returnvalue_2))) "")
    (bind _returnvalue_3 (Collision|LineTraceByChannel (+ (LocalVariables|GetTraceStart) _array_element) (LocalVariables|GetTraceEnd) "TraceTypeQuery6" false 0 "None"))
    (if (not _returnvalue_3)
      (return true)))
  (return false))

(fn RemoveIndexesWithoutLineOfSight
  (params (OriginIndex :type Int%20Point%20Structure) (Indexes :type Array%20of%20Int%20Point%20Structures) (Cast :type S%20Ability%20Data%20Cast%20Structure))
  (for _array_element Indexes
    (if (Abilities|HasLineOfSight OriginIndex _array_element Cast)
      (Utilities|Array|Add (LocalVariables|GetRet) _array_element)))
  (return (LocalVariables|GetRet)))

(fn RemoveIndexesNotWalkable
  (params (Indexes :type Array%20of%20Int%20Point%20Structures))
  (for _array_element Indexes
    (if (Default|IsTileWalkable (Variables|Default|GetGrid) _array_element)
      (Utilities|Array|Add (LocalVariables|GetRet) _array_element)))
  (return (LocalVariables|GetRet)))

(fn SetUnitTeamIndex
  (params (Unit :type BP%20Unit%20Object%20Reference) (TeamIndex :type Integer))
  (Utilities|FlowControl|Sequence
    (:then_0
      (if (!= (Variables|/Game/Blueprints/Tactical/Units/BP_Unit.BP_Unit_C|GetTeamIndex Unit) -1)
        (bind _output_get (LocalVariables|SetUnitSet (.unitset (.Value (Utilities|Map|Find (Variables|Default|GetUnitTeams) (Variables|/Game/Blueprints/Tactical/Units/BP_Unit.BP_Unit_C|GetTeamIndex Unit))))))
        (Utilities|Set|Remove _output_get Unit)
        (if (> (Utilities|Set|Length (LocalVariables|GetUnitSet)) 0)
          (Utilities|Map|Add (Variables|Default|GetUnitTeams) (Variables|/Game/Blueprints/Tactical/Units/BP_Unit.BP_Unit_C|GetTeamIndex Unit) (Utilities|Struct|MakeS_UnitSet (LocalVariables|GetUnitSet)))
          (else
            (Utilities|Map|Remove (Variables|Default|GetUnitTeams) (Variables|/Game/Blueprints/Tactical/Units/BP_Unit.BP_Unit_C|GetTeamIndex Unit))))))
    (:then_1
      (if (!= TeamIndex -1)
        (bind _output_get_2 (LocalVariables|SetUnitSet (.unitset (.Value (Utilities|Map|Find (Variables|Default|GetUnitTeams) TeamIndex)))))
        (Utilities|Set|Add _output_get_2 Unit)
        (Utilities|Map|Add (Variables|Default|GetUnitTeams) TeamIndex (Utilities|Struct|MakeS_UnitSet (LocalVariables|GetUnitSet)))))
    (:then_2
      (Default|SetTeamIndex Unit TeamIndex)
      (Default|CallOnUnitTeamsChanged))))

(fn CanStartCombat
  (bind _unitsincombat (Variables|Default|GetUnitsInCombat))
  (bind _unitteams (Variables|Default|GetUnitTeams))
  (bind _isincombat (Variables|Default|GetIsInCombat))
  (bind _returnvalue (Utilities|Array|Length _unitsincombat))
  (bind _returnvalue_2 (Utilities|Map|Length _unitteams))
  (bind _returnvalue_3 (not _isincombat))
  (bind _returnvalue_4 (>= _returnvalue 2))
  (bind _returnvalue_5 (>= _returnvalue_2 2))
  (return (Math|Boolean|ANDBoolean _returnvalue_4 _returnvalue_5 _returnvalue_3) _returnvalue_4 _returnvalue_5 _returnvalue_3))

(fn StartCombat
  ;[1 1 1] Spawn random units.
  (bind _outactors (Actor|GetAllActorsOfClass "/Game/Blueprints/Tactical/Combat/BP_UnitSpawner.BP_UnitSpawner_C"))
  (for _array_element _outactors
    (Default|SpawnRandomUnit _array_element))
  (Variables|Default|SetIsInCombat true)
  ;[1 1 1] Notify units combat has started.
  (for _array_element_2 (Variables|Default|GetUnitsInCombat)
    (Default|CombatStarted _array_element_2))
  ;[1 1 1] Combat started notification.
  (Default|CallOnCombatStarted)
  (Variables|Default|SetCurrentUnit 0))

(fn EndCombat
  (Variables|Default|SetIsInCombat false)
  (Variables|Default|SetIsFinishingCombat false)
  (Variables|Default|SetCurrentUnit 0)
  (for _array_element (Variables|Default|GetUnitsInCombat)
    (Default|CombatEnded _array_element))
  (Default|CallOnCombatEnded))

(fn EndCurrentTurn
  (Utilities|FlowControl|Sequence
    (:then_0
      (Utilities|IsValid (Variables|Default|GetCurrentUnit)
        (:Is%20Valid
          (Default|TurnEnded (Variables|Default|GetCurrentUnit))
          (Default|CallOnUnitTurnEnded (Variables|Default|GetCurrentUnit)))))
    (:then_1
      (LocalVariables|SetCurrentIndex (Utilities|Array|FindItem (Variables|Default|GetUnitsInCombat) (Variables|Default|GetCurrentUnit)))
      (while (not (Utilities|IsValid (LocalVariables|GetNextLivingUnit))) ; Keep looking for a living unit
        (LocalVariables|SetCurrentIndex (Math|Integer|%(Integer) (+ (LocalVariables|GetCurrentIndex) 1) (Utilities|Array|Length (Variables|Default|GetUnitsInCombat))))
        (if (Default|IsAlive (Utilities|Array|Get(acopy) (Variables|Default|GetUnitsInCombat) (LocalVariables|GetCurrentIndex)))
          (LocalVariables|SetNextLivingUnit (Utilities|Array|Get(acopy) (Variables|Default|GetUnitsInCombat) (LocalVariables|GetCurrentIndex)))))
      (bind _output_get (Variables|Default|SetCurrentUnit (LocalVariables|GetNextLivingUnit)))
      (Default|TurnStarted _output_get)
      (Default|CallOnUnitTurnStarted _output_get)
      (Default|CenterCameraonGridTile (Variables|Default|GetGrid) (Variables|/Game/Blueprints/Tactical/Units/BP_Unit.BP_Unit_C|GetIndex _output_get)))))

(fn MoveUnit
  (params (Unit :type BP%20Unit%20Object%20Reference) (Path :type Array%20of%20Int%20Point%20Structures))
  (if (> (Utilities|Array|Length Path) 0)
    (Default|EventFollowPath Unit Path)
    (bind _cost (Default|GetPathCost (Variables|/Game/Blueprints/Tactical/Grid/BP_GridManager.BP_GridManager_C|GetGridPathfinding (Variables|Default|GetGrid)) Path))
    (Default|ModifyCurrentMP Unit (- 0 _cost) true false)
    (Units|SetUnitIndexonGrid Unit (Utilities|Array|Get(acopy) Path (Utilities|Array|LastIndex Path)) false false)))

(fn ProcessUnitDeath
  (params (Unit :type BP%20Unit%20Object%20Reference))
  (if (Variables|Default|GetIsInCombat)
    (Variables|/Game/Blueprints/Tactical/Units/BP_Unit.BP_Unit_C|SetSecondaryIndexForAbilityImpact Unit (Variables|/Game/Blueprints/Tactical/Units/BP_Unit.BP_Unit_C|GetIndex Unit))
    (Units|SetUnitIndexonGrid Unit (Utilities|Struct|MakeIntPoint -999 -999) false false)
    (Default|DebugHideUnitAfterDeath Unit)
    (bind _keys (Utilities|Map|Keys (Variables|Default|GetUnitTeams)))
    (for _array_element _keys
      (bind _output_get (LocalVariables|SetTeamIndex _array_element))
      (bind _result (Utilities|Set|ToArray (Utilities|Struct|BreakS_UnitSet (.Value (Utilities|Map|Find (Variables|Default|GetUnitTeams) _output_get)))))
      (bind _array_element_2 (Utilities|Array|ForEachLoopwithBreak _result :!label _label)
        (:LoopBody
          (if (Default|IsAlive _array_element_2)
            (Utilities|Array|Add (LocalVariables|GetTeamsAlive) (LocalVariables|GetTeamIndex))
            (goto _label Break)))))
    (if (== (Utilities|Array|Length (LocalVariables|GetTeamsAlive)) 1)
      (CombatFlow|FinishCombat (Utilities|Array|Get(acopy) (LocalVariables|GetTeamsAlive))))
    (else
      (Default|DebugRespawnAfterDeath Unit))))

(fn FinishCombat
  (params (WinningTeamIndex :type Integer))
  (Variables|Default|SetIsFinishingCombat true)
  (Default|CallOnCombatFinishing WinningTeamIndex))

(fn SetGrid
  (params (Grid :type BP%20Grid%20Manager%20Object%20Reference))
  (bind _output_get (Variables|Default|SetGrid Grid))
  (EventDispatchers|BindEventtoOnGridGenerated _output_get (EventDispatchers|CreateEvent :!event OnGridGenerated))
  (EventDispatchers|BindEventtoOnTileDataUpdated _output_get (EventDispatchers|CreateEvent :!event OnTileDataUpdated)))

(fn SpawnPlayerParty
  (bind _asgi_primary_game_instance (Utilities|Casting|CastToGI_PrimaryGameInstance (Game|GetGameInstance)))
  (bind _output_get (Variables|Default|SetPlayerParty (Variables|/Game/Blueprints/Utilities/GI_PrimaryGameInstance.GI_PrimaryGameInstance_C|GetPartyInBattle _asgi_primary_game_instance)))
  (for (_array_element _array_index) (.PartyMembers (Utilities|Struct|BreakS_Party _output_get))
    (LocalVariables|SetI _array_index)
    (bind _returnvalue (Game|SpawnActorfromClass "/Game/Blueprints/Tactical/Units/BP_Unit.BP_Unit_C" (Math|Transform|MakeTransform "0, 0, 0" "0, 0, 0" "1.000000,1.000000,1.000000") "Undefined" "MultiplyWithRoot" 0 (.Type (Utilities|Struct|BreakS_CharacterData _array_element)) 0))
    (Units|AddUnit _returnvalue (+ (Utilities|Struct|MakeIntPoint 25 25) (Utilities|Struct|MakeIntPoint (LocalVariables|GetI) 0)))))

(fn SpawnEnemies
  (bind _returnvalue (Game|SpawnActorfromClass "/Game/Blueprints/Tactical/Units/BP_Unit.BP_Unit_C" (Math|Transform|MakeTransform "0, 0, 0" "0, 0, 0" "1.000000,1.000000,1.000000") "Undefined" "MultiplyWithRoot" 0 "NewEnumerator3" 0))
  (Units|AddUnit _returnvalue (Utilities|Struct|MakeIntPoint 25 30) 1))