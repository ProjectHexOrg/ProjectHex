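; Ability animation actor for tactical combat that plays a visual attack from an origin tile onto each attacked grid tile.
; On BeginPlay it spawns one BP_AnimatedShape per attacked index, using the grid's tile mesh with randomized red brightness and play rate.
; Each finished shape raises a hit-tile event and removes its index.
; When none remain, the actor signals completion and destroys itself.
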(event Custom|Event_PlayAnimation
  (bind _grid (Variables|Default|GetGrid))
  (bind _originindex (Variables|Default|GetOriginIndex))
  (bind _data (Default|GetCurrentShapeData _grid))
  (bind _transform (CallFunction|GetTileTransform _originindex))
  (bind (_mesh _meshmaterial) (Utilities|Struct|BreakS_GridShapeData _data))
  (for _array_element (Variables|Default|GetAttackedIndexs)
    (bind _returnvalue (Game|SpawnActorfromClass "/Game/Blueprints/Tactical/Combat/Abilities/AbilityAnimations/Components/BP_AnimatedShape.BP_AnimatedShape_C" (Math|Transform|MakeTransform "0, 0, 0" "0, 0, 0" "1.000000,1.000000,1.000000") "AlwaysSpawn" "MultiplyWithRoot" 0 _mesh _meshmaterial (* "(R=1.000000,G=0.000000,B=0.016807,A=1.000000)" (Math|Random|RandomFloatinRange 0.5 1.5)) (Math|Transform|MakeTransform (.location _transform) (.rotation _transform) "0.010000,0.010000,0.010000") (CallFunction|GetTileTransform _array_element) (Math|Random|RandomFloatinRange 0.75 1.15) _array_element 0))
    (EventDispatchers|BindEventtoOnShapeAnimationCompleted _returnvalue (delegate Custom|Event_OnShapeAnimationCompleted))))

(event Custom|Event_OnShapeAnimationCompleted
  (params (AnimatedShape :type BP%20Animated%20Shape%20Object%20Reference))
  (bind _index (Variables|/Game/Blueprints/Tactical/Combat/Abilities/AbilityAnimations/Components/BP_AnimatedShape.BP_AnimatedShape_C|GetIndex AnimatedShape))
  (Default|CallOnAbilityAnimationHitTile self _index)
  (Utilities|Array|RemoveItem (Variables|Default|GetAttackedIndexs) _index)
  (if (== (Utilities|Array|Length (Variables|Default|GetAttackedIndexs)) 0)
    (CallFunction|EventCompleteAbilityAnimation)))

(event Custom|Event_CompleteAbilityAnimation
  (Default|CallOnAbilityAnimationCompleted self)
  (Actor|DestroyActor))

(event EventBeginPlay
  (CallFunction|EventPlayAnimation))

(fn ConstructionScript)

(fn GetTileTransform
  (params (Index :type Int%20Point%20Structure%20%28by%20ref%29))
  (return (.Transform (Utilities|Struct|BreakS_TileData (.Value (Utilities|Map|Find (Variables|/Game/Blueprints/Tactical/Grid/BP_GridManager.BP_GridManager_C|GetGridTiles (Variables|Default|GetGrid)) Index))))))

(fn OnShapeAnimationCompleted
  (params (AnimatedShape :type BP%20Animated%20Shape%20Object%20Reference)))