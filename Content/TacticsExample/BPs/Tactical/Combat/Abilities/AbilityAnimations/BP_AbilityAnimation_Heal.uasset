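; Ability animation actor that plays the heal effect on a targeted tile in tactical combat.
; On play it moves to the target tile, then a timeline spins and scales the effect root and drives opacity on ring and plus meshes.
; Shortly into the timeline it fires the hit-tile callback once, and on finish it completes the ability animation.
; The construction script tints the meshes in shades of green.
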(event EventBeginPlay
  (|CallParentFunction) ; This node is disabled and will not be called.\nDrag off pins to build functionality.
)

(event Collision|EventActorBeginOverlap
  (params (OtherActor :type Actor%20Object%20Reference)))

(event EventTick
  (params (DeltaSeconds :type Float%20%28single-precision%29)))

(event EventEventPlayAnimation
  (Transformation|SetActorLocation (.location (CallFunction|GetTileTransform (Variables|Default|GetTargetIndex))) false false)
  (bind (_direction _opacity _rotation _scale) (Timeline|Timeline_Heal PlayFromStart)
    (:Update
      (Transformation|SetRelativeRotation (Variables|Default|GetAnim_LocationRotationScale) (Math|Rotator|MakeRotator 0.0 0.0 _rotation) false false)
      (Transformation|SetRelativeScale3D (Variables|Default|GetAnim_LocationRotationScale) _scale)
      (Rendering|Material|SetScalarParameterValueonMaterials (Variables|Default|GetStaticMesh_Ring) "Opacity" _opacity)
      (if (>= (Components|Timeline|GetPlaybackPosition (Variables|Default|GetTimeline_Heal)) 0.2)
        (Utilities|FlowControl|DoOnce false
          (:Completed
            (Default|CallOnAbilityAnimationHitTile self (Variables|Default|GetTargetIndex))))))
    (:Finished
      (CallFunction|EventCompleteAbilityAnimation))))

(fn ConstructionScript
  (|CallParentFunction)
  (Rendering|Material|SetVectorParameterValueonMaterials (Variables|Default|GetStaticMesh_Ring) "Color" (Math|Conversions|ToVector(LinearColor) "(R=0.354083,G=1.000000,B=0.437987,A=1.000000)"))
  (Rendering|Material|SetVectorParameterValueonMaterials (Variables|Default|GetStaticMesh_Ring1) "Color" (Math|Conversions|ToVector(LinearColor) "(R=0.508316,G=1.000000,B=0.560634,A=1.000000)"))
  (Rendering|Material|SetVectorParameterValueonMaterials (Variables|Default|GetStaticMesh_Ring2) "Color" (Math|Conversions|ToVector(LinearColor) "(R=0.356400,G=1.000000,B=0.439657,A=1.000000)")))