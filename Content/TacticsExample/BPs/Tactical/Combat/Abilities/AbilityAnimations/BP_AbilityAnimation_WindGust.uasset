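; Ability animation for a wind gust in the tactical combat system, bursting from the target tile toward the other attacked tiles.
; After a brief delay it reports a hit on the target tile, then spawns an animated gust actor per remaining tile, rotated toward it, growing in scale, with randomized play rate.
; Each finished gust reports its tile as hit, and the ability animation completes once none remain.
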(event Custom|AnimationCompleted
  (params (AnimatedWindGust :type BP%20Animated%20Wind%20Gust%20Object%20Reference))
  (bind _index (Variables|/Game/Blueprints/Tactical/Combat/Abilities/AbilityAnimations/Components/BP_AnimatedWindGust.BP_AnimatedWindGust_C|GetIndex AnimatedWindGust))
  (Default|CallOnAbilityAnimationHitTile self _index)
  (Utilities|Array|RemoveItem (Variables|Default|GetAttackedIndexs) _index)
  (if (== (Utilities|Array|Length (Variables|Default|GetAttackedIndexs)) 0)
    (CallFunction|EventCompleteAbilityAnimation)))

(event EventBeginPlay
  (|CallParentFunction) ; This node is disabled and will not be called.\nDrag off pins to build functionality.
)

(event Collision|EventActorBeginOverlap
  (params (OtherActor :type Actor%20Object%20Reference)))

(event EventTick
  (params (DeltaSeconds :type Float%20%28single-precision%29)))

(event EventEventPlayAnimation
  (bind _targetindex (Variables|Default|GetTargetIndex))
  (bind _transform (CallFunction|GetTileTransform _targetindex))
  (Utilities|FlowControl|Delay 0.1)
  (Default|CallOnAbilityAnimationHitTile self (Variables|Default|GetTargetIndex))
  (Utilities|Array|RemoveItem (Variables|Default|GetAttackedIndexs) (Variables|Default|GetTargetIndex))
  (for _array_element (Variables|Default|GetAttackedIndexs)
    (bind _returnvalue (Game|SpawnActorfromClass "/Game/Blueprints/Tactical/Combat/Abilities/AbilityAnimations/Components/BP_AnimatedWindGust.BP_AnimatedWindGust_C" (Math|Transform|MakeTransform "0, 0, 0" "0, 0, 0" "1.000000,1.000000,1.000000") "Undefined" "MultiplyWithRoot" 0 (Math|Transform|MakeTransform (.location _transform) (Math|Rotator|FindLookatRotation (.location _transform) (.location (CallFunction|GetTileTransform _array_element))) "0.500000,0.500000,0.500000") (Math|Transform|MakeTransform (.location (CallFunction|GetTileTransform _array_element)) (Math|Rotator|FindLookatRotation (.location _transform) (.location (CallFunction|GetTileTransform _array_element))) "1.200000,1.200000,1.200000") (Math|Random|RandomFloatinRange 0.8 1.5) _array_element 0))
    (EventDispatchers|BindEventtoOnShapeAnimationCompleted _returnvalue (delegate Custom|AnimationCompleted))))

(fn ConstructionScript
  (|CallParentFunction))