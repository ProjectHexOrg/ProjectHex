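; Sword slash ability animation actor for tactical combat, played from an origin tile toward a target tile.
; On play, it moves to the origin tile and faces the target using a yaw derived from the grid indices.
; A Timeline animates the pitch and scale of AnimRotationScale, broadcasts the tile hit once at 0.4 seconds, then completes the ability animation when finished.
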(event EventBeginPlay
  (|CallParentFunction) ; This node is disabled and will not be called.\nDrag off pins to build functionality.
)

(event Collision|EventActorBeginOverlap
  (params (OtherActor :type Actor%20Object%20Reference)))

(event EventTick
  (params (DeltaSeconds :type Float%20%28single-precision%29)))

(event EventEventPlayAnimation
  (bind _anim_rotationscale (Variables|Default|GetAnim_RotationScale))
  (Transformation|SetActorLocationAndRotation (.location (CallFunction|GetTileTransform (Variables|Default|GetOriginIndex))) (Math|Rotator|FindLookatRotation (Math|Conversions|ToVector(Vector2D) (Math|Conversions|ToVector2D(IntPoint) (Variables|Default|GetOriginIndex))) (Math|Conversions|ToVector(Vector2D) (Math|Conversions|ToVector2D(IntPoint) (Variables|Default|GetTargetIndex)))))
  (bind (_direction _rotationy _scale) (Timeline|Timeline PlayFromStart)
    (:Update
      (Transformation|SetRelativeRotation _anim_rotationscale (Math|Rotator|MakeRotator 0.0 _rotationy 0.0) false false)
      (Transformation|SetRelativeScale3D _anim_rotationscale (Math|Conversions|ToVector(Float) _scale))
      (if (>= (Components|Timeline|GetPlaybackPosition (Variables|Default|GetTimeline)) 0.4)
        (Utilities|FlowControl|DoOnce false
          (:Completed
            (Default|CallOnAbilityAnimationHitTile self (Variables|Default|GetTargetIndex))))))
    (:Finished
      (CallFunction|EventCompleteAbilityAnimation))))

(fn ConstructionScript
  (|CallParentFunction))