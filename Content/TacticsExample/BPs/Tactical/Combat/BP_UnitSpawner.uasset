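; BP_UnitSpawner is a placed actor that spawns a random unit for a team on its tile of the tactical combat grid.
; It binds to CombatManager and Grid events, snapping and scaling itself to its tile when the grid generates.
; SpawnRandomUnit picks a type by weighted random from SpawnableUnitWeights and registers the new unit with CombatManager.
; Its icon hides during combat and returns when combat ends, when the unit is destroyed.
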(event Custom|Event_OnCombatStarted
  (Rendering|SetVisibility (Variables|Default|GetSpawnIcon) false true))

(event Custom|Event_OnCombatEnded
  (Rendering|SetVisibility (Variables|Default|GetSpawnIcon) true true)
  (Default|RemoveUnit (Variables|Default|GetCombatManager) (Variables|Default|GetUnit) true)
  (Variables|Default|SetUnit 0))

(event EventBeginPlay
  (bind _returnvalue (Actor|GetActorOfClass "/Game/Blueprints/Tactical/Combat/BP_CombatManager.BP_CombatManager_C"))
  (Variables|Default|SetCombatManager _returnvalue)
  (EventDispatchers|BindEventtoOnCombatStarted (Variables|Default|GetCombatManager) (EventDispatchers|CreateEvent :!event Custom|Event_OnCombatStarted))
  (EventDispatchers|BindEventtoOnCombatEnded (Variables|Default|GetCombatManager) (EventDispatchers|CreateEvent :!event Custom|Event_OnCombatEnded))
  (EventDispatchers|BindEventtoOnGridGenerated (Variables|/Game/Blueprints/Tactical/Combat/BP_CombatManager.BP_CombatManager_C|GetGrid (Variables|Default|GetCombatManager)) (EventDispatchers|CreateEvent :!event OnGridGenerated)))

(event Collision|EventActorBeginOverlap
  (params (OtherActor :type Actor%20Object%20Reference)))

(event EventTick
  (params (DeltaSeconds :type Float%20%28single-precision%29)))

(fn ConstructionScript)

(fn SetGridIndex
  (bind _index (Default|GetTileIndexfromWorldLocation (Variables|/Game/Blueprints/Tactical/Combat/BP_CombatManager.BP_CombatManager_C|GetGrid (Variables|Default|GetCombatManager)) (Transformation|GetWorldLocation (Variables|Default|GetDefaultSceneRoot self))))
  (Variables|Default|SetIndex _index))

(fn SelectRandomUnit
  (bind _weightsum (CallFunction|GetSpawnableUnitWeightSum))
  (bind _output_get (LocalVariables|SetWeightedSum _weightsum))
  (LocalVariables|SetSelection (Math|Random|RandomIntegerinRange 1 _output_get))
  (LocalVariables|SetRunningSum 0)
  (bind _keys (Utilities|Map|Keys (Variables|Default|GetSpawnableUnitWeights)))
  (for _array_element _keys
    (bind _output_get_2 (LocalVariables|SetSelectedType _array_element))
    (bind _output_get_3 (LocalVariables|SetRunningSum (+ (LocalVariables|GetRunningSum) (.Value (Utilities|Map|Find (Variables|Default|GetSpawnableUnitWeights) _output_get_2)))))
    (if (>= _output_get_3 (LocalVariables|GetSelection))
      (return (LocalVariables|GetSelectedType)))))

(fn GetSpawnableUnitWeightSum
  (LocalVariables|SetRet 0)
  (bind _values (Utilities|Map|Values (Variables|Default|GetSpawnableUnitWeights)))
  (for _array_element _values
    (LocalVariables|SetRet (+ _array_element (LocalVariables|GetRet))))
  (return (LocalVariables|GetRet)))

(fn SpawnRandomUnit
  (bind _unittype (CallFunction|SelectRandomUnit))
  (bind _returnvalue (Game|SpawnActorfromClass "/Game/Blueprints/Tactical/Units/BP_Unit.BP_Unit_C" (Math|Transform|MakeTransform "0, 0, 0" "0, 0, 0" "1.000000,1.000000,1.000000") "Undefined" "MultiplyWithRoot" 0 _unittype 0))
  (bind _output_get (Variables|Default|SetUnit _returnvalue))
  (Default|AddUnit (Variables|Default|GetCombatManager) _output_get (Variables|Default|GetIndex) (Variables|Default|GetTeamIndex)))

(fn OnGridGenerated
  (CallFunction|SetGridIndex)
  (Transformation|SetActorScale3D self (/ (Default|GetTileScale (Variables|/Game/Blueprints/Tactical/Combat/BP_CombatManager.BP_CombatManager_C|GetGrid (Variables|Default|GetCombatManager))) 2))
  (Transformation|SetActorLocation (Default|GetTileLocationfromGridIndex (Variables|/Game/Blueprints/Tactical/Combat/BP_CombatManager.BP_CombatManager_C|GetGrid (Variables|Default|GetCombatManager)) (Variables|Default|GetIndex)) false false))